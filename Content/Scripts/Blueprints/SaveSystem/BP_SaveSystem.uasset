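; BP_SaveSystem is a save data container for hero rosters, game progression, and inn and infirmary slot occupancy.
; Paired save and load functions copy values into and out of its variables: heroes, including those in tavern or infirmary, and progression such as week, resources, consumables, weekly recruitment and new-game state.
; ResetRecoverySlots empties both slot arrays.
; No function here writes to disk.
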(fn SaveHeroes
  (params (StructHeroes :type Array%20of%20STRUCT%20Heroes%20Data%20New%20Structures) (HeroesInTavern :type Array%20of%20STRUCT%20Heroes%20Data%20New%20Structures) (HeroesInInfirmary :type Array%20of%20STRUCT%20Heroes%20Data%20New%20Structures))
  (Variables|Heroes|SetStructHeroes StructHeroes)
  (Variables|Heroes|SetHeroesInTavern HeroesInTavern)
  (Variables|Heroes|SetHeroesInInfirmary HeroesInInfirmary))

(fn LoadHeroes
  (return (Variables|Heroes|GetStructHeroes) (Variables|Heroes|GetHeroesInTavern) (Variables|Heroes|GetHeroesInInfirmary)))

(fn SaveProgression
  (params (GameWeek :type Integer) (Resources :type Array%20of%20Struct%20Resources%20New%20Structures) (Consumables :type Array%20of%20STRUCT%20Consumables%20New%20Structures) (RecruitmentOfTheWeek :type Boolean) (NewGameCreated :type Boolean))
  (Variables|Progression|SetGameWeek GameWeek)
  (Variables|Progression|SetResources Resources)
  (Variables|Progression|SetConsumables Consumables)
  (Variables|Progression|SetRecruitmentOfTheWeek RecruitmentOfTheWeek)
  (Variables|Progression|SetNewGameCreated? NewGameCreated))

(fn LoadProgression
  (return (Variables|Progression|GetGameWeek) (Variables|Progression|GetResources) (Variables|Progression|GetConsumables) (Variables|Progression|GetRecruitmentOfTheWeek) (Variables|Progression|GetNewGameCreated?)))

(fn SaveInnData
  (params (InnSlotBusy :type Array%20of%20Booleans))
  (Variables|city|SetInnSlotBusy InnSlotBusy))

(fn SaveInfirmaryData
  (params (InfirmarySlotBusy :type Array%20of%20Booleans))
  (Variables|City|SetInfirmarySlotBusy InfirmarySlotBusy))

(fn LoadInnData
  (return (Variables|city|GetInnSlotBusy)))

(fn LoadInfirmaryData
  (return (Variables|City|GetInfirmarySlotBusy)))

(fn ResetRecoverySlots
  (Variables|City|SetInfirmarySlotBusy (Utilities|Array|MakeArray))
  (Variables|city|SetInnSlotBusy (Utilities|Array|MakeArray)))