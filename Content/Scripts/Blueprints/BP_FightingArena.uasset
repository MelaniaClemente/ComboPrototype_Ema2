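; Arena actor that spawns waves of randomized enemies after a player character enters its sphere, box or capsule trigger, configured in the Construction Script.
; A looping timer spawns at random local points up to concurrent and total caps, assigning race and moveset before AI initialization.
; MaxNumberOfEnemiesReached returns true while below the cap, despite its name.
; Tick copies SpawnEnded into ArenaEnabled while enabled; OnSnapDataLoaded destroys disabled arenas.
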(event OnComponentBeginOverlap(BoxTrigger)
  (params (OverlappedComponent :type Primitive%20Component%20Object%20Reference) (OtherActor :type Actor%20Object%20Reference) (OtherComp :type Primitive%20Component%20Object%20Reference) (OtherBodyIndex :type Integer) (bFromSweep :type Boolean) (SweepResult :type Hit%20Result%20Structure%20%28by%20ref%29))
  (CallFunction|ProcessonPlayerOverlap OtherActor))

(event OnComponentBeginOverlap(CapsuleTrigger)
  (params (OverlappedComponent :type Primitive%20Component%20Object%20Reference) (OtherActor :type Actor%20Object%20Reference) (OtherComp :type Primitive%20Component%20Object%20Reference) (OtherBodyIndex :type Integer) (bFromSweep :type Boolean) (SweepResult :type Hit%20Result%20Structure%20%28by%20ref%29))
  (CallFunction|ProcessonPlayerOverlap OtherActor))

(event OnComponentBeginOverlap(SphereTrigger)
  (params (OverlappedComponent :type Primitive%20Component%20Object%20Reference) (OtherActor :type Actor%20Object%20Reference) (OtherComp :type Primitive%20Component%20Object%20Reference) (OtherBodyIndex :type Integer) (bFromSweep :type Boolean) (SweepResult :type Hit%20Result%20Structure%20%28by%20ref%29))
  (CallFunction|ProcessonPlayerOverlap OtherActor))

(event EventBeginPlay)

(event Collision|EventActorBeginOverlap
  (params (OtherActor :type Actor%20Object%20Reference)))

(event EventTick
  (params (DeltaSeconds :type Float%20%28single-precision%29))
  (if (Variables|Arena|GetArenaEnabled?)
    (Variables|Arena|SetArenaEnabled? (CallFunction|SpawnEnded?))))

(event EventOnSnapDataLoaded
  (if (not (Variables|Arena|GetArenaEnabled?))
    (Actor|DestroyActor)))

(fn ConstructionScript
  (switch Utilities|FlowControl|Switch|SwitchonENUM_ColliderType (Variables|Collider|GetColliderType)
    (:NewEnumerator0
      (Utilities|IsValid (Variables|Default|GetSphereTrigger)
        (:Is%20Valid
          _)
        (:Is%20Not%20Valid
          (bind _returnvalue (AddComponent|AddSphereComponent false))
          (bind _output_get (Variables|Default|SetSphereTrigger _returnvalue))
          (Utilities|IsValid _output_get
            (:Is%20Valid
              _))))
      (Components|Sphere|SetSphereRadius _output_get (Variables|Collider|GetTriggerRadius) true)
      (Collision|SetCollisionResponsetoAllChannels (Variables|Default|GetSphereTrigger) "ECR_Ignore")
      (Collision|SetCollisionResponsetoChannel (Variables|Default|GetSphereTrigger) "ECC_Pawn" "ECR_Overlap")
      (Collision|SetCollisionResponsetoChannel (Variables|Default|GetSphereTrigger) "ECC_PhysicsBody" "ECR_Ignore")
      (Development|SetHiddeninGame (Variables|Default|GetSphereTrigger) (Variables|Collider|GetTriggerHiddenIngame) false)
      (Transformation|SetRelativeLocation (Variables|Default|GetSphereTrigger) (Variables|Collider|GetTriggerOffset) false false))
    (:NewEnumerator1
      (Utilities|IsValid (Variables|Default|GetBoxTrigger)
        (:Is%20Valid
          _)
        (:Is%20Not%20Valid
          (bind _returnvalue_2 (AddComponent|AddBoxComponent false))
          (bind _output_get_2 (Variables|Default|SetBoxTrigger _returnvalue_2))
          (Utilities|IsValid _output_get_2
            (:Is%20Valid
              _))))
      (Components|Box|SetBoxExtent _output_get_2 (Variables|Collider|GetTriggerBoxDimension) true)
      (Collision|SetCollisionResponsetoAllChannels (Variables|Default|GetBoxTrigger) "ECR_Ignore")
      (Collision|SetCollisionResponsetoChannel (Variables|Default|GetBoxTrigger) "ECC_Pawn" "ECR_Overlap")
      (Collision|SetCollisionResponsetoChannel (Variables|Default|GetBoxTrigger) "ECC_PhysicsBody" "ECR_Ignore")
      (Development|SetHiddeninGame (Variables|Default|GetBoxTrigger) (Variables|Collider|GetTriggerHiddenIngame) false)
      (Transformation|SetRelativeLocation (Variables|Default|GetBoxTrigger) (Variables|Collider|GetTriggerOffset) false false))
    (:NewEnumerator2
      (Utilities|IsValid (Variables|Default|GetCapsuleTrigger)
        (:Is%20Valid
          _)
        (:Is%20Not%20Valid
          (bind _returnvalue_3 (AddComponent|AddCapsuleComponent false))
          (bind _output_get_3 (Variables|Default|SetCapsuleTrigger _returnvalue_3))
          (Utilities|IsValid _output_get_3
            (:Is%20Valid
              _))))
      (Components|Capsule|SetCapsuleRadius _output_get_3 (Variables|Collider|GetTriggerRadius) true)
      (Components|Capsule|SetCapsuleHalfHeight (Variables|Default|GetCapsuleTrigger) (Variables|Collider|GetTriggerHalfHeight) true)
      (Collision|SetCollisionResponsetoAllChannels (Variables|Default|GetCapsuleTrigger) "ECR_Ignore")
      (Collision|SetCollisionResponsetoChannel (Variables|Default|GetCapsuleTrigger) "ECC_Pawn" "ECR_Overlap")
      (Collision|SetCollisionResponsetoChannel (Variables|Default|GetCapsuleTrigger) "ECC_PhysicsBody" "ECR_Ignore")
      (Development|SetHiddeninGame (Variables|Default|GetCapsuleTrigger) (Variables|Collider|GetTriggerHiddenIngame) false)
      (Transformation|SetRelativeLocation (Variables|Default|GetCapsuleTrigger) (Variables|Collider|GetTriggerOffset) false false))))

(fn ProcessonPlayerOverlap
  (params (Actor :type Actor%20Object%20Reference))
  (Utilities|Casting|CastToBP_PlayerCharacter Actor)
  (Utilities|Time|SetTimerbyFunctionName 0 "SpawnRandomEnemyFromClass" 2.0 true))

(fn MaxNumberOfEnemiesReached?
  (return (< (Utilities|Array|Length (Variables|Arena|GetEnemiesInArena)) (Variables|Arena|GetMaxEnemiesInArena))))

(fn SpawnRandomEnemyfromClass
  (CallFunction|UpdateEnemiesinArena)
  (if (and (CallFunction|MaxNumberOfEnemiesReached?) (not (CallFunction|SpawnEnded?)))
    (bind _returnvalue (Game|SpawnActorfromClass "/Game/Scripts/Blueprints/Characters/Enemies/BP_EnemyMaster.BP_EnemyMaster_C" (CallFunction|GetRandomSpawnTransform) "Undefined" 0 0))
    (Utilities|Array|Add (Variables|Arena|GetEnemiesInArena) _returnvalue)
    (CallFunction|IncreaseSpawnedEnemies)
    (Variables|/Game/Scripts/Blueprints/Characters/Enemies/BP_EnemyMaster.BP_EnemyMaster_C|SetRace _returnvalue (CallFunction|GetRandomRace))
    (Variables|/Game/Scripts/Blueprints/Characters/BP_CharacterMaster.BP_CharacterMaster_C|SetMoveset _returnvalue (CallFunction|GetRandomMoveset))
    (bind _asbp_aicontroller (Utilities|Casting|CastToBP_AIController (AI|GetAIController _returnvalue)))
    (Default|InitializeEnemy _asbp_aicontroller)))

(fn GetRandomSpawnTransform
  (bind _spawnpoints (Variables|Arena|GetSpawnPoints))
  (return (Math|Transform|MakeTransform (CallFunction|RelativeLoctoWorld (Utilities|Array|Get(acopy) _spawnpoints (Math|Random|RandomIntegerinRange 0 (Utilities|Array|LastIndex _spawnpoints))) (Transformation|GetActorTransform)))))

(fn IncreaseMaxEnemiesinArena)

(fn UpdateEnemiesinArena
  (bind _enemiesinarena (Variables|Arena|GetEnemiesInArena))
  (for _array_element _enemiesinarena
    (Utilities|IsValid _array_element
      (:Is%20Not%20Valid
        (Utilities|Array|RemoveItem _enemiesinarena _array_element)))))

(fn SpawnEnded?
  (return (>= (Variables|Arena|GetNumberOfSpawnDone) (Variables|Arena|GetTotalEnemiesToSpawn))))

(fn IncreaseSpawnedEnemies
  (Variables|Arena|SetNumberOfSpawnDone (+ (Variables|Arena|GetNumberOfSpawnDone) 1)))

(fn GetRandomRace
  (bind _allowedraces (Variables|Arena|GetAllowedRaces))
  (return (Utilities|Array|Get(acopy) _allowedraces (Math|Random|RandomIntegerinRange 0 (Utilities|Array|LastIndex _allowedraces)))))

(fn GetRandomMoveset
  (bind _allowedmovesets (Variables|Arena|GetAllowedMovesets))
  (return (Utilities|Array|Get(acopy) _allowedmovesets (Math|Random|RandomIntegerinRange 0 (Utilities|Array|LastIndex _allowedmovesets)))))