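; Example player controller that wires a lock-on Targeting System (TS) into player input, with logic meant to be copied into other Blueprints.
; On BeginPlay it initializes TS with its AIPerception component and the controlled pawn.
; Hard-coded T, Q and E key events call TS to lock onto a target, the target to the left, or the target to the right.
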(event EventBeginPlay
  ;[0 0 0] Initialize Targeting System's Key Variables and Mechanics|Copy and Paste Into Your Own Blueprints If Desired
  (Default|InitializeVariables (Variables|Default|GetTS) (Variables|Default|GetAIPerception) (Pawn|GetControlledPawn self)))

(event EventTick
  (params (DeltaSeconds :type Float%20%28single-precision%29)))

(event Input|KeyboardEvents|E
  (params (Key :type Key%20Structure :default "None"))
  ;[0 0 0] Lock On To Target|Copy and Paste Into Your Own Blueprints If Desired
  (:Pressed
    (Default|LockontoTargettotheRight (Variables|Default|GetTS))))

(event Input|KeyboardEvents|T
  (params (Key :type Key%20Structure :default "None"))
  ;[0 0 0] Lock On To Target|Copy and Paste Into Your Own Blueprints If Desired
  (:Pressed
    (Default|LockontoTarget (Variables|Default|GetTS))))

(event Input|KeyboardEvents|Q
  (params (Key :type Key%20Structure :default "None"))
  ;[0 0 0] Lock On To Target|Copy and Paste Into Your Own Blueprints If Desired
  (:Pressed
    (Default|LockontoTargettotheLeft (Variables|Default|GetTS))))

(fn ConstructionScript)