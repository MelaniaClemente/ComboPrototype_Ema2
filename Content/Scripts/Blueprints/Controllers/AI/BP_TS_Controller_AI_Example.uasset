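; Example AI controller that shows how to hook a targeting system component up to an AI-controlled pawn.
; On BeginPlay it initializes the targeting component with its AI Perception component and controlled pawn.
; Target center, left and right events call the component's lock-on functions to lock onto a target or shift it to either side.
; The event logic is commented as copy-and-paste snippets for other Blueprints.
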(event Custom|Target%20Center
  ;[0 0 0] Lock On To Target|Copy and Paste Into Your Own Blueprints If Desired
  (Default|LockontoTarget (Variables|Default|GetTS)))

(event Custom|Target%20Left
  ;[0 0 0] Lock On To Target|Copy and Paste Into Your Own Blueprints If Desired
  (Default|LockontoTargettotheLeft (Variables|Default|GetTS)))

(event Custom|Target%20Right
  ;[0 0 0] Lock On To Target|Copy and Paste Into Your Own Blueprints If Desired
  (Default|LockontoTargettotheRight (Variables|Default|GetTS)))

(event EventBeginPlay
  ;[0 0 0] Initialize Targeting System's Key Variables and Mechanics|Copy and Paste Into Your Own Blueprints If Desired
  (Default|InitializeVariables (Variables|Default|GetTS) (Variables|Default|GetAIPerception) (Pawn|GetControlledPawn self)))

(event EventTick
  (params (DeltaSeconds :type Float%20%28single-precision%29)))

(fn ConstructionScript)