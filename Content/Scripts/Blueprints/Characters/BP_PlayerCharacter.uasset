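; Player character for a dungeon game, initializing experience, combat, health, stamina, interaction and camera components.
; Health exhaustion plays death and fade, then respawns at the current checkpoint, or clears dungeon resources and loads the dungeon-end map without one.
; Stamina use restarts recovery and feeds fatigue when exhausted.
; Also handles rolling, movement speed and floor-traced checkpoint spawning, plus a Y-key debug drawing navigation paths to reachable doors.
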(event OnInitialization(BP_HealthComponent)
  (bind _bp_healthcomponent (Variables|Default|GetBP_HealthComponent))
  (Variables|/Game/Scripts/Blueprints/Components/GameParameters/BP_CharacterParametersComponent.BP_CharacterParametersComponent_C|SetGameAttribute _bp_healthcomponent (.Health (Utilities|Struct|BreakSTRUCT_HeroesData (Variables|/Game/Scripts/Blueprints/Components/GameParameters/BP_CharacterParametersComponent.BP_CharacterParametersComponent_C|GetHeroData _bp_healthcomponent)))))

(event OnInitialization(StaminaComponent)
  (bind _staminacomponent (Variables|Default|GetStaminaComponent))
  (Variables|/Game/Scripts/Blueprints/Components/GameParameters/BP_CharacterParametersComponent.BP_CharacterParametersComponent_C|SetGameAttribute _staminacomponent (.Stamina (Utilities|Struct|BreakSTRUCT_HeroesData (Variables|/Game/Scripts/Blueprints/Components/GameParameters/BP_CharacterParametersComponent.BP_CharacterParametersComponent_C|GetHeroData _staminacomponent)))))

(event OnParameterExhausted(BP_HealthComponent)
  (bind _controllerref (Variables|Default|GetControllerRef))
  (Utilities|IsValid _controllerref
    (:Is%20Valid
      (Input|SetIgnoreMoveInput _controllerref true)
      (Input|SetIgnoreLookInput _controllerref true)
      (Components|Movement|StopMovementImmediately (Variables|Character|GetCharacterMovement)))
    (:Is%20Not%20Valid
      _))
  (CallFunction|Death (Utilities|Array|Get(acopy) (Variables|/Game/Scripts/Blueprints/Components/Animation/BP_CombatComponent.BP_CombatComponent_C|GetSwordAndShield_Death (Variables|Default|GetBP_CombatComponent))))
  (Collision|SetCollisionResponsetoChannel (Variables|Default|GetCapsuleComponent) "ECC_Pawn" "ECR_Ignore")
  (CameraFades|StartCameraFade :self (Game|GetPlayerCameraManager 0) :ToAlpha 1.0 :Duration 1.5 :bShouldFadeAudio true :bHoldWhenFinished true)
  (Utilities|FlowControl|Delay 1.5)
  (CallFunction|Respawn))

(event Custom|InitializeComponents
  (CallFunction|InitializeClass)
  (Default|Initialization (Variables|Default|GetBP_Experience))
  (Default|Initialization (Variables|Default|GetBP_CombatComponent))
  (Default|Initialization (Variables|Default|GetBP_HealthComponent))
  (Default|Initialization (Variables|Default|GetStaminaComponent))
  (Default|Initialization (Variables|Default|GetBP_PlayerInteractionComponent))
  (Default|Initialization (Variables|Default|GetBP_PlayerCameraComponent))
  (CallFunction|InitializePlayerController)
  (CallFunction|InitializePhysicalAnimation)
  (Utilities|Time|SetTimerbyEvent (delegate Custom|CheckCameraRotation) 0.05 true))

(event Custom|Respawn
  (bind _controllerref (Variables|Default|GetControllerRef))
  ;[1 1 1] Death And Respawn
  (Utilities|IsValid (Variables|Default|GetCurrentCheckpoint)
    (:Is%20Valid
      (CallFunction|ResetGamplayAttributes)
      (Transformation|Teleport (.RespawnLocation (Default|GetRespawnLocationandRotation (Variables|Default|GetCurrentCheckpoint) self)) (.RespawnRotation (Default|GetRespawnLocationandRotation (Variables|Default|GetCurrentCheckpoint) self)))
      (Transformation|SetActorRotation (.RespawnRotation (Default|GetRespawnLocationandRotation (Variables|Default|GetCurrentCheckpoint) self)))
      (CameraFades|StartCameraFade :self (Game|GetPlayerCameraManager 0) :FromAlpha 1.0 :Duration 1.5 :bShouldFadeAudio true :bHoldWhenFinished true)
      (Utilities|FlowControl|Delay 2.0)
      (Variables|/Game/Scripts/Blueprints/LevelDesignHelper/Interaction/BP_InteractibleObject_Master.BP_InteractibleObject_Master_C|SetInteractionType (Variables|Default|GetCurrentCheckpoint) "NewEnumerator3")
      (Variables|Default|SetCurrentCheckpoint 0)
      (Utilities|IsValid _controllerref
        (:Is%20Valid
          (Input|SetIgnoreMoveInput _controllerref false)
          (Input|SetIgnoreLookInput _controllerref false)
          (Default|SetCurrentAnimationPriority (Variables|Default|GetBP_CombatComponent))
          (Default|ResetExhaustedEvent (Variables|Default|GetBP_HealthComponent)))))
    (:Is%20Not%20Valid
      (bind _asbp_gameplay_instance (Utilities|Casting|CastToBP_GameplayInstance (Game|GetGameInstance)))
      (for (_array_element _array_index) (Variables|/Game/Scripts/Blueprints/GameModes/BP_GameplayInstance.BP_GameplayInstance_C|GetStruct_DungeonResources _asbp_gameplay_instance)
        (bind _structout (Utilities|Struct|SetmembersinStruct_Resources _array_element))
        (Utilities|Array|SetArrayElem (Variables|/Game/Scripts/Blueprints/GameModes/BP_GameplayInstance.BP_GameplayInstance_C|GetStruct_DungeonResources _asbp_gameplay_instance) _array_index _structout))
      (Variables|/Game/Scripts/Blueprints/GameModes/BP_GameplayInstance.BP_GameplayInstance_C|SetSelectedHero _asbp_gameplay_instance "")
      (Game|OpenLevel(byName) "MAP_DungeonEnd"))))

(event Custom|CheckCameraRotation
  (if (not (Variables|Default|GetbUseControllerRotationYaw))
    (Variables|Default|SetbUseControllerRotationYaw true)
    (Variables|/Script/Engine.SpringArmComponent|SetbUsePawnControlRotation (Variables|Default|GetSpringArm) true)))

(event EventBeginPlay
  (|CallParentFunction))

(event Collision|EventActorBeginOverlap
  (params (OtherActor :type Actor%20Object%20Reference))
  (|CallParentFunction OtherActor) ; This node is disabled and will not be called.\nDrag off pins to build functionality.
)

(event EventTick
  (params (DeltaSeconds :type Float%20%28single-precision%29))
  (|CallParentFunction DeltaSeconds))

(event Input|KeyboardEvents|Y
  (params (Key :type Key%20Structure :default "None"))
  (:Pressed
    (bind _outactors (Actor|GetAllActorsOfClass "/Game/Scripts/Blueprints/LevelDesignHelper/Interaction/BP_MyDoor.BP_MyDoor_C"))
    (for _array_element _outactors
      (bind _returnvalue (Class|NavigationSystemV1|FindPathtoActorSynchronously (Transformation|GetActorLocation) _array_element 1.5e+06 (Pawn|GetController) 0))
      (if (<= (Math|Vector|Distance(Vector) (Utilities|Array|Get(acopy) (Variables|/Script/NavigationSystem.NavigationPath|GetPathPoints _returnvalue) (Utilities|Array|LastIndex (Variables|/Script/NavigationSystem.NavigationPath|GetPathPoints _returnvalue))) (Transformation|GetActorLocation _array_element)) 2e+02)
        (for (_array_element_2 _array_index) (Variables|/Script/NavigationSystem.NavigationPath|GetPathPoints _returnvalue)
          (switch int _array_index
            (:Default
              (Rendering|Debug|DrawDebugArrow (Utilities|Array|Get(acopy) (Variables|/Script/NavigationSystem.NavigationPath|GetPathPoints _returnvalue) (- _array_index 1)) _array_element_2 15.0 "(R=0.812500,G=0.424243,B=0.000000,A=1.000000)" 5.0 1e+01))))))))

(event Custom|Dodge/Roll
  (CallFunction|RollbyInput))

(event OnConsume(StaminaComponent)
  (params (ValueToConsume :type Float%20%28single-precision%29) (PrintDebugToScreen :type Boolean))
  (bind _staminacomponent (Variables|Default|GetStaminaComponent))
  ;[1 1 1] Stamina Events
  (if (Default|IsExhausted (Variables|Default|GetStaminaComponent))
    (Default|RestoreValue (Variables|Default|GetFatigueComponent) 0.1 false))
  (Default|SetModifierPerSecond (Variables|Default|GetStaminaComponent) 0.0)
  (Default|InvalidateRecoveryTimer _staminacomponent)
  (Default|StartRecoveryTimer _staminacomponent))

(fn ConstructionScript
  (|CallParentFunction))

(fn GetMyPlayerCharacter
  (return self))

(fn GetMyPlayerControllerbyInterface
  (bind _returnvalue (Pawn|GetController))
  (if (Utilities|DoesObjectImplementInterface _returnvalue "/Game/Scripts/Blueprints/Interfaces/BP_CharacterInterface.BP_CharacterInterface_C")
    (bind _myplayercontroller (Class|BPCharacterInterface|GetMyPlayerController(Message) _returnvalue))
    (return _myplayercontroller)
    (else
      (CallFunction|DebugMsgDoesNotImplementCharacterInterface _returnvalue false))))

(fn GetTeamID
  (return "NewEnumerator0"))

(fn ResetGamplayAttributes
  (bind _bp_healthcomponent (Variables|Default|GetBP_HealthComponent))
  (bind _staminacomponent (Variables|Default|GetStaminaComponent))
  (Default|SetCurrentValue _bp_healthcomponent (Default|GetMaxValue _bp_healthcomponent))
  (Default|SetCurrentValue _staminacomponent (Default|GetMaxValue _staminacomponent)))

(fn SpawnCheckpoint
  (params (SpawnDistance :type Float%20%28single-precision%29))
  (bind _returnvalue (Transformation|GetActorLocation))
  (bind _returnvalue_2 (Transformation|GetActorForwardVector))
  (bind _capsulecomponent (Variables|Default|GetCapsuleComponent))
  (bind _returnvalue_3 (Components|Capsule|GetScaledCapsuleRadius _capsulecomponent))
  (bind _returnvalue_4 (+ _returnvalue_3 SpawnDistance))
  (bind _returnvalue_5 (* _returnvalue_2 _returnvalue_4))
  (bind _returnvalue_6 (+ _returnvalue _returnvalue_5))
  (Utilities|IsValid (Variables|Default|GetCheckpoint)
    (:Is%20Valid
      (Development|PrintString (Utilities|String|Append "Already had a checkpoint: " (Utilities|GetDisplayName (Variables|Default|GetCheckpoint))))
      (LocalVariables|SetSuccess false))
    (:Is%20Not%20Valid
      (bind (_outhit _returnvalue_7) (Collision|LineTraceByChannel _returnvalue_6 (+ _returnvalue_6 "0, 0,-500.000000") "TraceTypeQuery1" false (Utilities|Array|MakeArray self) "None"))
      (if _returnvalue_7
        (bind _returnvalue_8 (Game|SpawnActorfromClass "/Game/Scripts/Blueprints/SavingSystem/BP_Checkpoint.BP_Checkpoint_C" (Math|Transform|MakeTransform (.Location (Collision|BreakHitResult _outhit)) (Math|Rotator|MakeRotator 0.0 0.0 (+ (.yaw (Math|Rotator|FindLookatRotation (.Location (Collision|BreakHitResult _outhit)) (Transformation|GetActorLocation))) -9e+01)) "1,1,1") "Undefined" 0 0))
        (Variables|Default|SetCheckpoint _returnvalue_8)
        (LocalVariables|SetSuccess true)
        (else
          (Development|PrintString "Can not spawn the checkpoint: no floor detected in front of the character")
          (LocalVariables|SetSuccess false)))))
  (return (LocalVariables|GetSuccess)))

(fn UpdateMaxmovementSpeed
  (if (Variables|Default|GetIsBlocking)
    (Variables|/Script/Engine.CharacterMovementComponent|SetMaxWalkSpeed (Variables|Character|GetCharacterMovement) (Variables|Default|GetMaxSpeed_Block))
    (elif (Variables|Default|GetIsSprinting)
      (Variables|/Script/Engine.CharacterMovementComponent|SetMaxWalkSpeed (Variables|Character|GetCharacterMovement) (Variables|Default|GetMaxSpeed_Sprint))
      (else
        (Variables|/Script/Engine.CharacterMovementComponent|SetMaxWalkSpeed (Variables|Character|GetCharacterMovement) (Variables|Default|GetMaxSpeed_Default)))))
  (return))

(fn InitializeClass
  (CallFunction|InitializeGameplayEffectsbyMoveset)
  (CallFunction|UpdateWeaponsMeshandSockets))

(fn GetInteractionController
  (bind _asbp_player_conroller (Utilities|Casting|CastToBP_PlayerConroller (Game|GetPlayerController 0)))
  (return _asbp_player_conroller))