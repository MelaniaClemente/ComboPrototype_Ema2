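; Base character Blueprint for combat, with moveset-driven weapon meshes, sockets and sword-and-shield damage and block values.
; BPCombatComponent supplies animations and priority checks for directional rolls, combo attacks and the death montage triggered by health exhaustion.
; Helpers handle sphere-trace hits, damage, eight-way relative direction and spawning effects or team-tagged projectiles.
; Optional physical animation simulates bodies below a chosen bone, and interface-style getters provide mostly empty defaults.
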(event ParameterExhausted(BP_HealthComponent)
  (bind _controllerref (Variables|Default|GetControllerRef))
  (Utilities|IsValid _controllerref
    (:Is%20Valid
      (Input|SetIgnoreMoveInput _controllerref true)
      (Input|SetIgnoreLookInput _controllerref true)
      (Components|Movement|StopMovementImmediately (Variables|Character|GetCharacterMovement)))
    (:Is%20Not%20Valid
      _))
  (CallFunction|Death (Utilities|Array|Get(acopy) (Variables|/Game/Scripts/Blueprints/Components/Animation/BP_CombatComponent.BP_CombatComponent_C|GetSwordAndShield_Death (Variables|Default|GetBP_CombatComponent))))
  (Collision|SetCollisionResponsetoChannel (Variables|Collision|GetCapsuleComponent) "ECC_Pawn" "ECR_Ignore"))

(event EventBeginPlay
  (CallFunction|InitializePhysicalAnimation)
  (Variables|Default|SetControllerRef (.MyPlayerController (CallFunction|GetMyPlayerControllerbyInterface false self)))
  (switch Utilities|FlowControl|Switch|SwitchonENUM_Movesets (Variables|Default|GetMoveset)
    (:NewEnumerator0
      (Variables|Combat|Attack|SetWeaponTypeDamageMultiplier (Variables|/Game/Scripts/Blueprints/Components/Animation/BP_CombatComponent.BP_CombatComponent_C|GetSwordAndShieldDamageMultiplier (Variables|Default|GetBP_CombatComponent))))))

(event Collision|EventActorBeginOverlap
  (params (OtherActor :type Actor%20Object%20Reference)))

(event EventTick
  (params (DeltaSeconds :type Float%20%28single-precision%29)))

(event Input|KeyboardEvents|H
  (params (Key :type Key%20Structure))
  (:Pressed
    (CallFunction|SpawnProjectile "/Game/Scripts/Blueprints/Projectiles/BP_ProjectileMaster.BP_ProjectileMaster_C" 0 0 "0, 0, 0" "0, 0, 0" "1.000000,1.000000,1.000000" "0, 0, 0" 0.0)))

(fn ConstructionScript
  (CallFunction|UpdateWeaponsMeshandSockets))

(fn RollbyInput
  (bind _bp_combatcomponent (Variables|Default|GetBP_CombatComponent))
  (bind _controllerref (Variables|Default|GetControllerRef))
  (bind _returnvalue (Default|GetForwardCameraInputVector _controllerref))
  (bind _rollanimationlist (Variables|/Game/Scripts/Blueprints/Components/Animation/BP_CombatComponent.BP_CombatComponent_C|GetRollAnimationList _bp_combatcomponent))
  (bind _rollangle (Default|GetRollDirectionbyMovementInput _bp_combatcomponent (.x _returnvalue) (.y _returnvalue)))
  (bind _rolldirectionstring (Default|GetRollDirectionTypebyAngle _bp_combatcomponent _rollangle))
  (bind (_value _returnvalue_2) (Utilities|Map|Find _rollanimationlist _rolldirectionstring))
  (Variables|/Game/Scripts/Blueprints/Components/Animation/BP_CombatComponent.BP_CombatComponent_C|SetNextAnimation _bp_combatcomponent (Utilities|Array|Get(acopy) (Variables|/Game/Scripts/Blueprints/Components/Animation/BP_CombatComponent.BP_CombatComponent_C|GetRolls _bp_combatcomponent) _value))
  (bind _output_get (LocalVariables|SetSuccess (and (Default|CheckAnimationPriority _bp_combatcomponent) _returnvalue_2)))
  (if _output_get
    (Default|UpdateCurrentAnimation _bp_combatcomponent)
    (Default|PlayMontage (Variables|Default|GetBP_CombatComponent) "MontageLength" true))
  (return (LocalVariables|GetSuccess)))

(fn Death
  (params (NextAnimation :type STRUCT%20Gameplay%20Animations%20Structure))
  (bind _bp_combatcomponent (Variables|Default|GetBP_CombatComponent))
  (Variables|/Game/Scripts/Blueprints/Components/Animation/BP_CombatComponent.BP_CombatComponent_C|SetNextAnimation _bp_combatcomponent NextAnimation)
  (if (Default|CheckAnimationPriority _bp_combatcomponent)
    (bind _updatedcurrentanimation (Default|UpdateCurrentAnimation _bp_combatcomponent))
    (bind _montage (Default|PlayDynamicMontage _bp_combatcomponent _updatedcurrentanimation "FullBody"))
    (Variables|Combat|Attack|SetHighPriorityMontage _montage)))

(fn PlayNextAttack
  (bind _bp_combatcomponent (Variables|Default|GetBP_CombatComponent))
  (bind _montage (Default|PlayDynamicMontage _bp_combatcomponent (Variables|/Game/Scripts/Blueprints/Components/Animation/BP_CombatComponent.BP_CombatComponent_C|GetNextAnimation _bp_combatcomponent) "FullBody"))
  (Variables|Combat|Attack|SetHighPriorityMontage _montage)
  (Math|Integer|IncrementInt (Variables|/Game/Scripts/Blueprints/Components/Animation/BP_CombatComponent.BP_CombatComponent_C|GetComboCounter _bp_combatcomponent)
    (:%20%20
      (Variables|/Game/Scripts/Blueprints/Components/Animation/BP_CombatComponent.BP_CombatComponent_C|SetLastIncreaseComboTime _bp_combatcomponent (Utilities|Time|GetTimeSeconds))
      (return))))

(fn WeaponTrace
  (params (Radius :type Float%20%28single-precision%29) (ObjectTypes :type Array%20of%20EObjectTypeQuery%20Enums :default "ObjectTypeQuery1") (bTraceComplex :type Boolean) (DrawDebugType :type EDrawDebugTrace%20Enum :default "None") (bIgnoreSelf :type Boolean) (Start :type Vector) (End :type Vector))
  (bind (_outhit _returnvalue) (Collision|SphereTraceForObjects Start End Radius ObjectTypes bTraceComplex (Variables|Combat|Attack|GetActorsToIgnureDuringAttacks) DrawDebugType bIgnoreSelf))
  (return _outhit _returnvalue))

(fn SingleTargetAttack
  (params (Target%20Actor :type Actor%20Object%20Reference) (GameplayAction :type Array%20of%20STRUCT%20Game%20Actions%20Structures) (DamagerReductionDuringBlocking :type Float%20%28single-precision%29) (PrintDebugOnScreen :type Boolean))
  (CallFunction|SingleTargetAttack Target%20Actor GameplayAction (Variables|Combat|Attack|GetAttackTypeDamageMultiplier) (Variables|Combat|Attack|GetWeaponTypeDamageMultiplier) DamagerReductionDuringBlocking (Variables|Combat|GetBaseDamage) PrintDebugOnScreen))

(fn SpawnGameplayEffect
  (params (Class :type Actor%20Class%20Reference) (SpawnTransform :type Transform) (CollisionHandlingOverride :type ESpawnActorCollisionHandlingMethod%20Enum :default "Undefined"))
  (bind _returnvalue (Game|SpawnActorfromClass Class SpawnTransform CollisionHandlingOverride 0 0))
  (bind _asbp_gameplay_effect_master (Utilities|Casting|CastToBP_GameplayEffect_Master _returnvalue)
    (:then
      _)
    (:CastFailed
      _))
  (return _asbp_gameplay_effect_master))

(fn UpdateSocketLocationforAttackTrace
  (params (StartingSocket :type Name) (EndingSocket :type Name))
  (bind _mesh (Variables|Character|GetMesh))
  (Variables|Combat|Attack|SetSocketLocationsAttackTrace_Start (Transformation|GetSocketLocation _mesh StartingSocket))
  (Variables|Combat|Attack|SetSockeLocationAttackTrace_End (Transformation|GetSocketLocation _mesh EndingSocket)))

(fn GetSocketsLocations
  (params (Socket1 :type Name) (Socket2 :type Name))
  (bind _mesh (Variables|Character|GetMesh))
  (return (Transformation|GetSocketLocation _mesh Socket1) (Transformation|GetSocketLocation _mesh Socket2)))

(fn RollbyAngle
  (params (Angle :type Float%20%28single-precision%29))
  (bind _bp_combatcomponent (Variables|Default|GetBP_CombatComponent))
  (bind _rolldirectionstring (Default|GetRollDirectionTypebyAngle _bp_combatcomponent Angle))
  (bind _rollanimationlist (Variables|/Game/Scripts/Blueprints/Components/Animation/BP_CombatComponent.BP_CombatComponent_C|GetRollAnimationList _bp_combatcomponent))
  (bind (_value _returnvalue) (Utilities|Map|Find _rollanimationlist _rolldirectionstring))
  (Variables|/Game/Scripts/Blueprints/Components/Animation/BP_CombatComponent.BP_CombatComponent_C|SetNextAnimation _bp_combatcomponent (Utilities|Array|Get(acopy) (Variables|/Game/Scripts/Blueprints/Components/Animation/BP_CombatComponent.BP_CombatComponent_C|GetRolls _bp_combatcomponent) _value))
  (bind _output_get (LocalVariables|SetSuccess (and (Default|CheckAnimationPriority _bp_combatcomponent) _returnvalue)))
  (if _output_get
    (Default|UpdateCurrentAnimation _bp_combatcomponent)
    (Default|PlayDynamicMontage _bp_combatcomponent (Variables|/Game/Scripts/Blueprints/Components/Animation/BP_CombatComponent.BP_CombatComponent_C|GetCurrentAnimation _bp_combatcomponent) "FullBody"))
  (return (LocalVariables|GetSuccess)))

(fn InitializePhysicalAnimation
  (bind _physicalbonebelow (Variables|PhysicalAnimation|GetPhysicalBoneBelow))
  (bind _enablephysicalanimation_ (Variables|PhysicalAnimation|GetEnablePhysicalAnimation?))
  (if _enablephysicalanimation_
    (Class|PhysicalAnimationComponent|SetSkeletalMeshComponent (Variables|Default|GetPhysicalAnimation) (Variables|Character|GetMesh))
    (Class|PhysicalAnimationComponent|ApplyPhysicalAnimationSettingsBelow (Variables|Default|GetPhysicalAnimation) _physicalbonebelow (Variables|PhysicalAnimation|GetPhysicalAnimation%20Data) true)
    (Class|SkeletalMeshComponent|SetAllBodiesBelowSimulatePhysics (Variables|Character|GetMesh) _physicalbonebelow _enablephysicalanimation_ false)))

(fn GetRelativeDirectionbyActor
  (params (TargetActor :type Actor%20Object%20Reference) (StartActor :type Actor%20Object%20Reference))
  (return (CallFunction|GetDirectionbyAngle (.yaw (Math|Rotator|Delta(Rotator) (Transformation|GetActorRotation StartActor) (Math|Rotator|FindLookatRotation (Transformation|GetActorLocation StartActor) (Transformation|GetActorLocation TargetActor)))))))

(fn GetDirectionbyAngle
  (params (Angle :type Float%20%28single-precision%29))
  (return (select (Math|Float|InRange(Float) Angle -22.5 22.5) "NewEnumerator0" (select (Math|Float|InRange(Float) Angle -67.5 -22.5) "NewEnumerator1" (select (Math|Float|InRange(Float) Angle 22.5 67.5) "NewEnumerator2" (select (Math|Float|InRange(Float) Angle -112.5 -67.5) "NewEnumerator3" (select (Math|Float|InRange(Float) Angle 67.5 112.5) "NewEnumerator4" (select (Math|Float|InRange(Float) Angle -157.5 -112.5) "NewEnumerator5" (select (Math|Float|InRange(Float) Angle 112.5 157.5) "NewEnumerator6" "NewEnumerator7")))))))))

(fn UpdateBlockValuebyWeapon
  (switch Utilities|FlowControl|Switch|SwitchonENUM_Movesets (Variables|Default|GetMoveset)
    (:NewEnumerator0
      (Variables|Combat|SetBlockMultiplier (Variables|/Game/Scripts/Blueprints/Components/Animation/BP_CombatComponent.BP_CombatComponent_C|GetSwordAndShield_BlockValue (Variables|Default|GetBP_CombatComponent))))))

(fn GetBlockDamageReduction
  (switch Utilities|FlowControl|Switch|SwitchonENUM_Movesets (Variables|Default|GetMoveset)
    (:NewEnumerator0
      (LocalVariables|SetDamageReduction (Variables|/Game/Scripts/Blueprints/Components/Animation/BP_CombatComponent.BP_CombatComponent_C|GetSwordAndShield_BlockValue (Variables|Default|GetBP_CombatComponent)))
      (return (LocalVariables|GetDamageReduction)))))

(fn UpdateWeaponsMeshandSockets
  (bind _righthandequip (Variables|Default|GetRightHandEquip))
  (bind _lefthandequip (Variables|Default|GetLeftHandEquip))
  (switch Utilities|FlowControl|Switch|SwitchonENUM_Movesets (Variables|Default|GetMoveset)
    (:NewEnumerator0
      (Transformation|AttachComponentToComponent (Variables|Default|GetRightHandEquip) (Variables|Character|GetMesh) (Variables|Sockets|GetSwordSocketName) "KeepRelative" "KeepRelative" "KeepRelative" true)
      (Transformation|AttachComponentToComponent (Variables|Default|GetLeftHandEquip) (Variables|Character|GetMesh) (Variables|Sockets|GetShieldSocketName) "KeepRelative" "KeepRelative" "KeepRelative" true)
      (Components|StaticMesh|SetStaticMesh _righthandequip "/Game/Assets/StaticMeshes/Knight/Weapons/SM_Wep_Broadsword_01.SM_Wep_Broadsword_01")
      (Components|StaticMesh|SetStaticMesh _lefthandequip "/Game/Assets/StaticMeshes/Dungeon/Weapons/SM_Wep_Shield_Heater_02.SM_Wep_Shield_Heater_02"))
    (:NewEnumerator1
      (Transformation|AttachComponentToComponent (Variables|Default|GetRightHandEquip) (Variables|Character|GetMesh) (Variables|Sockets|GetArrowSocketName) "KeepRelative" "KeepRelative" "KeepRelative" true)
      (Transformation|AttachComponentToComponent (Variables|Default|GetLeftHandEquip) (Variables|Character|GetMesh) (Variables|Sockets|GetBowSocketName) "KeepRelative" "KeepRelative" "KeepRelative" true)
      (Components|StaticMesh|SetStaticMesh _righthandequip "/Game/Assets/StaticMeshes/Dungeon/Items/SM_item_Arrow_01.SM_item_Arrow_01")
      (Components|StaticMesh|SetStaticMesh _lefthandequip "/Game/Assets/StaticMeshes/Dungeon/Weapons/SM_Bow_Blockout.SM_Bow_Blockout"))))

(fn SpawnProjectile
  (params (Class :type Actor%20Class%20Reference) (Owner :type Actor%20Object%20Reference) (Instigator :type Pawn%20Object%20Reference) (Spawn%20Transform%20Location :type Vector) (Spawn%20Transform%20Rotation :type Rotator) (Spawn%20Transform%20Scale :type Vector :default "1.000000,1.000000,1.000000") (Direction :type Vector) (ImpulseStrenght :type Float%20%28single-precision%29))
  (bind _asbp_projectile_master (Utilities|SpawnProjectile Class (Math|Transform|MakeTransform Spawn%20Transform%20Location Spawn%20Transform%20Rotation Spawn%20Transform%20Scale) "AlwaysSpawn" Owner Instigator)
    (:CastSucceded
      (bind _output_get (LocalVariables|SetProjectile _asbp_projectile_master))
      (Utilities|IsValid _output_get
        (:Is%20Valid
          (Variables|/Game/Scripts/Blueprints/Projectiles/BP_ProjectileMaster.BP_ProjectileMaster_C|SetOwnerBaseDamage (LocalVariables|GetProjectile) (Variables|Combat|GetBaseDamage))
          (Variables|/Game/Scripts/Blueprints/Projectiles/BP_ProjectileMaster.BP_ProjectileMaster_C|SetOwnerShooter (LocalVariables|GetProjectile) self)
          (bind _id (CallFunction|GetTeamID))
          (Variables|/Game/Scripts/Blueprints/Projectiles/BP_ProjectileMaster.BP_ProjectileMaster_C|SetTeamID (LocalVariables|GetProjectile) _id)
          (Default|EnableMeshOverlap (LocalVariables|GetProjectile))
          (Default|SpawnGameplayEffect (LocalVariables|GetProjectile))
          (Default|ActivateProjectileImpulse (LocalVariables|GetProjectile) Direction ImpulseStrenght true))))))

(fn ToogleSprint
  (params (IsSprinting :type Boolean))
  (Variables|Default|SetIsSprinting IsSprinting))

(fn GetMyCharacterMaster
  (return self))

(fn GetMyEnemyCharacter
  (return 0))

(fn GetMyMasterAnimInstance
  (return 0))

(fn GetMyPlayerCharacter
  (return 0))

(fn GetMyPlayerController
  (return 0))

(fn GetTeamID
  (return "NewEnumerator0"))