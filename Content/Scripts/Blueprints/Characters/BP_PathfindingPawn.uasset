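; BP_PathfindingPawn is an AI pawn that travels along the navmesh to a target actor, leaving a sparkle-dust trail behind it.
; After a one-second delay on BeginPlay, it runs AI MoveTo toward ActorToFollow with continuous goal tracking, if that actor is valid.
; It destroys itself immediately if the request fails, or one second after the move finishes.
; Tick spawns a new dust emitter at its location every frame.
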(event EventBeginPlay
  (bind _actortofollow (Variables|Default|GetActorToFollow))
  (Variables|Default|SetStartingLocation (Transformation|GetActorLocation))
  (Utilities|FlowControl|Delay 1.0)
  (Utilities|IsValid _actortofollow
    (:Is%20Valid
      (AI|AIMoveTo (AI|GetAIController self) "0, 0, 0" _actortofollow 5e+01 "Disable" "Disable" true true true "Enable"
        (:OnRequestFailed
          _)
        (:OnMoveFinished
          (Utilities|FlowControl|Delay 1.0)))
      (Actor|DestroyActor))))

(event Collision|EventActorBeginOverlap
  (params (OtherActor :type Actor%20Object%20Reference)))

(event EventTick
  (params (DeltaSeconds :type Float%20%28single-precision%29))
  (Effects|SpawnEmitteratLocation "/Game/Assets/Particles/Trails/P_ky_trail_shineDust.P_ky_trail_shineDust" (Transformation|GetActorLocation)))

(fn ConstructionScript)