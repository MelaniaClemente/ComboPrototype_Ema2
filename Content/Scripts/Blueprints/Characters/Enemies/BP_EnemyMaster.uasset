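; Base enemy character that wires health, combat and AI combat logic components to a BP_AIController.
; Pawn sensing and health events drive an Idle/Combat/Death state, with sight also updating the controller's target lock and focus.
; Attack start and end adjust the player's aggro count, while timeline-animated pulse-ring material and swappable particles telegraph light and heavy attacks.
; Health bar and optional AI debug widget yaw toward the player camera every tick.
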(event OnSeePawn(PawnSensing)
  (params (Pawn :type Pawn%20Object%20Reference))
  (bind _aicontrollerref (Variables|Default|GetAIControllerRef))
  (if (not (Default|IsExhausted (Variables|Default|GetBP_HealthComponent)))
    (Utilities|IsValid Pawn
      (:Is%20Valid
        (bind _asbp_player_character (Utilities|Casting|CastToBP_PlayerCharacter Pawn))
        (Default|ProcessLastVision _aicontrollerref _asbp_player_character)
        (switch Utilities|FlowControl|Switch|SwitchonENUM_AIMainStates (Default|GetCurrentMainState _aicontrollerref)
          (:NewEnumerator0
            (Variables|/Game/Scripts/Blueprints/Controllers/AI/BP_AIController.BP_AIController_C|SetTargetLocked _aicontrollerref false)
            (Variables|/Game/Scripts/Blueprints/Controllers/AI/BP_AIController.BP_AIController_C|SetTargetToFocus _aicontrollerref 0))
          (:NewEnumerator3
            (Variables|/Game/Scripts/Blueprints/Controllers/AI/BP_AIController.BP_AIController_C|SetTargetLocked _aicontrollerref true)
            (Variables|/Game/Scripts/Blueprints/Controllers/AI/BP_AIController.BP_AIController_C|SetTargetToFocus _aicontrollerref _asbp_player_character))
          (:NewEnumerator4
            (Variables|/Game/Scripts/Blueprints/Controllers/AI/BP_AIController.BP_AIController_C|SetTargetToFocus _aicontrollerref 0))))
      (:Is%20Not%20Valid
        (Development|PrintString "Hello")
        (Variables|/Game/Scripts/Blueprints/Controllers/AI/BP_AIController.BP_AIController_C|SetTargetToFocus (Variables|Default|GetAIControllerRef) 0)
        (Variables|AI|SetMainState "NewEnumerator0")))
    (else
      (Variables|AI|SetMainState "NewEnumerator4"))))

(event OnConsume(BP_HealthComponent)
  (params (ValueToConsume :type Float%20%28single-precision%29) (PrintDebugToScreen :type Boolean))
  (if (not (Default|IsExhausted (Variables|Default|GetBP_HealthComponent)))
    (Variables|AI|SetMainState "NewEnumerator3")
    (else
      (Variables|AI|SetMainState "NewEnumerator4"))))

(event OnParameterExhausted(BP_HealthComponent)
  (Variables|AI|SetMainState "NewEnumerator4")
  (Rendering|SetVisibility (Variables|Default|GetHealthBar) false false))

(event OnHearNoise(PawnSensing)
  (params (Instigator :type Pawn%20Object%20Reference) (Location :type Vector%20%28by%20ref%29 :default "0, 0, 0") (Volume :type Float%20%28single-precision%29))
  (if (not (Default|IsExhausted (Variables|Default|GetBP_HealthComponent)))
    (Utilities|IsValid Instigator
      (:Is%20Valid
        (bind _asbp_player_character (Utilities|Casting|CastToBP_PlayerCharacter Instigator))
        (if (not (Default|IsExhausted (Variables|/Game/Scripts/Blueprints/Characters/BP_CharacterMaster.BP_CharacterMaster_C|GetBP_HealthComponent _asbp_player_character)))
          (Variables|AI|SetMainState "NewEnumerator3"))))
    (else
      (Variables|AI|SetMainState "NewEnumerator4"))))

(event OnAttackStart(BP_CombatComponent)
  (bind _asbp_character_master (Utilities|Casting|CastToBP_CharacterMaster (Game|GetPlayerCharacter 0)))
  (Default|IncrementAggro _asbp_character_master 1 self))

(event OnAttackEnd(BP_CombatComponent)
  (bind _asbp_character_master (Utilities|Casting|CastToBP_CharacterMaster (Game|GetPlayerCharacter 0)))
  (Default|DecrementAggro _asbp_character_master 1 self))

(event Custom|InitializeComponents
  (Default|Initialization (Variables|Default|GetBP_CombatComponent))
  (Default|Initialization (Variables|Default|GetBP_HealthComponent))
  (Default|Initialization (Variables|Default|GetBP_AICombatLogic))
  (CallFunction|InitializePulseRing))

(event Custom|PlayHeavyAttackAnticipationFeedback
  (Rendering|Material|SetVectorParameterValue (Variables|Default|GetPulseRingMaterial) "ColorRing" (Variables|Default|GetHeavyAttackAnticipationColor) :!class /Script/Engine.MaterialInstanceDynamic)
  (Development|SetHiddeninGame (Variables|Default|GetPulseRingPlane) false false)
  (bind _alpharadius (Timeline|Timeline_0 PlayFromStart)
    (:Update
      (Rendering|Material|SetScalarParameterValue (Variables|Default|GetPulseRingMaterial) "Radius" _alpharadius :!class /Script/Engine.MaterialInstanceDynamic))
    (:Finished
      (Development|SetHiddeninGame (Variables|Default|GetPulseRingPlane) true false))))

(event Custom|PlayLightAttackFeedback
  (Rendering|Material|SetVectorParameterValue (Variables|Default|GetPulseRingMaterial) "ColorRing" (Variables|Default|GetLightAttackAnticipationColor) :!class /Script/Engine.MaterialInstanceDynamic)
  (Development|SetHiddeninGame (Variables|Default|GetPulseRingPlane) false false)
  (bind _alpharadius (Timeline|PulseRingAnimation PlayFromStart)
    (:Update
      (Rendering|Material|SetScalarParameterValue (Variables|Default|GetPulseRingMaterial) "Radius" _alpharadius :!class /Script/Engine.MaterialInstanceDynamic))
    (:Finished
      (Development|SetHiddeninGame (Variables|Default|GetPulseRingPlane) true false))))

(event EventBeginPlay
  (|CallParentFunction)
  (CallFunction|Initialize3DWidget)
  (bind _asbp_aicontroller (Utilities|Casting|CastToBP_AIController (AI|GetAIController self)))
  (Variables|Default|SetAIControllerRef _asbp_aicontroller))

(event Collision|EventActorBeginOverlap
  (params (OtherActor :type Actor%20Object%20Reference))
  (|CallParentFunction OtherActor) ; This node is disabled and will not be called.\nDrag off pins to build functionality.
)

(event EventTick
  (params (DeltaSeconds :type Float%20%28single-precision%29))
  (|CallParentFunction DeltaSeconds)
  (CallFunction|Rotate3DWidgettoPlayer))

(fn ConstructionScript
  (|CallParentFunction))

(fn Initialize3DWidget
  (bind _bp_aicombatlogic (Variables|Default|GetBP_AICombatLogic))
  (bind _asbp_health_bar (Utilities|Casting|CastToBP_HealthBar (UserInterface|GetUserWidgetObject (Variables|Default|GetHealthBar)))
    (:then
      (Variables|/Game/Scripts/Blueprints/UI/CustomProgressBars/BP_HealthBar.BP_HealthBar_C|SetOwnerCharacter _asbp_health_bar self)
      (Default|Initialization _asbp_health_bar))
    (:CastFailed
      _))
  (bind _asbp_aistates (Utilities|Casting|CastToBP_AIStates (UserInterface|GetUserWidgetObject (Variables|Default|GetStateDebugWidget))))
  (Variables|/Game/Scripts/Blueprints/UI/Debug/BP_AIStates.BP_AIStates_C|SetAICombatLogic _asbp_aistates _bp_aicombatlogic)
  (if (Variables|/Game/Scripts/Blueprints/Components/AI/BP_AICombatLogic.BP_AICombatLogic_C|GetEnableStateDebug? _bp_aicombatlogic)
    (Widget|SetVisibility _asbp_aistates "Visible")
    (else
      (Widget|SetVisibility _asbp_aistates "Hidden"))))

(fn Rotate3DWidgettoPlayer
  (bind _returnvalue (Game|GetPlayerCharacter 0))
  (if (Utilities|DoesObjectImplementInterface _returnvalue "/Game/Scripts/Blueprints/Interfaces/BP_CharacterInterface.BP_CharacterInterface_C")
    (bind _newparam (Class|BPCharacterInterface|GetMyPlayerCharacter(Message) _returnvalue))
    (Transformation|SetWorldRotation (Variables|Default|GetHealthBar) (Math|Rotator|MakeRotator 0.0 0.0 (.yaw (Math|Rotator|FindLookatRotation (Transformation|GetWorldLocation (Variables|Default|GetHealthBar)) (Transformation|GetWorldLocation (Variables|/Game/Scripts/Blueprints/Characters/BP_PlayerCharacter.BP_PlayerCharacter_C|GetCamera _newparam))))) false false)
    (Transformation|SetWorldRotation (Variables|Default|GetStateDebugWidget) (Math|Rotator|MakeRotator 0.0 0.0 (.yaw (Math|Rotator|FindLookatRotation (Transformation|GetWorldLocation (Variables|Default|GetHealthBar)) (Transformation|GetWorldLocation (Variables|/Game/Scripts/Blueprints/Characters/BP_PlayerCharacter.BP_PlayerCharacter_C|GetCamera _newparam))))) false false)
    (Transformation|SetWorldRotation (Variables|Default|GetSpringArm) (Math|Rotator|MakeRotator 0.0 0.0 (.yaw (Math|Rotator|FindLookatRotation (Transformation|GetWorldLocation (Variables|Default|GetHealthBar)) (Transformation|GetWorldLocation (Variables|/Game/Scripts/Blueprints/Characters/BP_PlayerCharacter.BP_PlayerCharacter_C|GetCamera _newparam))))) false false)))

(fn GetMyEnemyCharacter
  (return self))

(fn GetTeamID
  (return "NewEnumerator1"))

(fn UpdateMovementSpeedbyPerceptionState
  (params (Idle :type Float%20%28single-precision%29) (Combat :type Float%20%28single-precision%29))
  (Variables|/Script/Engine.CharacterMovementComponent|SetMaxWalkSpeed (Variables|Character|GetCharacterMovement) (Utilities|Select :Index (Variables|AI|GetMainState) :NewEnumerator0 Idle :NewEnumerator3 Combat :NewEnumerator4 0.0)))

(fn GetMovementSpeedbyPerceptionState
  (return (Variables|Default|GetIdleSpeed) (Variables|Default|GetCombatSpeed)))

(fn GetDodgeDirectionbyTwoPoints
  (params (Start :type Vector%20%28by%20ref%29) (Target :type Vector%20%28by%20ref%29))
  (bind _dodgelocationarrow (Variables|Default|GetDodgeLocationArrow))
  (Transformation|SetWorldRotation _dodgelocationarrow (Math|Rotator|FindLookatRotation Start Target) false false)
  (return (.yaw (Variables|/Script/Engine.SceneComponent|GetRelativeRotation _dodgelocationarrow))))

(fn AcivateLightAttackAnticipation
  (bind _anticipationparticle (Variables|Default|GetAnticipationParticle))
  (Effects|Components|ParticleSystem|SetTemplate _anticipationparticle (Variables|Default|GetLightAttackAnticipationParticle))
  (Components|Activation|ToggleActive _anticipationparticle))

(fn AcivateHeavyAttackAnticipation
  (bind _anticipationparticle (Variables|Default|GetAnticipationParticle))
  (Effects|Components|ParticleSystem|SetTemplate _anticipationparticle (Variables|Default|GetHeavyAttackAnticipation))
  (Components|Activation|ToggleActive _anticipationparticle))

(fn InitializePulseRing
  (bind _returnvalue (Rendering|Material|CreateDynamicMaterialInstance (Variables|Default|GetPulseRingPlane) 0 "/Game/Scripts/Materials/Masters/Particles/MI_PulseRing.MI_PulseRing" "None" :!class /Script/Engine.PrimitiveComponent))
  (bind _output_get (Variables|Default|SetPulseRingMaterial _returnvalue))
  (Rendering|Material|SetMaterial (Variables|Default|GetPulseRingPlane) 0 _output_get))