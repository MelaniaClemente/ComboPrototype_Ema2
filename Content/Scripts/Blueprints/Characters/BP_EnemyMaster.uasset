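; Base enemy character Blueprint that randomizes its right-hand equipment mesh on construction and reports a fixed team ID.
; On BeginPlay it links the health bar and AI combat debug widgets to itself and its combat component.
; Each tick it yaws both widgets toward the player camera.
; Helpers set walk speed by Idle, Combat or Death state and derive dodge yaw from an arrow component, though the roll test is unwired.
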(event EventBeginPlay
  (|CallParentFunction)
  (CallFunction|Initialize3DWidget))

(event Collision|EventActorBeginOverlap
  (params (OtherActor :type Actor%20Object%20Reference))
  (|CallParentFunction OtherActor) ; This node is disabled and will not be called.\nDrag off pins to build functionality.
)

(event EventTick
  (params (DeltaSeconds :type Float%20%28single-precision%29))
  (|CallParentFunction DeltaSeconds)
  (CallFunction|Rotate3DWidgettoPlayer))

(fn ConstructionScript
  (bind _righthandequipmesh (Variables|Default|GetRightHandEquipMesh))
  (|CallParentFunction)
  (Components|StaticMesh|SetStaticMesh (Variables|Default|GetRightHandEquip) (Utilities|Array|Get(acopy) _righthandequipmesh (Math|Random|RandomIntegerinRange 0 (Utilities|Array|LastIndex _righthandequipmesh)))))

(fn Initialize3DWidget
  (bind _bp_aicombatlogic (Variables|Default|GetBP_AICombatLogic))
  (bind _asbp_health_bar (Utilities|Casting|CastToBP_HealthBar (UserInterface|GetUserWidgetObject (Variables|Default|GetHealthBar)))
    (:then
      (Variables|/Game/Scripts/Blueprints/UI/CustomProgressBars/BP_HealthBar.BP_HealthBar_C|SetOwnerCharacter _asbp_health_bar self))
    (:CastFailed
      _))
  (bind _asbp_aistate_debug (Utilities|Casting|CastToBP_AIStateDebug (UserInterface|GetUserWidgetObject (Variables|Default|GetStateDebugWidget))))
  (Variables|/Game/Scripts/Blueprints/UI/Debug/BP_AIStateDebug.BP_AIStateDebug_C|SetAICombatComponent _asbp_aistate_debug _bp_aicombatlogic)
  (if (Variables|/Game/Scripts/Blueprints/Components/AI/BP_AICombatLogic.BP_AICombatLogic_C|GetEnableStateDebug? _bp_aicombatlogic)
    (Widget|SetVisibility _asbp_aistate_debug "Visible")
    (else
      (Widget|SetVisibility _asbp_aistate_debug "Hidden"))))

(fn Rotate3DWidgettoPlayer
  (bind _returnvalue (Game|GetPlayerCharacter 0))
  (if (Utilities|DoesObjectImplementInterface _returnvalue "/Game/Scripts/Blueprints/Interfaces/BP_CharacterInterface.BP_CharacterInterface_C")
    (bind _newparam (Class|BPCharacterInterface|GetMyPlayerCharacter(Message) _returnvalue))
    (Transformation|SetWorldRotation (Variables|Default|GetHealthBar) (Math|Rotator|MakeRotator 0.0 0.0 (.yaw (Math|Rotator|FindLookatRotation (Transformation|GetWorldLocation (Variables|Default|GetHealthBar)) (Transformation|GetWorldLocation (Variables|/Game/Scripts/Blueprints/Characters/BP_PlayerCharacter.BP_PlayerCharacter_C|GetCamera _newparam))))) false false)
    (Transformation|SetWorldRotation (Variables|Default|GetStateDebugWidget) (Math|Rotator|MakeRotator 0.0 0.0 (.yaw (Math|Rotator|FindLookatRotation (Transformation|GetWorldLocation (Variables|Default|GetHealthBar)) (Transformation|GetWorldLocation (Variables|/Game/Scripts/Blueprints/Characters/BP_PlayerCharacter.BP_PlayerCharacter_C|GetCamera _newparam))))) false false)))

(fn GetMyEnemyCharacter
  (return self))

(fn GetTeamID
  (return "NewEnumerator1"))

(fn UpdateMovementSpeedbyPerceptionState
  (params (Idle :type Float%20%28single-precision%29) (Combat :type Float%20%28single-precision%29))
  (Variables|/Script/Engine.CharacterMovementComponent|SetMaxWalkSpeed (Variables|Character|GetCharacterMovement) (Utilities|Select :Index (Variables|AI|GetMainState) :NewEnumerator0 Idle :NewEnumerator3 Combat :NewEnumerator4 0.0)))

(fn GetMovementSpeedbyPerceptionState
  (return (Variables|Default|GetIdleSpeed) (Variables|Default|GetCombatSpeed)))

(fn GetDodgeDirectionbyTwoPoints
  (params (Start :type Vector%20%28by%20ref%29) (Target :type Vector%20%28by%20ref%29))
  (bind _dodgelocationarrow (Variables|Default|GetDodgeLocationArrow))
  (Transformation|SetWorldRotation _dodgelocationarrow (Math|Rotator|FindLookatRotation Start Target) false false)
  (return (.yaw (Variables|/Script/Engine.SceneComponent|GetRelativeRotation _dodgelocationarrow))))