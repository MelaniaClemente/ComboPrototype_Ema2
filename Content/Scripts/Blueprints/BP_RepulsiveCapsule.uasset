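; BP_RepulsiveCapsule is a capsule hazard that registers a hit on any BP_PlayerCharacter that overlaps it.
; On overlap it records itself as the player's attacker, sets the hit type, and forces a game attribute to the hyper armor component's minimum value.
; A looping timer started at BeginPlay targets a movement-speed increase event, which is currently empty.
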(event OnComponentBeginOverlap(Capsule)
  (params (OverlappedComponent :type Primitive%20Component%20Object%20Reference) (OtherActor :type Actor%20Object%20Reference) (OtherComp :type Primitive%20Component%20Object%20Reference) (OtherBodyIndex :type Integer) (bFromSweep :type Boolean) (SweepResult :type Hit%20Result%20Structure%20%28by%20ref%29))
  (bind _asbp_player_character (Utilities|Casting|CastToBP_PlayerCharacter OtherActor))
  (Variables|/Game/Scripts/Blueprints/Characters/BP_CharacterMaster.BP_CharacterMaster_C|SetAttackerActor _asbp_player_character self)
  (Variables|/Game/Scripts/Blueprints/Characters/BP_CharacterMaster.BP_CharacterMaster_C|SetLastHitType _asbp_player_character "NewEnumerator2")
  (CallFunction|ForceCurrentGameAttribute _asbp_player_character (Utilities|Struct|MakeSTRUCT_GameActions_new "NewEnumerator0" (Utilities|Array|MakeArray "NewEnumerator6") (Utilities|Array|MakeArray (Default|GetMinValue (Variables|/Game/Scripts/Blueprints/Characters/BP_CharacterMaster.BP_CharacterMaster_C|GetBP_HyperArmorComponent _asbp_player_character)))) false))

(event Custom|Increase%20movmenet%20speed)

(event EventBeginPlay
  (Utilities|Time|SetTimerbyEvent (delegate Custom|Increase%20movmenet%20speed) 3e+01 true))

(event Collision|EventActorBeginOverlap
  (params (OtherActor :type Actor%20Object%20Reference)))

(event EventTick
  (params (DeltaSeconds :type Float%20%28single-precision%29)))

(fn ConstructionScript)