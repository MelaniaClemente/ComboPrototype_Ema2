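; BP_ExampleFogInteractor is an example actor that feeds its location to an indexed custom source position in a fog post-process material.
; UpdateFog runs on construction and every Tick, acting only when the referenced PostProcessVolume and its blendable at MaterialIndex are valid.
; Each update creates a new dynamic instance of BaseMaterial, sets the FogIndex-prefixed vector parameter, and replaces that blendable with it.
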(event EventTick
  (params (DeltaSeconds :type Float%20%28single-precision%29))
  (CallFunction|UpdateFog))

(fn ConstructionScript
  (CallFunction|UpdateFog))

(fn UpdateFog
  (Utilities|IsValid (Variables|Default|GetPostProcessVolume)
    (:Is%20Valid
      (Utilities|IsValid (.Object (Utilities|Struct|BreakWeightedBlendable (CallFunction|GetBlendable)))
        (:Is%20Valid
          (bind _returnvalue (Rendering|Material|CreateDynamicMaterialInstance (Variables|Default|GetBaseMaterial) "None" :!class /Script/Engine.KismetMaterialLibrary))
          (bind _asmaterial_instance_dynamic (Utilities|Casting|CastToMaterialInstanceDynamic _returnvalue))
          (Rendering|Material|SetVectorParameterValue _asmaterial_instance_dynamic (Utilities|String|StringToName (Utilities|String|ToString(Text) (Utilities|Text|FormatText "{Index} CustomSourcePosition" (Variables|Default|GetFogIndex)))) (Math|Conversions|ToLinearColor(Vector) (Transformation|GetActorLocation)) :!class /Script/Engine.MaterialInstanceDynamic)
          (Utilities|Struct|SetmembersinWeightedBlendable (Utilities|Array|Get(acopy) (Utilities|Struct|BreakWeightedBlendables (Utilities|Struct|BreakPostProcessSettings (Variables|/Script/Engine.PostProcessVolume|GetSettings (Variables|Default|GetPostProcessVolume)))) (Variables|Default|GetMaterialIndex)) _returnvalue))))))

(fn GetBlendable
  (return (Utilities|Array|Get(acopy) (Utilities|Struct|BreakWeightedBlendables (Utilities|Struct|BreakPostProcessSettings (Variables|/Script/Engine.PostProcessVolume|GetSettings (Variables|Default|GetPostProcessVolume)))) (Variables|Default|GetMaterialIndex))))