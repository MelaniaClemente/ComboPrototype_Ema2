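; BP_DebugMessages is a Blueprint function library of debug prints and interface-checked getters for the player controller, player character and master character.
; Message functions print errors for blocked attribute consume or restore, invalid objects and objects lacking BP_CharacterInterface, with optional screen output.
; Each getter tests the target, or its controller for the player controller lookup, for BP_CharacterInterface, then returns the interface message result or prints the missing-interface error.
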(fn DebugMsgCantConsumeAttribute
  (params (TextColor :type Linear%20Color%20Structure :default "(R=1.000000,G=0.000000,B=0.000000,A=1.000000)") (Duration :type Float%20%28single-precision%29) (bPrintToScreen :type Boolean))
  (Development|PrintString 0 "Error: The Attribute Can not be consumed: bCanBeConsumed is set to false. The Game Attribute will not be modified." bPrintToScreen true TextColor Duration))

(fn DebugMsgCantRestoreAttribute
  (params (TextColor :type Linear%20Color%20Structure :default "(R=1.000000,G=0.000000,B=0.000000,A=1.000000)") (Duration :type Float%20%28single-precision%29) (bPrintToScreen :type Boolean))
  (Development|PrintString 0 "Error: The Attribute Can not be restore: bCanBeRestored is set to false. The Game Attribute will not be modified." bPrintToScreen true TextColor Duration))

(fn DebugMsgDoesNotImplementCharacterInterface
  (params (Object :type Object%20Object%20Reference) (bPrintToScreen :type Boolean))
  (Development|PrintString (LocalVariables|Get__WorldContext) (Utilities|String|Append "EROOR:" (Utilities|GetObjectName Object) "Does not implement the Character interface.") bPrintToScreen true "(R=1.000000,G=0.000000,B=0.000000,A=1.000000)"))

(fn GetMyPlayerControllerbyInterface
  (params (bPrintToScreen :type Boolean) (Target :type Pawn%20Object%20Reference))
  (bind _returnvalue (Pawn|GetController Target))
  (if (Utilities|DoesObjectImplementInterface _returnvalue "/Game/Scripts/Blueprints/Interfaces/BP_CharacterInterface.BP_CharacterInterface_C")
    (bind _myplayercontroller (Class|BPCharacterInterface|GetMyPlayerController(Message) _returnvalue))
    (else
      (CallFunction|DebugMsgDoesNotImplementCharacterInterface _returnvalue bPrintToScreen (LocalVariables|Get__WorldContext))))
  (return false _myplayercontroller))

(fn GetMyPlayerCharacterbyInterface
  (params (bPrintToScreen :type Boolean) (Target :type Actor%20Object%20Reference))
  (if (Utilities|DoesObjectImplementInterface Target "/Game/Scripts/Blueprints/Interfaces/BP_CharacterInterface.BP_CharacterInterface_C")
    (bind _newparam (Class|BPCharacterInterface|GetMyPlayerCharacter(Message) Target))
    (else
      (CallFunction|DebugMsgDoesNotImplementCharacterInterface Target bPrintToScreen (LocalVariables|Get__WorldContext))))
  (return _newparam))

(fn GetMyCharacterMasterbyInterface
  (params (bPrintToScreen :type Boolean) (Target :type Actor%20Object%20Reference))
  (if (Utilities|DoesObjectImplementInterface Target "/Game/Scripts/Blueprints/Interfaces/BP_CharacterInterface.BP_CharacterInterface_C")
    (bind _charactermaster (Class|BPCharacterInterface|GetMyCharacterMaster(Message) Target))
    (else
      (CallFunction|DebugMsgDoesNotImplementCharacterInterface Target bPrintToScreen (LocalVariables|Get__WorldContext))))
  (return _charactermaster))

(fn DebugMsgUnvalidObject
  (params (Object :type Object%20Object%20Reference) (bPrintToScreen :type Boolean))
  (Development|PrintString (LocalVariables|Get__WorldContext) (Utilities|String|Append "ERROR:" (Utilities|GetObjectName Object) " is not valid") bPrintToScreen true "(R=1.000000,G=0.000000,B=0.000000,A=1.000000)"))