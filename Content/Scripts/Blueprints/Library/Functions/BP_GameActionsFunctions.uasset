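; Blueprint function library that applies data-driven gameplay actions to actors' Health and Stamina components, with helpers to clamp and compare attributes.
; SingleTargetGameplayAction dispatches an action struct to force, consume, restore or configure attributes, padding short value arrays with their last entry.
; Line, sphere and box trace wrappers feed hit actors into it, and SingleTargetAttack feeds it multiplier-scaled values.
; SetModifierPerSecondGameAttribute calls RestoreValue for Health instead of setting its modifier.
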(fn ClampGameAttribute
  (params (GameAttribute :type STRUCT%20Game%20Attribute%20Structure))
  (LocalVariables|SetCurrentClampedValue (Math|Float|Clamp(Float) (.currentvalue GameAttribute) (.minvalue GameAttribute) (.maxvalue GameAttribute)))
  (return (Utilities|Struct|MakeSTRUCT_GameAttribute (.minvalue GameAttribute) (.maxvalue GameAttribute) (.startvalue GameAttribute) (LocalVariables|GetCurrentClampedValue) (.modifierpersecond GameAttribute) (.bcanbeconsumed GameAttribute) (.bcanberestored GameAttribute))))

(fn CompareCurrentGameAttribute
  (params (ValueToCompare :type ENUM_CompareNumbers%20Enum :default "NewEnumerator0") (GameAttribute :type STRUCT%20Game%20Attribute%20Structure) (Value :type Float%20%28single-precision%29))
  (return (Utilities|Select :Index ValueToCompare :NewEnumerator0 (> (.currentvalue GameAttribute) Value) :NewEnumerator1 (>= (.currentvalue GameAttribute) Value) :NewEnumerator2 (< (.currentvalue GameAttribute) Value) :NewEnumerator3 (<= (.currentvalue GameAttribute) Value) :NewEnumerator4 (== (.currentvalue GameAttribute) Value))))

(fn GetGameAttributePercentageValue
  (params (GameAttribute :type STRUCT%20Game%20Attribute%20Structure))
  (if (> (.maxvalue GameAttribute) 0.0)
    (return (/ (.currentvalue GameAttribute) (.maxvalue GameAttribute)))))

(fn ForceCurrentGameAttribute
  (params (Target%20Actor :type Actor%20Object%20Reference) (GameActionsStruct :type STRUCT%20Game%20Actions%20Structure) (PrintDebugToScreen :type Boolean))
  (bind (_gameplayaction _gameparametersinfluenced _gameparameter_floatvalues) (Utilities|Struct|BreakSTRUCT_GameActions GameActionsStruct))
  (bind _output_get (LocalVariables|SetLocalValueArray _gameparameter_floatvalues))
  (if (>= (Utilities|Array|Length _output_get) 1)
    _
    (else
      (Utilities|Array|Add (LocalVariables|GetLocalValueArray) 0.0)))
  (LocalVariables|SetPrintDebug PrintDebugToScreen)
  (bind _output_get_2 (LocalVariables|SetActor Target%20Actor))
  (Utilities|IsValid _output_get_2
    (:Is%20Valid
      (for (_array_element _array_index) _gameparametersinfluenced
        (if (Utilities|Array|IsValidIndex (LocalVariables|GetLocalValueArray) _array_index)
          _
          (else
            (Utilities|Array|Add (LocalVariables|GetLocalValueArray) (Utilities|Array|Get(acopy) (LocalVariables|GetLocalValueArray) (- _array_index 1)))))
        (LocalVariables|SetValueLocal (Utilities|Array|Get(acopy) (LocalVariables|GetLocalValueArray) _array_index))
        (switch Utilities|FlowControl|Switch|SwitchonENUM_GameParameterType _array_element
          (:NewEnumerator0
            (Utilities|IsValid (Actor|GetComponentbyClass (LocalVariables|GetActor) "/Game/Scripts/Blueprints/Components/GameParameters/Childs/BP_HealthComponent.BP_HealthComponent_C")
              (:Is%20Valid
                (Default|SetCurrentValue (Actor|GetComponentbyClass (LocalVariables|GetActor) "/Game/Scripts/Blueprints/Components/GameParameters/Childs/BP_HealthComponent.BP_HealthComponent_C") (LocalVariables|GetValueLocal)))
              (:Is%20Not%20Valid
                (Development|PrintString 0 "ERROR: Can't find the right GameParameters Component in ForceCurrentGameAttribute function." (LocalVariables|GetPrintDebug) true "(R=1.000000,G=0.000000,B=0.000000,A=1.000000)" :!label _label))))
          (:NewEnumerator1
            (Utilities|IsValid (Actor|GetComponentbyClass (LocalVariables|GetActor) "/Game/Scripts/Blueprints/Components/GameParameters/Childs/BP_StaminaComponent.BP_StaminaComponent_C")
              (:Is%20Valid
                (Default|SetCurrentValue (Actor|GetComponentbyClass (LocalVariables|GetActor) "/Game/Scripts/Blueprints/Components/GameParameters/Childs/BP_StaminaComponent.BP_StaminaComponent_C") (LocalVariables|GetValueLocal)))
              (:Is%20Not%20Valid
                (goto _label)))))))
    (:Is%20Not%20Valid
      (Development|PrintString 0 "ERROR: Actor target missing in ForceCurrentGameAttribute function" (LocalVariables|GetPrintDebug)))))

(fn SetMinGameAttribute
  (params (Target%20Actor :type Actor%20Object%20Reference) (GameActionsStruct :type STRUCT%20Game%20Actions%20Structure) (PrintDebugToScreen :type Boolean))
  (bind (_gameplayaction _gameparametersinfluenced _gameparameter_floatvalues) (Utilities|Struct|BreakSTRUCT_GameActions GameActionsStruct))
  (bind _output_get (LocalVariables|SetLocalValueArray _gameparameter_floatvalues))
  (if (>= (Utilities|Array|Length _output_get) 1)
    _
    (else
      (Utilities|Array|Add (LocalVariables|GetLocalValueArray) 0.0)))
  (LocalVariables|SetPrintDebug PrintDebugToScreen)
  (bind _output_get_2 (LocalVariables|SetActor Target%20Actor))
  (Utilities|IsValid _output_get_2
    (:Is%20Valid
      (for (_array_element _array_index) _gameparametersinfluenced
        (if (Utilities|Array|IsValidIndex (LocalVariables|GetLocalValueArray) _array_index)
          _
          (else
            (Utilities|Array|Add (LocalVariables|GetLocalValueArray) (Utilities|Array|Get(acopy) (LocalVariables|GetLocalValueArray) (- _array_index 1)))))
        (LocalVariables|SetValueLocal (Utilities|Array|Get(acopy) (LocalVariables|GetLocalValueArray) _array_index))
        (switch Utilities|FlowControl|Switch|SwitchonENUM_GameParameterType _array_element
          (:NewEnumerator0
            (Utilities|IsValid (Actor|GetComponentbyClass (LocalVariables|GetActor) "/Game/Scripts/Blueprints/Components/GameParameters/Childs/BP_HealthComponent.BP_HealthComponent_C")
              (:Is%20Valid
                (Default|SetMinValue (Actor|GetComponentbyClass (LocalVariables|GetActor) "/Game/Scripts/Blueprints/Components/GameParameters/Childs/BP_HealthComponent.BP_HealthComponent_C") (LocalVariables|GetValueLocal)))
              (:Is%20Not%20Valid
                (Development|PrintString 0 "ERROR: Can't find the right GameParameters Component in SetMinGameAttribute function." (LocalVariables|GetPrintDebug) true "(R=1.000000,G=0.000000,B=0.000000,A=1.000000)" :!label _label))))
          (:NewEnumerator1
            (Utilities|IsValid (Actor|GetComponentbyClass (LocalVariables|GetActor) "/Game/Scripts/Blueprints/Components/GameParameters/Childs/BP_StaminaComponent.BP_StaminaComponent_C")
              (:Is%20Valid
                (Default|SetMinValue (Actor|GetComponentbyClass (LocalVariables|GetActor) "/Game/Scripts/Blueprints/Components/GameParameters/Childs/BP_StaminaComponent.BP_StaminaComponent_C") (LocalVariables|GetValueLocal)))
              (:Is%20Not%20Valid
                (goto _label)))))))
    (:Is%20Not%20Valid
      (Development|PrintString 0 "ERROR: Actor target missing in SetMinGameAttribute function" (LocalVariables|GetPrintDebug)))))

(fn SetMaxGameAttribute
  (params (Target%20Actor :type Actor%20Object%20Reference) (GameActionsStruct :type STRUCT%20Game%20Actions%20Structure) (PrintDebugToScreen :type Boolean))
  (bind (_gameplayaction _gameparametersinfluenced _gameparameter_floatvalues) (Utilities|Struct|BreakSTRUCT_GameActions GameActionsStruct))
  (bind _output_get (LocalVariables|SetLocalValueArray _gameparameter_floatvalues))
  (if (>= (Utilities|Array|Length _output_get) 1)
    _
    (else
      (Utilities|Array|Add (LocalVariables|GetLocalValueArray) 0.0)))
  (LocalVariables|SetPrintDebug PrintDebugToScreen)
  (bind _output_get_2 (LocalVariables|SetActor Target%20Actor))
  (Utilities|IsValid _output_get_2
    (:Is%20Valid
      (for (_array_element _array_index) _gameparametersinfluenced
        (if (Utilities|Array|IsValidIndex (LocalVariables|GetLocalValueArray) _array_index)
          _
          (else
            (Utilities|Array|Add (LocalVariables|GetLocalValueArray) (Utilities|Array|Get(acopy) (LocalVariables|GetLocalValueArray) (- _array_index 1)))))
        (LocalVariables|SetValueLocal (Utilities|Array|Get(acopy) (LocalVariables|GetLocalValueArray) _array_index))
        (switch Utilities|FlowControl|Switch|SwitchonENUM_GameParameterType _array_element
          (:NewEnumerator0
            (Utilities|IsValid (Actor|GetComponentbyClass (LocalVariables|GetActor) "/Game/Scripts/Blueprints/Components/GameParameters/Childs/BP_HealthComponent.BP_HealthComponent_C")
              (:Is%20Valid
                (Default|SetMaxValue (Actor|GetComponentbyClass (LocalVariables|GetActor) "/Game/Scripts/Blueprints/Components/GameParameters/Childs/BP_HealthComponent.BP_HealthComponent_C") (LocalVariables|GetValueLocal)))
              (:Is%20Not%20Valid
                (Development|PrintString 0 "ERROR: Can't find the right GameParameters Component in SetMaxGameAttribute function." (LocalVariables|GetPrintDebug) true "(R=1.000000,G=0.000000,B=0.000000,A=1.000000)" :!label _label))))
          (:NewEnumerator1
            (Utilities|IsValid (Actor|GetComponentbyClass (LocalVariables|GetActor) "/Game/Scripts/Blueprints/Components/GameParameters/Childs/BP_StaminaComponent.BP_StaminaComponent_C")
              (:Is%20Valid
                (Default|SetMaxValue (Actor|GetComponentbyClass (LocalVariables|GetActor) "/Game/Scripts/Blueprints/Components/GameParameters/Childs/BP_StaminaComponent.BP_StaminaComponent_C") (LocalVariables|GetValueLocal)))
              (:Is%20Not%20Valid
                (goto _label)))))))
    (:Is%20Not%20Valid
      (Development|PrintString 0 "ERROR: Actor target missing in SetMaxGameAttribute function" (LocalVariables|GetPrintDebug)))))

(fn ConsumeGameAttribute
  (params (Target%20Actor :type Actor%20Object%20Reference) (GameActionsStruct :type STRUCT%20Game%20Actions%20Structure) (PrintDebugToScreen :type Boolean))
  (bind (_gameplayaction _gameparametersinfluenced _gameparameter_floatvalues) (Utilities|Struct|BreakSTRUCT_GameActions GameActionsStruct))
  (bind _output_get (LocalVariables|SetLocalValueArray _gameparameter_floatvalues))
  (if (>= (Utilities|Array|Length _output_get) 1)
    _
    (else
      (Utilities|Array|Add (LocalVariables|GetLocalValueArray) 0.0)))
  (LocalVariables|SetPrintDebug PrintDebugToScreen)
  (bind _output_get_2 (LocalVariables|SetActor Target%20Actor))
  (Utilities|IsValid _output_get_2
    (:Is%20Valid
      (for (_array_element _array_index) _gameparametersinfluenced
        (if (Utilities|Array|IsValidIndex (LocalVariables|GetLocalValueArray) _array_index)
          _
          (else
            (Utilities|Array|Add (LocalVariables|GetLocalValueArray) (Utilities|Array|Get(acopy) (LocalVariables|GetLocalValueArray) (- _array_index 1)))))
        (LocalVariables|SetValueLocal (Utilities|Array|Get(acopy) (LocalVariables|GetLocalValueArray) _array_index))
        (switch Utilities|FlowControl|Switch|SwitchonENUM_GameParameterType _array_element
          (:NewEnumerator0
            (Utilities|IsValid (Actor|GetComponentbyClass (LocalVariables|GetActor) "/Game/Scripts/Blueprints/Components/GameParameters/Childs/BP_HealthComponent.BP_HealthComponent_C")
              (:Is%20Valid
                (Default|ConsumeValue (Actor|GetComponentbyClass (LocalVariables|GetActor) "/Game/Scripts/Blueprints/Components/GameParameters/Childs/BP_HealthComponent.BP_HealthComponent_C") (LocalVariables|GetValueLocal) (LocalVariables|GetPrintDebug)))
              (:Is%20Not%20Valid
                (Development|PrintString 0 "ERROR: Can't find the right GameParameters Component in ConsumeGameAttribute function." (LocalVariables|GetPrintDebug) true "(R=1.000000,G=0.000000,B=0.000000,A=1.000000)" :!label _label))))
          (:NewEnumerator1
            (Utilities|IsValid (Actor|GetComponentbyClass (LocalVariables|GetActor) "/Game/Scripts/Blueprints/Components/GameParameters/Childs/BP_StaminaComponent.BP_StaminaComponent_C")
              (:Is%20Valid
                (Default|ConsumeValue (Actor|GetComponentbyClass (LocalVariables|GetActor) "/Game/Scripts/Blueprints/Components/GameParameters/Childs/BP_StaminaComponent.BP_StaminaComponent_C") (LocalVariables|GetValueLocal) (LocalVariables|GetPrintDebug)))
              (:Is%20Not%20Valid
                (goto _label)))))))
    (:Is%20Not%20Valid
      (Development|PrintString 0 "ERROR: Actor target missing in ConsumeGameAttribute function" (LocalVariables|GetPrintDebug)))))

(fn RestoreGameAttribute
  (params (Target%20Actor :type Actor%20Object%20Reference) (GameActionsStruct :type STRUCT%20Game%20Actions%20Structure) (PrintDebugToScreen :type Boolean))
  (bind (_gameplayaction _gameparametersinfluenced _gameparameter_floatvalues) (Utilities|Struct|BreakSTRUCT_GameActions GameActionsStruct))
  (bind _output_get (LocalVariables|SetLocalValueArray _gameparameter_floatvalues))
  (if (>= (Utilities|Array|Length _output_get) 1)
    _
    (else
      (Utilities|Array|Add (LocalVariables|GetLocalValueArray) 0.0)))
  (LocalVariables|SetPrintDebug PrintDebugToScreen)
  (bind _output_get_2 (LocalVariables|SetActor Target%20Actor))
  (Utilities|IsValid _output_get_2
    (:Is%20Valid
      (for (_array_element _array_index) _gameparametersinfluenced
        (if (Utilities|Array|IsValidIndex (LocalVariables|GetLocalValueArray) _array_index)
          _
          (else
            (Utilities|Array|Add (LocalVariables|GetLocalValueArray) (Utilities|Array|Get(acopy) (LocalVariables|GetLocalValueArray) (- _array_index 1)))))
        (LocalVariables|SetValueLocal (Utilities|Array|Get(acopy) (LocalVariables|GetLocalValueArray) _array_index))
        (switch Utilities|FlowControl|Switch|SwitchonENUM_GameParameterType _array_element
          (:NewEnumerator0
            (Utilities|IsValid (Actor|GetComponentbyClass (LocalVariables|GetActor) "/Game/Scripts/Blueprints/Components/GameParameters/Childs/BP_HealthComponent.BP_HealthComponent_C")
              (:Is%20Valid
                (Default|RestoreValue (Actor|GetComponentbyClass (LocalVariables|GetActor) "/Game/Scripts/Blueprints/Components/GameParameters/Childs/BP_HealthComponent.BP_HealthComponent_C") (LocalVariables|GetValueLocal) (LocalVariables|GetPrintDebug)))
              (:Is%20Not%20Valid
                (Development|PrintString 0 "ERROR: Can't find the right GameParameters Component in RestoreGameAttribute function." (LocalVariables|GetPrintDebug) true "(R=1.000000,G=0.000000,B=0.000000,A=1.000000)" :!label _label))))
          (:NewEnumerator1
            (Utilities|IsValid (Actor|GetComponentbyClass (LocalVariables|GetActor) "/Game/Scripts/Blueprints/Components/GameParameters/Childs/BP_StaminaComponent.BP_StaminaComponent_C")
              (:Is%20Valid
                (Default|RestoreValue (Actor|GetComponentbyClass (LocalVariables|GetActor) "/Game/Scripts/Blueprints/Components/GameParameters/Childs/BP_StaminaComponent.BP_StaminaComponent_C") (LocalVariables|GetValueLocal) (LocalVariables|GetPrintDebug)))
              (:Is%20Not%20Valid
                (goto _label)))))))
    (:Is%20Not%20Valid
      (Development|PrintString 0 "ERROR: Actor target missing in RestoreGameAttribute function" (LocalVariables|GetPrintDebug)))))

(fn SetModifierPerSecondGameAttribute
  (params (Target%20Actor :type Actor%20Object%20Reference) (GameActionsStruct :type STRUCT%20Game%20Actions%20Structure) (PrintDebugToScreen :type Boolean))
  (bind (_gameplayaction _gameparametersinfluenced _gameparameter_floatvalues) (Utilities|Struct|BreakSTRUCT_GameActions GameActionsStruct))
  (bind _output_get (LocalVariables|SetLocalValueArray _gameparameter_floatvalues))
  (if (>= (Utilities|Array|Length _output_get) 1)
    _
    (else
      (Utilities|Array|Add (LocalVariables|GetLocalValueArray) 0.0)))
  (LocalVariables|SetPrintDebug PrintDebugToScreen)
  (bind _output_get_2 (LocalVariables|SetActor Target%20Actor))
  (Utilities|IsValid _output_get_2
    (:Is%20Valid
      (for (_array_element _array_index) _gameparametersinfluenced
        (if (Utilities|Array|IsValidIndex (LocalVariables|GetLocalValueArray) _array_index)
          _
          (else
            (Utilities|Array|Add (LocalVariables|GetLocalValueArray) (Utilities|Array|Get(acopy) (LocalVariables|GetLocalValueArray) (- _array_index 1)))))
        (LocalVariables|SetValueLocal (Utilities|Array|Get(acopy) (LocalVariables|GetLocalValueArray) _array_index))
        (switch Utilities|FlowControl|Switch|SwitchonENUM_GameParameterType _array_element
          (:NewEnumerator0
            (Utilities|IsValid (Actor|GetComponentbyClass (LocalVariables|GetActor) "/Game/Scripts/Blueprints/Components/GameParameters/Childs/BP_HealthComponent.BP_HealthComponent_C")
              (:Is%20Valid
                (Default|RestoreValue (Actor|GetComponentbyClass (LocalVariables|GetActor) "/Game/Scripts/Blueprints/Components/GameParameters/Childs/BP_HealthComponent.BP_HealthComponent_C") (LocalVariables|GetValueLocal) (LocalVariables|GetPrintDebug)))
              (:Is%20Not%20Valid
                (Development|PrintString 0 "ERROR: Can't find the right GameParameters Component in SetModifierPerSecondGameAttribute function." (LocalVariables|GetPrintDebug) true "(R=1.000000,G=0.000000,B=0.000000,A=1.000000)" :!label _label))))
          (:NewEnumerator1
            (Utilities|IsValid (Actor|GetComponentbyClass (LocalVariables|GetActor) "/Game/Scripts/Blueprints/Components/GameParameters/Childs/BP_StaminaComponent.BP_StaminaComponent_C")
              (:Is%20Valid
                (Default|SetModifierPerSecond (Actor|GetComponentbyClass (LocalVariables|GetActor) "/Game/Scripts/Blueprints/Components/GameParameters/Childs/BP_StaminaComponent.BP_StaminaComponent_C") (LocalVariables|GetValueLocal)))
              (:Is%20Not%20Valid
                (goto _label)))))))
    (:Is%20Not%20Valid
      (Development|PrintString 0 "ERROR: Actor target missing in SetModifierPerSecondGameAttribute function" (LocalVariables|GetPrintDebug)))))

(fn SetCanbeConsumed
  (params (Target%20Actor :type Actor%20Object%20Reference) (GameActionsStruct :type STRUCT%20Game%20Actions%20Structure) (PrintDebugToScreen :type Boolean))
  (bind (_gameplayaction _gameparametersinfluenced _gameparameter_floatvalues _gameparameters_boolvalues) (Utilities|Struct|BreakSTRUCT_GameActions GameActionsStruct))
  (bind _output_get (LocalVariables|SetLocalBoolArray _gameparameters_boolvalues))
  (if (>= (Utilities|Array|Length _output_get) 1)
    _
    (else
      (Utilities|Array|Add (LocalVariables|GetLocalBoolArray) true)))
  (LocalVariables|SetPrintDebug PrintDebugToScreen)
  (bind _output_get_2 (LocalVariables|SetActor Target%20Actor))
  (Utilities|IsValid _output_get_2
    (:Is%20Valid
      (for (_array_element _array_index) _gameparametersinfluenced
        (if (Utilities|Array|IsValidIndex (LocalVariables|GetLocalBoolArray) _array_index)
          _
          (else
            (Utilities|Array|Add (LocalVariables|GetLocalBoolArray) (Utilities|Array|Get(acopy) (LocalVariables|GetLocalBoolArray) (- _array_index 1)))))
        (LocalVariables|SetLocalBool (Utilities|Array|Get(acopy) (LocalVariables|GetLocalBoolArray) _array_index))
        (switch Utilities|FlowControl|Switch|SwitchonENUM_GameParameterType _array_element
          (:NewEnumerator0
            (Utilities|IsValid (Actor|GetComponentbyClass (LocalVariables|GetActor) "/Game/Scripts/Blueprints/Components/GameParameters/Childs/BP_HealthComponent.BP_HealthComponent_C")
              (:Is%20Valid
                (Default|SetCanbeConsumedValue (Actor|GetComponentbyClass (LocalVariables|GetActor) "/Game/Scripts/Blueprints/Components/GameParameters/Childs/BP_HealthComponent.BP_HealthComponent_C") (LocalVariables|GetLocalBool)))
              (:Is%20Not%20Valid
                (Development|PrintString 0 "ERROR: Can't find the right GameParameters Component in SetModifierPerSecondGameAttribute function." (LocalVariables|GetPrintDebug) true "(R=1.000000,G=0.000000,B=0.000000,A=1.000000)" :!label _label))))
          (:NewEnumerator1
            (Utilities|IsValid (Actor|GetComponentbyClass (LocalVariables|GetActor) "/Game/Scripts/Blueprints/Components/GameParameters/Childs/BP_StaminaComponent.BP_StaminaComponent_C")
              (:Is%20Valid
                (Default|SetCanbeConsumedValue (Actor|GetComponentbyClass (LocalVariables|GetActor) "/Game/Scripts/Blueprints/Components/GameParameters/Childs/BP_StaminaComponent.BP_StaminaComponent_C") (LocalVariables|GetLocalBool)))
              (:Is%20Not%20Valid
                (goto _label)))))))
    (:Is%20Not%20Valid
      (Development|PrintString 0 "ERROR: Actor target missing in SetModifierPerSecondGameAttribute function" (LocalVariables|GetPrintDebug)))))

(fn SetCanbeRestored
  (params (Target%20Actor :type Actor%20Object%20Reference) (GameActionsStruct :type STRUCT%20Game%20Actions%20Structure) (PrintDebugToScreen :type Boolean))
  (bind (_gameplayaction _gameparametersinfluenced _gameparameter_floatvalues _gameparameters_boolvalues) (Utilities|Struct|BreakSTRUCT_GameActions GameActionsStruct))
  (bind _output_get (LocalVariables|SetLocalBoolArray _gameparameters_boolvalues))
  (if (>= (Utilities|Array|Length _output_get) 1)
    _
    (else
      (Utilities|Array|Add (LocalVariables|GetLocalBoolArray) true)))
  (LocalVariables|SetPrintDebug PrintDebugToScreen)
  (bind _output_get_2 (LocalVariables|SetActor Target%20Actor))
  (Utilities|IsValid _output_get_2
    (:Is%20Valid
      (for (_array_element _array_index) _gameparametersinfluenced
        (if (Utilities|Array|IsValidIndex (LocalVariables|GetLocalBoolArray) _array_index)
          _
          (else
            (Utilities|Array|Add (LocalVariables|GetLocalBoolArray) (Utilities|Array|Get(acopy) (LocalVariables|GetLocalBoolArray) (- _array_index 1)))))
        (LocalVariables|SetLocalBool (Utilities|Array|Get(acopy) (LocalVariables|GetLocalBoolArray) _array_index))
        (switch Utilities|FlowControl|Switch|SwitchonENUM_GameParameterType _array_element
          (:NewEnumerator0
            (Utilities|IsValid (Actor|GetComponentbyClass (LocalVariables|GetActor) "/Game/Scripts/Blueprints/Components/GameParameters/Childs/BP_HealthComponent.BP_HealthComponent_C")
              (:Is%20Valid
                (Default|SetCanbeRestoredValue (Actor|GetComponentbyClass (LocalVariables|GetActor) "/Game/Scripts/Blueprints/Components/GameParameters/Childs/BP_HealthComponent.BP_HealthComponent_C") (LocalVariables|GetLocalBool)))
              (:Is%20Not%20Valid
                (Development|PrintString 0 "ERROR: Can't find the right GameParameters Component in SetModifierPerSecondGameAttribute function." (LocalVariables|GetPrintDebug) true "(R=1.000000,G=0.000000,B=0.000000,A=1.000000)" :!label _label))))
          (:NewEnumerator1
            (Utilities|IsValid (Actor|GetComponentbyClass (LocalVariables|GetActor) "/Game/Scripts/Blueprints/Components/GameParameters/Childs/BP_StaminaComponent.BP_StaminaComponent_C")
              (:Is%20Valid
                (Default|SetCanbeRestoredValue (Actor|GetComponentbyClass (LocalVariables|GetActor) "/Game/Scripts/Blueprints/Components/GameParameters/Childs/BP_StaminaComponent.BP_StaminaComponent_C") (LocalVariables|GetLocalBool)))
              (:Is%20Not%20Valid
                (goto _label)))))))
    (:Is%20Not%20Valid
      (Development|PrintString 0 "ERROR: Actor target missing in SetModifierPerSecondGameAttribute function" (LocalVariables|GetPrintDebug)))))

(fn SingleTargetGameplayAction
  (params (Target%20Actor :type Actor%20Object%20Reference) (GameplayActionData :type STRUCT%20Game%20Actions%20Structure) (PrintDebugOnScreen :type Boolean))
  (bind ___worldcontext (LocalVariables|Get__WorldContext))
  (LocalVariables|SetLocalPrintDebug PrintDebugOnScreen)
  (LocalVariables|SetTarget Target%20Actor)
  (LocalVariables|SetLocalGameActions GameplayActionData)
  (switch Utilities|FlowControl|Switch|SwitchonENUM_GameplayActions (.GameplayAction (Utilities|Struct|BreakSTRUCT_GameActions GameplayActionData))
    (:NewEnumerator0
      (GameActions|SetGameAttributes|ForceCurrentGameAttribute (LocalVariables|GetTarget) (LocalVariables|GetLocalGameActions) (LocalVariables|GetLocalPrintDebug) ___worldcontext))
    (:NewEnumerator1
      (GameActions|SetGameAttributes|SetMinGameAttribute (LocalVariables|GetTarget) (LocalVariables|GetLocalGameActions) (LocalVariables|GetLocalPrintDebug) ___worldcontext))
    (:NewEnumerator2
      (GameActions|SetGameAttributes|SetMaxGameAttribute (LocalVariables|GetTarget) (LocalVariables|GetLocalGameActions) (LocalVariables|GetLocalPrintDebug) ___worldcontext))
    (:NewEnumerator3
      (GameActions|SetGameAttributes|ConsumeGameAttribute (LocalVariables|GetTarget) (LocalVariables|GetLocalGameActions) (LocalVariables|GetLocalPrintDebug) ___worldcontext))
    (:NewEnumerator4
      (GameActions|SetGameAttributes|RestoreGameAttribute (LocalVariables|GetTarget) (LocalVariables|GetLocalGameActions) (LocalVariables|GetLocalPrintDebug) ___worldcontext))
    (:NewEnumerator5
      (GameActions|SetGameAttributes|SetModifierPerSecondGameAttribute (LocalVariables|GetTarget) (LocalVariables|GetLocalGameActions) (LocalVariables|GetLocalPrintDebug) ___worldcontext))
    (:NewEnumerator6
      (GameActions|SetGameAttributes|SetCanbeConsumed (LocalVariables|GetTarget) (LocalVariables|GetLocalGameActions) (LocalVariables|GetLocalPrintDebug) ___worldcontext))
    (:NewEnumerator7
      (GameActions|SetGameAttributes|SetCanbeRestored (LocalVariables|GetTarget) (LocalVariables|GetLocalGameActions) (LocalVariables|GetLocalPrintDebug) ___worldcontext))))

(fn LineGameplayAction
  (params (Targets :type ENUM_GameplayActionTargetType%20Enum :default "NewEnumerator0") (GameplayActionData :type STRUCT%20Game%20Actions%20Structure) (PrintDebugOnScreen :type Boolean) (Start :type Vector) (End :type Vector) (TraceChannel :type ETraceTypeQuery%20Enum :default "TraceTypeQuery1") (bTraceComplex :type Boolean) (ActorsToIgnore :type Array%20of%20Actor%20Object%20References) (DrawDebugType :type EDrawDebugTrace%20Enum :default "None") (bIgnoreSelf :type Boolean))
  (switch Utilities|FlowControl|Switch|SwitchonENUM_GameplayActionTargetType Targets
    (:NewEnumerator0
      (bind (_outhit _returnvalue) (Collision|LineTraceByChannel (LocalVariables|Get__WorldContext) Start End TraceChannel bTraceComplex ActorsToIgnore DrawDebugType bIgnoreSelf))
      (if _returnvalue
        (GameActions|Actions|SingleTargetGameplayAction (.hitactor _outhit) GameplayActionData PrintDebugOnScreen (LocalVariables|Get__WorldContext))))
    (:NewEnumerator1
      (bind (_outhits _returnvalue_2) (Collision|MultiLineTraceByChannel (LocalVariables|Get__WorldContext) Start End TraceChannel bTraceComplex ActorsToIgnore DrawDebugType bIgnoreSelf))
      (if _returnvalue_2
        (for _array_element _outhits
          (GameActions|Actions|SingleTargetGameplayAction (.hitactor _array_element) GameplayActionData PrintDebugOnScreen (LocalVariables|Get__WorldContext)))))))

(fn SphereAreaGameplayAction
  (params (Targets :type ENUM_GameplayActionTargetType%20Enum :default "NewEnumerator0") (GameplayActionData :type STRUCT%20Game%20Actions%20Structure) (PrintDebugOnScreen :type Boolean) (Start :type Vector) (End :type Vector) (Radius :type Float%20%28single-precision%29) (TraceChannel :type ETraceTypeQuery%20Enum :default "TraceTypeQuery1") (bTraceComplex :type Boolean) (ActorsToIgnore :type Array%20of%20Actor%20Object%20References) (DrawDebugType :type EDrawDebugTrace%20Enum :default "None") (bIgnoreSelf :type Boolean))
  (switch Utilities|FlowControl|Switch|SwitchonENUM_GameplayActionTargetType Targets
    (:NewEnumerator0
      (bind _outhit (Collision|SphereTraceByChannel (LocalVariables|Get__WorldContext) Start End Radius TraceChannel bTraceComplex ActorsToIgnore DrawDebugType bIgnoreSelf))
      (if true
        (GameActions|Actions|SingleTargetGameplayAction (.hitactor _outhit) GameplayActionData PrintDebugOnScreen (LocalVariables|Get__WorldContext))))
    (:NewEnumerator1
      (bind (_outhits _returnvalue) (Collision|MultiSphereTraceByChannel (LocalVariables|Get__WorldContext) Start End Radius TraceChannel bTraceComplex ActorsToIgnore DrawDebugType bIgnoreSelf))
      (if _returnvalue
        (for _array_element _outhits
          (GameActions|Actions|SingleTargetGameplayAction (.hitactor _array_element) GameplayActionData PrintDebugOnScreen (LocalVariables|Get__WorldContext)))))))

(fn CubeAreaGameplayAction
  (params (Targets :type ENUM_GameplayActionTargetType%20Enum :default "NewEnumerator0") (GameplayActionData :type STRUCT%20Game%20Actions%20Structure) (PrintDebugOnScreen :type Boolean) (Start :type Vector) (End :type Vector) (HalfSize :type Vector) (Orientation :type Rotator) (TraceChannel :type ETraceTypeQuery%20Enum :default "TraceTypeQuery1") (bTraceComplex :type Boolean) (ActorsToIgnore :type Array%20of%20Actor%20Object%20References) (DrawDebugType :type EDrawDebugTrace%20Enum :default "None") (bIgnoreSelf :type Boolean))
  (switch Utilities|FlowControl|Switch|SwitchonENUM_GameplayActionTargetType Targets
    (:NewEnumerator0
      (bind (_outhit _returnvalue) (Collision|BoxTraceByChannel (LocalVariables|Get__WorldContext) Start End HalfSize Orientation TraceChannel bTraceComplex ActorsToIgnore DrawDebugType bIgnoreSelf))
      (if _returnvalue
        (GameActions|Actions|SingleTargetGameplayAction (.hitactor _outhit) GameplayActionData PrintDebugOnScreen (LocalVariables|Get__WorldContext))))
    (:NewEnumerator1
      (bind (_outhits _returnvalue_2) (Class|KismetSystemLibrary|BoxTraceMulti (LocalVariables|Get__WorldContext) Start End HalfSize Orientation TraceChannel bTraceComplex ActorsToIgnore DrawDebugType bIgnoreSelf))
      (if _returnvalue_2
        (for _array_element _outhits
          (GameActions|Actions|SingleTargetGameplayAction (.hitactor _array_element) GameplayActionData PrintDebugOnScreen (LocalVariables|Get__WorldContext)))))))

(fn CheckGameAttributeforGameAction
  (params (Actor :type Actor%20Object%20Reference) (ComparationType :type ENUM_CompareNumbers%20Enum :default "NewEnumerator0") (GameAction :type STRUCT%20Game%20Actions%20Structure))
  (LocalVariables|SetValues (.gameparameter_floatvalues GameAction))
  (LocalVariables|SetLocalActor Actor)
  (for (_array_element _array_index) (.gameparametersinfluenced GameAction)
    (LocalVariables|SetCurrentValue (Utilities|Array|Get(acopy) (LocalVariables|GetValues) _array_index))
    (switch Utilities|FlowControl|Switch|SwitchonENUM_GameParameterType _array_element
      (:NewEnumerator0
        (Utilities|IsValid (Actor|GetComponentbyClass (LocalVariables|GetLocalActor) "/Game/Scripts/Blueprints/Components/GameParameters/Childs/BP_HealthComponent.BP_HealthComponent_C")
          (:Is%20Valid
            (bind _output_get (LocalVariables|SetReturn (Utility|CompareCurrentGameAttribute ComparationType (Variables|/Game/Scripts/Blueprints/Components/GameParameters/BP_CharacterParametersComponent.BP_CharacterParametersComponent_C|GetGameAttribute (Actor|GetComponentbyClass (LocalVariables|GetLocalActor) "/Game/Scripts/Blueprints/Components/GameParameters/Childs/BP_HealthComponent.BP_HealthComponent_C")) (LocalVariables|GetCurrentValue) (LocalVariables|Get__WorldContext))))
            (if (not _output_get)
              (return (LocalVariables|GetReturn))))))
      (:NewEnumerator1
        (Utilities|IsValid (Actor|GetComponentbyClass (LocalVariables|GetLocalActor) "/Game/Scripts/Blueprints/Components/GameParameters/Childs/BP_StaminaComponent.BP_StaminaComponent_C")
          (:Is%20Valid
            (bind _output_get_2 (LocalVariables|SetReturn (Utility|CompareCurrentGameAttribute ComparationType (Variables|/Game/Scripts/Blueprints/Components/GameParameters/BP_CharacterParametersComponent.BP_CharacterParametersComponent_C|GetGameAttribute (Actor|GetComponentbyClass (LocalVariables|GetLocalActor) "/Game/Scripts/Blueprints/Components/GameParameters/Childs/BP_StaminaComponent.BP_StaminaComponent_C")) (LocalVariables|GetCurrentValue) (LocalVariables|Get__WorldContext))))
            (if (not _output_get_2)
              (return (LocalVariables|GetReturn))))))))
  (return (LocalVariables|GetReturn)))

(fn SingleTargetAttack
  (params (TargetActor :type Actor%20Object%20Reference) (GameplayActions :type Array%20of%20STRUCT%20Game%20Actions%20Structures) (AttackTypeMultiplier :type Float%20%28single-precision%29) (WeaponTyperMultiplier :type Float%20%28single-precision%29) (BlockMultiplier :type Float%20%28single-precision%29) (PrintDebugOnScreen :type Boolean))
  (for _array_element GameplayActions
    (Utilities|Array|Resize (LocalVariables|GetFloatValues) 0)
    (for _array_element_2 (.GameParameter_FloatValues (Utilities|Struct|BreakSTRUCT_GameActions _array_element))
      (Utilities|Array|SetArrayElem (LocalVariables|GetFloatValues) 0 (* _array_element_2 AttackTypeMultiplier WeaponTyperMultiplier BlockMultiplier) true))
    (GameActions|Actions|SingleTargetGameplayAction TargetActor (Utilities|Struct|MakeSTRUCT_GameActions (.GameplayAction (Utilities|Struct|BreakSTRUCT_GameActions _array_element)) (.GameParametersInfluenced (Utilities|Struct|BreakSTRUCT_GameActions _array_element)) (LocalVariables|GetFloatValues) (.GameParameters_BoolValues (Utilities|Struct|BreakSTRUCT_GameActions _array_element))) PrintDebugOnScreen (LocalVariables|Get__WorldContext))))