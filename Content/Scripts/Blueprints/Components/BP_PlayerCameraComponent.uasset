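; Player camera component that drives the character's spring arm length and socket offset from movement.
; Each tick, forward motion raises a clamped blend between minimum and maximum arm length and other motion lowers it, at a rate scaled by distance from a speed-based target.
; Side and height offsets then follow the current arm length.
; CameraZoom forwards zoom requests through OnCameraZoom; a right-side trace helper exists but is not called here.
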(event Custom|Initialization
  (CallFunction|UpdateRef)
  (Variables|Default|SetInitialized true))

(event Custom|CameraZoom
  (params (NewMaxLenght :type Float%20%28single-precision%29) (NewMinArmLenght :type Float%20%28single-precision%29) (CameraZoomCurve :type Curve%20Float%20Object%20Reference))
  (Default|CallOnCameraZoom NewMaxLenght NewMinArmLenght CameraZoomCurve))

(event EventBeginPlay)

(event EventTick
  (params (DeltaSeconds :type Float%20%28single-precision%29))
  (Variables|Default|SetDT DeltaSeconds)
  (if (Variables|Default|GetInitialized)
    (CallFunction|UpdateArmLenght (Variables|Default|GetForwardCameraAcceleration))
    (CallFunction|UpdateSocketOffset)))

(fn UpdateRef
  (bind _asbp_player_character (Utilities|Casting|CastToBP_PlayerCharacter (Components|GetOwner)))
  (bind _output_get (Variables|References|SetPlayerChar_ref _asbp_player_character))
  (Variables|References|SetArm_Ref (Variables|/Game/Scripts/Blueprints/Characters/BP_PlayerCharacter.BP_PlayerCharacter_C|GetSpringArm _output_get))
  (bind _asbp_player_conroller (Utilities|Casting|CastToBP_PlayerConroller (Pawn|GetController _output_get)))
  (Variables|References|SetController_ref _asbp_player_conroller)
  (Variables|References|SetCharacterMovement_ref (Variables|/Script/Engine.Character|GetCharacterMovement _asbp_player_character))
  (Variables|References|SetCamera_Ref (Variables|/Game/Scripts/Blueprints/Characters/BP_PlayerCharacter.BP_PlayerCharacter_C|GetCamera _asbp_player_character)))

(fn GetLastArmLenghtFraction
  (params (Acceleration :type Float%20%28single-precision%29))
  (LocalVariables|SetLastFraction (* (/ (Math|Float|Absolute(Float) (- (Variables|Default|GetArmLenghtObjective) (Variables|/Script/Engine.SpringArmComponent|GetTargetArmLength (Variables|References|GetArm_Ref)))) (Math|Float|Absolute(Float) (- (Variables|Default|GetMaxArmLenght) (Variables|Default|GetMinArmLenght)))) Acceleration))
  (return (LocalVariables|GetLastFraction)))

(fn UpdateArmLenght
  (params (ForwardAcceleration :type Float%20%28single-precision%29))
  (bind _playerchar_ref (Variables|References|GetPlayerChar_ref))
  (Variables|Default|SetArmLenghtObjective (Math|Float|Lerp (Variables|Default|GetMinArmLenght) (Variables|Default|GetMaxArmLenght) (Math|Float|Clamp(Float) (/ (Math|Vector|VectorLength (Transformation|GetVelocity _playerchar_ref)) (Variables|/Game/Scripts/Blueprints/Characters/BP_CharacterMaster.BP_CharacterMaster_C|GetMaxSpeed_Sprint _playerchar_ref)))))
  (if (> (CallFunction|GetForwardSpeedNormalized) 0.0)
    (Variables|Default|SetArmLenghtUpdateSpeed (CallFunction|GetIncreasetForwardArmSpeed ForwardAcceleration))
    (else
      (Variables|Default|SetArmLenghtUpdateSpeed (CallFunction|GetDecreasedForwadArmSpeed ForwardAcceleration))))
  (Variables|/Script/Engine.SpringArmComponent|SetTargetArmLength (Variables|References|GetArm_Ref) (Math|Float|Lerp (Variables|Default|GetMinArmLenght) (Variables|Default|GetMaxArmLenght) (Variables|Default|GetArmLenghtUpdateSpeed))))

(fn GetForwardSpeedNormalized
  (return (Math|Vector|DotProduct (Transformation|GetActorForwardVector (Variables|References|GetPlayerChar_ref)) (Math|Vector|Normalize (Variables|/Script/Engine.MovementComponent|GetVelocity (Variables|References|GetCharacterMovement_ref))))))

(fn GetIncreasetForwardArmSpeed
  (params (Acceleration :type Float%20%28single-precision%29))
  (return (Math|Float|Clamp(Float) (+ (Variables|Default|GetArmLenghtUpdateSpeed) (* (Variables|Default|GetDT) (CallFunction|GetLastArmLenghtFraction Acceleration))))))

(fn GetDecreasedForwadArmSpeed
  (params (Acceleration :type Float%20%28single-precision%29))
  (return (Math|Float|Clamp(Float) (- (Variables|Default|GetArmLenghtUpdateSpeed) (* (Variables|Default|GetDT) (CallFunction|GetLastArmLenghtFraction Acceleration))))))

(fn RightCameraTracing
  (bind _camera_ref (Variables|References|GetCamera_Ref))
  (bind _returnvalue (Transformation|GetWorldLocation _camera_ref))
  (bind (_outhit _returnvalue_2) (Collision|LineTraceByChannel _returnvalue (+ _returnvalue (* (Math|Vector|GetRightVector _camera_ref) (Variables|Default|GetRightOffset))) "TraceTypeQuery1" false (Utilities|Array|MakeArray (Variables|References|GetPlayerChar_ref)) "None"))
  (return _outhit _returnvalue_2))

(fn GetMidArmPoint
  (return (* (+ (Variables|Default|GetMaxArmLenght) (Variables|Default|GetMinArmLenght)) 0.5)))

(fn UpdateSocketOffset
  (bind _arm_ref (Variables|References|GetArm_Ref))
  (bind _targetarmlength (Variables|/Script/Engine.SpringArmComponent|GetTargetArmLength _arm_ref))
  (Variables|/Script/Engine.SpringArmComponent|SetSocketOffset (Variables|References|GetArm_Ref) (Math|Vector|MakeVector 0.0 (* (Variables|Default|GetYProportion) (- (Variables|Default|GetMaxArmLenght) _targetarmlength)) (* _targetarmlength (Variables|Default|GetZProportion)))))