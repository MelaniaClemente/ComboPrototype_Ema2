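; AI combat component that picks an enemy character's combat state at random: strafe, charge, dodge or attack.
; BeginPlay caches the owner's enemy character through BP_CharacterInterface.
; Every Tick rolls between Min and the summed chances, tests cumulative bands with attack as fallback, and prints the state.
; ChargeChance only feeds the sum: the charge band's width uses DodgeChance and the dodge band's uses AttackChance.
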(event EventBeginPlay
  (bind _returnvalue (Components|GetOwner))
  (if (Utilities|DoesObjectImplementInterface _returnvalue "/Game/Scripts/Blueprints/Interfaces/BP_CharacterInterface.BP_CharacterInterface_C")
    (bind _enemycharacter (Class|BPCharacterInterface|GetMyEnemyCharacter(Message) _returnvalue))
    (Variables|Default|SetOwnerCharacter _enemycharacter)))

(event EventTick
  (params (DeltaSeconds :type Float%20%28single-precision%29))
  (Variables|CombatStates|Probabilities|SetMax (CallFunction|GetSum))
  (Variables|CombatStates|Probabilities|SetRandom (Math|Random|RandomFloatinRange (Variables|CombatStates|Probabilities|GetMin) (Variables|CombatStates|Probabilities|GetMax)))
  (if (CallFunction|GetStrafingChance)
    (Variables|Default|SetCombatState "NewEnumerator0")
    (elif (CallFunction|GetChargingChance)
      (Variables|Default|SetCombatState "NewEnumerator1")
      (elif (CallFunction|GetDodgingChance)
        (Variables|Default|SetCombatState "NewEnumerator2")
        (elif (CallFunction|GetAttackChance)
          (Variables|Default|SetCombatState "NewEnumerator3")
          (else
            (Variables|Default|SetCombatState "NewEnumerator3"))))))
  (Development|PrintString (Utilities|String|EnumtoString (Variables|Default|GetCombatState))))

(fn GetSum
  (return (+ (Variables|CombatStates|Probabilities|GetStrafeChance) (Variables|CombatStates|Probabilities|GetChargeChance) (Variables|CombatStates|Probabilities|GetDodgeChance) (Variables|CombatStates|Probabilities|GetAttackChance))))

(fn GetStrafingChance
  (return (and (>= (Variables|CombatStates|Probabilities|GetRandom) (Variables|CombatStates|Probabilities|GetMin)) (< (Variables|CombatStates|Probabilities|GetRandom) (Variables|CombatStates|Probabilities|GetStrafeChance)))))

(fn GetChargingChance
  (return (and (>= (Variables|CombatStates|Probabilities|GetRandom) (+ (Variables|CombatStates|Probabilities|GetMin) (Variables|CombatStates|Probabilities|GetStrafeChance))) (< (Variables|CombatStates|Probabilities|GetRandom) (+ (Variables|CombatStates|Probabilities|GetMin) (Variables|CombatStates|Probabilities|GetStrafeChance) (Variables|CombatStates|Probabilities|GetDodgeChance))))))

(fn GetDodgingChance
  (return (and (>= (Variables|CombatStates|Probabilities|GetRandom) (+ (Variables|CombatStates|Probabilities|GetMin) (Variables|CombatStates|Probabilities|GetStrafeChance) (Variables|CombatStates|Probabilities|GetDodgeChance))) (< (Variables|CombatStates|Probabilities|GetRandom) (+ (Variables|CombatStates|Probabilities|GetMin) (Variables|CombatStates|Probabilities|GetStrafeChance) (Variables|CombatStates|Probabilities|GetDodgeChance) (Variables|CombatStates|Probabilities|GetAttackChance))))))

(fn GetAttackChance
  (return (>= (Variables|CombatStates|Probabilities|GetRandom) (+ (Variables|CombatStates|Probabilities|GetMin) (Variables|CombatStates|Probabilities|GetStrafeChance) (Variables|CombatStates|Probabilities|GetDodgeChance) (Variables|CombatStates|Probabilities|GetAttackChance)))))

(fn GetCombatState
  (return (Variables|Default|GetCombatState)))