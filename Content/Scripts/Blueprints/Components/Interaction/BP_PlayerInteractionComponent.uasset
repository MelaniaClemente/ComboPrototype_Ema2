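; Player interaction component that identifies the interaction type of the interactible object in front of the camera.
; On BeginPlay it caches the owning player character through an interface.
; Helper functions build a camera-forward segment and line trace it, storing the hit BP_MasterInteractibleObject's type or resetting to the default enum value.
; The tracing call sits in unconnected event-graph logic and Tick is empty, so the trace never runs here.
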(event Custom|Initialization
  (bind _returnvalue (Components|GetOwner))
  (bind _playercharacter (CallFunction|GetMyPlayerCharacterbyInterface false _returnvalue))
  (Utilities|IsValid _playercharacter
    (:Is%20Valid
      (Variables|Default|SetPlayerCharacter_Ref _playercharacter))))

(event EventBeginPlay
  (CallFunction|Initialization))

(event EventTick
  (params (DeltaSeconds :type Float%20%28single-precision%29)))

(fn InteractionTracing
  (params (Start :type Vector) (End :type Vector) (DrawDebugType :type EDrawDebugTrace%20Enum :default "None"))
  (bind (_outhit _returnvalue) (Collision|LineTraceByChannel Start End "TraceTypeQuery3" false (Utilities|Array|MakeArray (Components|GetOwner)) DrawDebugType))
  (if _returnvalue
    (bind _asbp_master_interactible_object (Utilities|Casting|CastToBP_MasterInteractibleObject (.hitactor _outhit))
      (:then
        (Utilities|IsValid _asbp_master_interactible_object
          (:Is%20Valid
            (Variables|Interactions|SetCurrentInteractionType (Variables|/Game/Scripts/Blueprints/LevelDesignHelper/Interaction/BP_MasterInteractibleObject.BP_MasterInteractibleObject_C|GetInteractionType _asbp_master_interactible_object)))
          (:Is%20Not%20Valid
            (CallFunction|DebugMsgUnvalidObject _asbp_master_interactible_object false)
            (Variables|Interactions|SetCurrentInteractionType "NewEnumerator0" :!label _label))))
      (:CastFailed
        (goto _label)))
    (else
      (goto _label))))

(fn GetForwardCameraTracingData
  (bind _playercharacter_ref (Variables|Default|GetPlayerCharacter_Ref))
  (bind _camera (Variables|/Game/Scripts/Blueprints/Characters/BP_PlayerCharacter.BP_PlayerCharacter_C|GetCamera _playercharacter_ref))
  (bind _returnvalue (Transformation|GetWorldLocation _camera))
  (return _returnvalue (+ _returnvalue (* (Math|Vector|GetForwardVector _camera) (Variables|Interactions|GetTracingLenght)))))