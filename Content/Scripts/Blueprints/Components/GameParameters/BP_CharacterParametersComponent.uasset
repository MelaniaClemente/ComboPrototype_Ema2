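; Character component that manages one clamped game attribute with min, max, start and current values, plus flags allowing it to be consumed or restored.
; BeginPlay applies the start value and caches player character and character master references from the owner.
; Tick applies the per-second modifier scaled by delta time and fires exhausted or maximized calls at the limits, either every tick or once until reset.
; Consume and restore functions print warnings when disallowed.
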(event Custom|ResetExhaustedEvent
  (Utilities|FlowControl|DoOnce false) ; enters at Reset
)

(event Custom|ResetMaximizedEvent
  (Utilities|FlowControl|DoOnce false) ; enters at Reset
)

(event EventBeginPlay
  (bind _returnvalue (Components|GetOwner))
  (SetFunctions|SetCurrentValue (.startvalue (Variables|GameParameter|GetGameAttribute)))
  (Variables|Default|SetPlayer%20Character_ref (CallFunction|GetMyPlayerCharacterbyInterface false _returnvalue))
  (Variables|Default|SetCharacter%20Master_ref (CallFunction|GetMyCharacterMasterbyInterface false _returnvalue)))

(event EventTick
  (params (DeltaSeconds :type Float%20%28single-precision%29))
  (Variables|Default|SetDS DeltaSeconds)
  (Utilities|FlowControl|Sequence
    (:then_0
      (if (Bool|IsExhausted)
        (if (Variables|GameParameter|GetCallParameterExhaustedEachTick)
          _
          (else
            (Utilities|FlowControl|DoOnce false
              (:Completed
                _))))
        (Default|CallParameterExhausted)))
    (:then_1
      (if (Bool|IsMaximized)
        (if (Variables|GameParameter|GetCallParameterMaximizedEachTick)
          _
          (else
            (Utilities|FlowControl|DoOnce false
              (:Completed
                _))))
        (Default|CallParameterMaximized)))
    (:then_2
      ;[0 0 0] Modifier per tick
      (if (or (Bool|IsRegeneratingOverTime) (Bool|IsConsumingOverTime))
        (SetFunctions|SetCurrentValue (+ (GetFunctions|GetModifierPerTick) (GetFunctions|GetCurrentValue)))))))

(fn IsZero
  (return (CallFunction|CompareCurrentGameAttribute "NewEnumerator3" (Variables|GameParameter|GetGameAttribute) 0.0)))

(fn ConsumeValue
  (params (ValueToConsume :type Float%20%28single-precision%29) (PrintDebugToScreen :type Boolean))
  (if (.bCanBeConsumed (Utilities|Struct|BreakSTRUCT_GameAttribute (Variables|GameParameter|GetGameAttribute)))
    (bind _structout (Utilities|Struct|SetmembersinSTRUCT_GameAttribute (Variables|GameParameter|GetGameAttribute) (- (.CurrentValue (Utilities|Struct|BreakSTRUCT_GameAttribute (Variables|GameParameter|GetGameAttribute))) ValueToConsume)))
    (Variables|GameParameter|SetGameAttribute (CallFunction|ClampGameAttribute _structout))
    (else
      (Development|PrintString (Utilities|String|Append "WARNING:" (Utilities|GetObjectName self) "can't consume the current value. The variable bCanBeConsumed is set to false.") PrintDebugToScreen true "(R=1.000000,G=1.000000,B=0.000000,A=1.000000)")))
  (return))

(fn GetCurrentValue
  (return (.currentvalue (Variables|GameParameter|GetGameAttribute))))

(fn GetMaxValue
  (return (.maxvalue (Variables|GameParameter|GetGameAttribute))))

(fn GetMinValue
  (return (.minvalue (Variables|GameParameter|GetGameAttribute))))

(fn CanbeConsumed
  (return (.bcanbeconsumed (Variables|GameParameter|GetGameAttribute))))

(fn CanbeRestore
  (return (.bcanberestored (Variables|GameParameter|GetGameAttribute))))

(fn SetMaxValue
  (params (NewMaxValue :type Float%20%28single-precision%29))
  (bind _structout (Utilities|Struct|SetmembersinSTRUCT_GameAttribute (Variables|GameParameter|GetGameAttribute) NewMaxValue))
  (Variables|GameParameter|SetGameAttribute _structout))

(fn SetMinValue
  (params (NewMinValue :type Float%20%28single-precision%29))
  (bind _structout (Utilities|Struct|SetmembersinSTRUCT_GameAttribute (Variables|GameParameter|GetGameAttribute) NewMinValue))
  (Variables|GameParameter|SetGameAttribute _structout))

(fn SetStartingValue
  (params (NewStartingValue :type Float%20%28single-precision%29))
  (bind _structout (Utilities|Struct|SetmembersinSTRUCT_GameAttribute (Variables|GameParameter|GetGameAttribute) NewStartingValue))
  (Variables|GameParameter|SetGameAttribute _structout))

(fn GetModifierPerSecond
  (return (.modifierpersecond (Variables|GameParameter|GetGameAttribute))))

(fn SetModifierPerSecond
  (params (NewModifierValue :type Float%20%28single-precision%29))
  (bind _structout (Utilities|Struct|SetmembersinSTRUCT_GameAttribute (Variables|GameParameter|GetGameAttribute) NewModifierValue))
  (Variables|GameParameter|SetGameAttribute _structout))

(fn GetModifierPerTick
  (return (* (.modifierpersecond (Variables|GameParameter|GetGameAttribute)) (Variables|Default|GetDS))))

(fn IsRegeneratingOverTime
  (return (and (> (GetFunctions|GetModifierPerSecond) 0.0) (Bool|CanbeRestore))))

(fn IsConsumingOverTime
  (return (and (< (GetFunctions|GetModifierPerSecond) 0.0) (Bool|CanbeConsumed))))

(fn SetCurrentValue
  (params (NewCurrentValue :type Float%20%28single-precision%29))
  (bind _structout (Utilities|Struct|SetmembersinSTRUCT_GameAttribute (Variables|GameParameter|GetGameAttribute) NewCurrentValue))
  (Variables|GameParameter|SetGameAttribute (CallFunction|ClampGameAttribute _structout)))

(fn RestoreValue
  (params (ValueToRestore :type Float%20%28single-precision%29) (PrintDebugToScreen :type Boolean))
  (if (.bCanBeRestored (Utilities|Struct|BreakSTRUCT_GameAttribute (Variables|GameParameter|GetGameAttribute)))
    (bind _structout (Utilities|Struct|SetmembersinSTRUCT_GameAttribute (Variables|GameParameter|GetGameAttribute) (+ ValueToRestore (.CurrentValue (Utilities|Struct|BreakSTRUCT_GameAttribute (Variables|GameParameter|GetGameAttribute))))))
    (Variables|GameParameter|SetGameAttribute (CallFunction|ClampGameAttribute _structout))
    (else
      (Development|PrintString (Utilities|String|Append "WARNING:" (Utilities|GetObjectName self) "can't restore the current value. The variable bCanBeRestored is set to false.") PrintDebugToScreen true "(R=1.000000,G=1.000000,B=0.000000,A=1.000000)")))
  (return))

(fn IsExhausted
  (return (CallFunction|CompareCurrentGameAttribute "NewEnumerator3" (Variables|GameParameter|GetGameAttribute) (GetFunctions|GetMinValue))))

(fn IsMaximized
  (return (CallFunction|CompareCurrentGameAttribute "NewEnumerator1" (Variables|GameParameter|GetGameAttribute) (GetFunctions|GetMaxValue))))

(fn SetCanbeConsumedValue
  (params (Value :type Boolean))
  (bind _structout (Utilities|Struct|SetmembersinSTRUCT_GameAttribute (Variables|GameParameter|GetGameAttribute) Value))
  (Variables|GameParameter|SetGameAttribute _structout)
  (return))

(fn SetCanbeRestoredValue
  (params (Value :type Boolean))
  (bind _structout (Utilities|Struct|SetmembersinSTRUCT_GameAttribute (Variables|GameParameter|GetGameAttribute) Value))
  (Variables|GameParameter|SetGameAttribute _structout)
  (return))

(fn GameplayAction)