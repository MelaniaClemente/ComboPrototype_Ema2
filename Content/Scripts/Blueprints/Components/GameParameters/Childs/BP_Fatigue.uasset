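; BP_Fatigue is a fatigue game parameter component that converts its current value into a damage multiplier.
; GetDamageMultiplier linearly interpolates by the current-to-max ratio, from MaxDamageMultiplier at zero down to MinDamageMultiplier at the maximum value.
; Tick only forwards to the parent, which the component relies on for its value, and a debug print of that value is left unconnected.
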(event EventBeginPlay
  (|CallParentFunction) ; This node is disabled and will not be called.\nDrag off pins to build functionality.
)

(event EventTick
  (params (DeltaSeconds :type Float%20%28single-precision%29))
  (|CallParentFunction DeltaSeconds))

(fn GetDamageMultiplier
  (return (Math|Float|Lerp (Variables|Default|GetMaxDamageMultiplier) (Variables|Default|GetMinDamageMultiplier) (/ (CallFunction|GetCurrentValue) (CallFunction|GetMaxValue)))))