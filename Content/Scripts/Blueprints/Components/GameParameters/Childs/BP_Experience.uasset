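; Experience game parameter component, a child in the GameParameters family, that tracks experience for the selected hero.
; On BeginPlay it sets min and max from a curve's value range and the current value by sampling that curve at the character level.
; It then binds to the initialization event, whose handler copies the selected hero's Experience attribute and level from the gameplay GameInstance.
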(event Custom|InitializeLevelFromGameInstance
  (bind _asbp_gameplay_instance (Utilities|Casting|CastToBP_GameplayInstance (Game|GetGameInstance)))
  (Variables|Default|SetGameAttribute (.experience (Variables|/Game/Scripts/Blueprints/GameModes/BP_GameplayInstance.BP_GameplayInstance_C|GetSelectedHero _asbp_gameplay_instance)))
  (Variables|Default|SetCharacterCurrentLevel (.level (Variables|/Game/Scripts/Blueprints/GameModes/BP_GameplayInstance.BP_GameplayInstance_C|GetSelectedHero _asbp_gameplay_instance))))

(event EventBeginPlay
  (bind (_minvalue _maxvalue) (CallFunction|GetCurveValueRange))
  (|CallParentFunction)
  (CallFunction|SetMaxValue _maxvalue)
  (CallFunction|SetMinValue _minvalue)
  (CallFunction|SetCurrentValue (CallFunction|GetCurveValue (Math|Conversions|ToFloat(Integer) (Variables|Default|GetCharacterCurrentLevel))))
  (EventDispatchers|BindEventtoOnInitialization (delegate Custom|InitializeLevelFromGameInstance)))

(event EventTick
  (params (DeltaSeconds :type Float%20%28single-precision%29))
  (|CallParentFunction DeltaSeconds))