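; Game parameter component for hyper armor that regenerates its value after a short delay.
; StartRecoveryTimer sets a one-shot timer that fires Recovery, which sets the per-second modifier to a fraction of the max value.
; InvalidateRecoveryTimer clears that timer and zeroes the modifier, halting pending or active regeneration.
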(event Custom|StartRecoveryTimer
  (bind _returnvalue (Utilities|Time|SetTimerbyEvent (delegate Custom|Recovery) 1.5))
  (Variables|Default|SetRecoveryTimer _returnvalue))

(event Custom|Recovery
  (CallFunction|SetModifierPerSecond (* (CallFunction|GetMaxValue) (Variables|Default|GetRecoveryValuePerSec))))

(event EventBeginPlay
  (|CallParentFunction) ; This node is disabled and will not be called.\nDrag off pins to build functionality.
)

(event EventTick
  (params (DeltaSeconds :type Float%20%28single-precision%29))
  (|CallParentFunction DeltaSeconds))

(fn InvalidateRecoveryTimer
  (Utilities|Time|ClearandInvalidateTimerbyHandle (Variables|Default|GetRecoveryTimer))
  (CallFunction|SetModifierPerSecond 0.0))