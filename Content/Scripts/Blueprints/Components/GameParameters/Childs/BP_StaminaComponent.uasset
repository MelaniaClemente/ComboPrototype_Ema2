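; Stamina component for characters, built on a parent parameter component that supplies current value, max and per-second modifier.
; BeginPlay caches the owning character, its combat component and movement through BP_CharacterInterface.
; A two-second timer event sets recovery to a tenth of max per second.
; Helpers for movement-based drain and stamina-scaled combat play rate are disconnected from Tick, and InvalidateRecoveryTimer invalidates the handle without clearing the timer.
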(event Custom|StartRecoveryTimer
  (bind _returnvalue (Utilities|Time|SetTimerbyEvent (delegate Custom|Recovery) 2.0))
  (Variables|Default|SetRecoveryTimer _returnvalue))

(event Custom|Recovery
  (CallFunction|SetModifierPerSecond (* (CallFunction|GetMaxValue) 0.1)))

(event EventBeginPlay
  (|CallParentFunction)
  (CallFunction|InitializeReferences))

(event EventTick
  (params (DeltaSeconds :type Float%20%28single-precision%29))
  (|CallParentFunction DeltaSeconds))

(fn GetRegenerationValue
  (params (Min :type Float%20%28single-precision%29) (Max :type Float%20%28single-precision%29) (LerpSpeed :type Float%20%28single-precision%29))
  (LocalVariables|SetRecoveryValue (Math|Float|Lerp Min Max LerpSpeed))
  (return (+ (CallFunction|GetCurrentValue) (* (LocalVariables|GetRecoveryValue) (Utilities|Time|GetWorldDeltaSeconds)))))

(fn InitializeReferences
  (bind _returnvalue (Components|GetOwner))
  (if (Utilities|DoesObjectImplementInterface _returnvalue "/Game/Scripts/Blueprints/Interfaces/BP_CharacterInterface.BP_CharacterInterface_C")
    (bind _charactermaster (Class|BPCharacterInterface|GetMyCharacterMaster(Message) _returnvalue))
    (Variables|Default|SetCharacterMasterRef _charactermaster)
    (Variables|Default|SetCombatComponentRef (Actor|GetComponentbyClass _charactermaster "/Game/Scripts/Blueprints/Components/Animation/BP_CombatComponent.BP_CombatComponent_C"))
    (Variables|Default|SetCharacterMovementRef (Variables|/Script/Engine.Character|GetCharacterMovement _charactermaster))))

(fn GetCharacterVelocity
  (return (Math|Vector|VectorLength (Variables|/Script/Engine.MovementComponent|GetVelocity (Variables|Default|GetCharacterMovementRef)))))

(fn UpdateConsumebyVelocity
  (if (> (CallFunction|GetCharacterVelocity) 0.0)
    (if (not (Variables|Default|GetComeOverTimeEnabled))
      (CallFunction|SetModifierPerSecond (- (CallFunction|GetModifierPerSecond) (Variables|Default|GetBaseStaminaConsumePerSecond)))
      (Variables|Default|SetComeOverTimeEnabled true))
    (elif (Variables|Default|GetComeOverTimeEnabled)
      (CallFunction|SetModifierPerSecond (+ (CallFunction|GetModifierPerSecond) (Variables|Default|GetBaseStaminaConsumePerSecond)))
      (Variables|Default|SetComeOverTimeEnabled false))))

(fn UpdateAnimationPlayRate
  (Variables|/Game/Scripts/Blueprints/Components/Animation/BP_CombatComponent.BP_CombatComponent_C|SetPlayRateByStamina (Variables|Default|GetCombatComponentRef) (Math|Float|Lerp (Variables|Default|GetMinPlayRate) (Variables|Default|GetMaxPlayRate) (CallFunction|GetStaminaPercentage))))

(fn GetStaminaPercentage
  (return (/ (CallFunction|GetCurrentValue) (CallFunction|GetMaxValue))))

(fn InvalidateRecoveryTimer
  (bind _returnvalue (Utilities|Time|InvalidateTimerHandle (Variables|Default|GetRecoveryTimer)))
  (Variables|Default|SetRecoveryTimer _returnvalue))