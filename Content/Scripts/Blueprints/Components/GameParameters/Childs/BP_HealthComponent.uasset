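; BP_HealthComponent is a game parameter component that supplies the health attribute for its owning character.
; InitializeBinding_Health checks that the owner is BP_PlayerCharacter, then copies Health from the game instance's SelectedHero data into GameAttribute.
; BeginPlay and Tick only call the parent, and the node binding InitializeBinding_Health to OnInitialization is unconnected, so this graph never registers it.
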(event Custom|InitializeBinding_Health
  (Utilities|Casting|CastToBP_PlayerCharacter (Components|GetOwner))
  (bind _output_get (Variables|Default|SetHeroData (Variables|/Game/Scripts/Blueprints/GameModes/BP_GameplayInstance.BP_GameplayInstance_C|GetSelectedHero (Variables|Default|GetGameInstance_ref))))
  (Variables|Default|SetGameAttribute (.health _output_get)))

(event EventBeginPlay
  (|CallParentFunction))

(event EventTick
  (params (DeltaSeconds :type Float%20%28single-precision%29))
  (|CallParentFunction DeltaSeconds))