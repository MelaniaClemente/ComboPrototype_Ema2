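; Damage component, a child game parameter, that computes and applies a character's standard hit to a target's HP and hyper armor.
; Damage scales the current parameter value by armor reduction, player fatigue, the current combat animation's multipliers and block multipliers, then goes out as a single-target gameplay action.
; Helpers derive block reduction from the owner's moveset and attack type; heavy attacks bypass block, while other types deal no hyper armor damage.
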(event EventBeginPlay
  (|CallParentFunction)
  (bind _asbp_character_master (Utilities|Casting|CastToBP_CharacterMaster (Components|GetOwner)))
  (Variables|Default|SetCombatComponentRef (Variables|/Game/Scripts/Blueprints/Characters/BP_CharacterMaster.BP_CharacterMaster_C|GetBP_CombatComponent _asbp_character_master)))

(event EventTick
  (params (DeltaSeconds :type Float%20%28single-precision%29))
  (|CallParentFunction DeltaSeconds) ; This node is disabled and will not be called.\nDrag off pins to build functionality.
)

(fn CalculateStandardDamage
  (params (Target%20Actor :type Actor%20Object%20Reference) (ArmorReductionMultiplier :type Float%20%28single-precision%29) (HP_BlockReductionMultiplier :type Float%20%28single-precision%29) (HA_BlockReductionMultiplier :type Float%20%28single-precision%29))
  (bind _currentvalue (CallFunction|GetCurrentValue))
  (bind _combatcomponentref (Variables|Default|GetCombatComponentRef))
  (bind _currentanimation (Variables|/Game/Scripts/Blueprints/Components/Animation/BP_CombatComponent.BP_CombatComponent_C|GetCurrentAnimation _combatcomponentref))
  (bind _asbp_player_character (Utilities|Casting|CastToBP_PlayerCharacter (Components|GetOwner))
    (:then
      (LocalVariables|SetFatigue%20multiplier (Default|GetDamageMultiplier (Variables|/Game/Scripts/Blueprints/Characters/BP_PlayerCharacter.BP_PlayerCharacter_C|GetFatigueComponent _asbp_player_character))))
    (:CastFailed
      (LocalVariables|SetFatigue%20multiplier 1.0)))
  (CallFunction|SingleTargetGameplayAction Target%20Actor (Utilities|Struct|MakeSTRUCT_GameActions_new "NewEnumerator3" (Utilities|Array|MakeArray "NewEnumerator0" "NewEnumerator6") (Utilities|Array|MakeArray (* (* ArmorReductionMultiplier _currentvalue (LocalVariables|GetFatigue%20multiplier)) (.damagemultiplier_hp _currentanimation) HP_BlockReductionMultiplier) (* (* ArmorReductionMultiplier _currentvalue (LocalVariables|GetFatigue%20multiplier)) (.damagemultiplier_hyperarmor _currentanimation) HA_BlockReductionMultiplier)) 0) false)
  (Development|PrintString (Utilities|String|Append "Current Value: " (Utilities|String|ToString(Float) _currentvalue) "Armor Reduction: " (Utilities|String|ToString(Float) ArmorReductionMultiplier) "FatigueMulitplier: " (Utilities|String|ToString(Float) (LocalVariables|GetFatigue%20multiplier))) true true "(R=1.000000,G=0.000000,B=0.183144,A=1.000000)" 1e+01))

(fn GetBlockDamageReductionBYAttackType
  (params (AttackType :type ENUM_AnimationPhase%20Enum :default "NewEnumerator0") (BlockDamageReduction :type Float%20%28single-precision%29))
  (LocalVariables|SetHpMultiplier BlockDamageReduction)
  (switch Utilities|FlowControl|Switch|SwitchonENUM_AnimationPhase AttackType
    (:NewEnumerator0
      (LocalVariables|SetHA 0.0 :!label _label))
    (:NewEnumerator1
      (goto _label))
    (:NewEnumerator2
      (goto _label))
    (:NewEnumerator3
      (LocalVariables|SetHA 1.0)
      (LocalVariables|SetHpMultiplier 1.0))
    (:NewEnumerator4
      (goto _label))
    (:NewEnumerator5
      (goto _label)))
  (return (LocalVariables|GetHpMultiplier) (LocalVariables|GetHA)))

(fn GetBlockDamageReductionbyMoveset
  (bind _asbp_character_master (Utilities|Casting|CastToBP_CharacterMaster (Components|GetOwner)))
  (LocalVariables|SetDmgReduction (Math|Float|Clamp(Float) (- 1.0 (Utilities|Select :Index (Variables|/Game/Scripts/Blueprints/Characters/BP_CharacterMaster.BP_CharacterMaster_C|GetMoveset _asbp_character_master) :NewEnumerator2 0.0 :NewEnumerator5 0.5 :NewEnumerator0 0.75 :NewEnumerator1 0.25 :NewEnumerator3 0.75 :NewEnumerator4 0.5))))
  (return (LocalVariables|GetDmgReduction)))