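; AI component that rerolls an enemy's combat state (attack, defend, strafe), attack type (light or heavy) and defence type (dodge or block) every tick.
; Each option averages base efficiency over its configured methods (constant, random, own health, player attacking or blocking), then applies a constant, linear, logarithmic or exponential growth curve.
; The resulting chances act as weights for a random pick, though CalculateProbabilities only sums adjacent entries rather than a full cumulative total.
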(event Custom|Initialization
  (Variables|Default|SethealthComponent (Variables|/Game/Scripts/Blueprints/Characters/BP_CharacterMaster.BP_CharacterMaster_C|GetBP_HealthComponent (CallFunction|GetOwnerEnemyCharacter))))

(event EventBeginPlay
  (CallFunction|Initialization))

(event EventTick
  (params (DeltaSeconds :type Float%20%28single-precision%29))
  (UpdateFunctions|CombatState|UpdateCombatState)
  (UpdateFunctions|AttackState|UpdateAttackState)
  (UpdateFunctions|DefenceState|UpdateDefenceState))

(fn GetCombatStateSum
  (return (+ (Variables|CombatStates|Probabilities|GetStrafeChance) (Variables|CombatStates|Probabilities|GetDefenceChance) (Variables|CombatStates|Probabilities|GetAttackChance))))

(fn GetStrafingChance
  (params (Min :type Float%20%28single-precision%29) (Random :type Float%20%28single-precision%29))
  (return (and (>= Random Min) (< Random (Variables|CombatStates|Probabilities|GetStrafeChance)))))

(fn GetDodgingChance
  (params (Min :type Float%20%28single-precision%29) (Random :type Float%20%28single-precision%29))
  (return (and (>= Random (+ Min (Variables|CombatStates|Probabilities|GetStrafeChance))) (< Random (+ Min (Variables|CombatStates|Probabilities|GetStrafeChance) (Variables|CombatStates|Probabilities|GetDefenceChance))))))

(fn GetAttackChance
  (params (Min :type Float%20%28single-precision%29) (Random :type Float%20%28single-precision%29))
  (return (>= Random (+ Min (Variables|CombatStates|Probabilities|GetStrafeChance) (Variables|CombatStates|Probabilities|GetDefenceChance)))))

(fn GetCombatState
  (return (Variables|CombatStates|GetCombatState)))

(fn UpdateCombatState
  (UpdateFunctions|CombatState|UpdateCombatStateChances (Variables|CombatStates|GetBehaviorRandomDeviation))
  (LocalVariables|SetMax (GetFunction|CombatState|GetCombatStateSum))
  (LocalVariables|SetRandom (Math|Random|RandomFloatinRange (LocalVariables|GetMin) (LocalVariables|GetMax)))
  (bind _index (CallFunction|CalculateProbabilities (Utilities|Array|MakeArray (Variables|CombatStates|Probabilities|GetAttackChance) (Variables|CombatStates|Probabilities|GetDefenceChance) (Variables|CombatStates|Probabilities|GetStrafeChance)) (LocalVariables|GetRandom)))
  (switch int _index
    (:Default
      (Variables|CombatStates|SetCombatState "NewEnumerator3"))
    (:0
      (Variables|CombatStates|SetCombatState "NewEnumerator3"))
    (:1
      (Variables|CombatStates|SetCombatState "NewEnumerator2"))
    (:2
      (Variables|CombatStates|SetCombatState "NewEnumerator0")))
  (return))

(fn GetAttackState
  (return (Variables|AttackState|GetAttackState)))

(fn GetAttackStateSum
  (return (+ (Variables|AttackState|GetLightAttacksChance) (Variables|AttackState|GetHeavyAttackChance))))

(fn GetSingleAttackChance
  (params (Min :type Float%20%28single-precision%29) (Random :type Float%20%28single-precision%29))
  (return (and (>= Random Min) (< Random (Variables|AttackState|GetSingleAttackChance)))))

(fn GetChargeChance
  (params (Min :type Float%20%28single-precision%29) (Random :type Float%20%28single-precision%29))
  (bind _singleattackchance (Variables|AttackState|GetSingleAttackChance))
  (return (and (>= Random (+ Min _singleattackchance)) (< Random (+ Min _singleattackchance (Variables|AttackState|GetChargeChance))))))

(fn GetComboChance
  (params (Min :type Float%20%28single-precision%29) (Random :type Float%20%28single-precision%29))
  (bind _singleattackchance (Variables|AttackState|GetSingleAttackChance))
  (bind _chargechance (Variables|AttackState|GetChargeChance))
  (return (and (>= Random (+ Min _singleattackchance _chargechance)) (< Random (+ Min _singleattackchance _chargechance (Variables|AttackState|GetComboChance))))))

(fn GetSpecialSkillChance
  (params (Min :type Float%20%28single-precision%29) (Random :type Float%20%28single-precision%29))
  (return (>= Random (+ Min (Variables|AttackState|GetSingleAttackChance) (Variables|AttackState|GetChargeChance) (Variables|AttackState|GetComboChance)))))

(fn GetGrownEfficiency
  (params (AIBehaviorStructure :type STRUCT%20AI%20Behavior%20Selection%20Structure) (Efficiency :type Float%20%28single-precision%29))
  (bind (_efficiencymethod _growthmethod _baseefficiency _basegrowth) (Utilities|Struct|BreakSTRUCT_AIBehaviorSelection AIBehaviorStructure))
  (switch Utilities|FlowControl|Switch|SwitchonENUM_AIGrowthMethod _growthmethod
    (:NewEnumerator3
      (LocalVariables|SetNewChance Efficiency))
    (:NewEnumerator0
      (LocalVariables|SetNewChance (* Efficiency _basegrowth)))
    (:NewEnumerator1
      (LocalVariables|SetNewChance (Math|Float|Clamp(Float) (Math|Float|Log Efficiency _basegrowth) 0.0 4.003012324209197e+18)))
    (:NewEnumerator2
      (LocalVariables|SetNewChance (Math|Float|Power Efficiency _basegrowth))))
  (return (LocalVariables|GetNewChance)))

(fn SetEfficiencybyMethod
  (params (AiBehaviorStruct :type STRUCT%20AI%20Behavior%20Selection%20Structure) (RandomDeviation :type Float%20%28single-precision%29))
  (bind (_efficiencymethod _growthmethod _baseefficiency) (Utilities|Struct|BreakSTRUCT_AIBehaviorSelection AiBehaviorStruct))
  (bind _returnvalue (Utilities|Array|Length _efficiencymethod))
  (LocalVariables|SetBase%20Efficiency_Ref _baseefficiency)
  (for _array_element _efficiencymethod
    (switch Utilities|FlowControl|Switch|SwitchonENUM_AIBehaviorEfficiencyMethod _array_element
      (:NewEnumerator0
        ;[1 1 1] Constant
        (bind _output_get (LocalVariables|SetEfficiency%20Sum (+ (LocalVariables|GetCurrentEfficiency) (LocalVariables|GetBase%20Efficiency_Ref))))
        (LocalVariables|SetCurrentEfficiency _output_get))
      (:NewEnumerator1
        ;[1 1 1] Random
        (bind _output_get_2 (LocalVariables|SetEfficiency%20Sum (+ (LocalVariables|GetCurrentEfficiency) (* (LocalVariables|GetBase%20Efficiency_Ref) (CallFunction|GetRandomDeviationValue RandomDeviation)))))
        (LocalVariables|SetCurrentEfficiency _output_get_2))
      (:NewEnumerator2
        ;[1 1 1] OnMaxHealth
        (bind _output_get_3 (LocalVariables|SetEfficiency%20Sum (+ (* (LocalVariables|GetBase%20Efficiency_Ref) (CallFunction|GetHealtPercentage)) (LocalVariables|GetCurrentEfficiency))))
        (LocalVariables|SetCurrentEfficiency _output_get_3))
      (:NewEnumerator3
        ;[1 1 1] OnPLayerAttack
        (if (CallFunction|IsEnemyAttacking? 5e+02)
          (bind _output_get_4 (LocalVariables|SetEfficiency%20Sum (+ (LocalVariables|GetBase%20Efficiency_Ref) (LocalVariables|GetCurrentEfficiency))))
          (LocalVariables|SetCurrentEfficiency _output_get_4)
          (else
            (bind _output_get_5 (LocalVariables|SetEfficiency%20Sum (LocalVariables|GetCurrentEfficiency)))
            (LocalVariables|SetCurrentEfficiency _output_get_5))))
      (:NewEnumerator4
        ;[1 1 1] OnPlayerBlock
        (if (CallFunction|IsEnemyBlocking?)
          (bind _output_get_6 (LocalVariables|SetEfficiency%20Sum (+ (LocalVariables|GetCurrentEfficiency) (LocalVariables|GetBase%20Efficiency_Ref))))
          (LocalVariables|SetCurrentEfficiency _output_get_6)
          (else
            (bind _output_get_7 (LocalVariables|SetEfficiency%20Sum (LocalVariables|GetCurrentEfficiency)))
            (LocalVariables|SetCurrentEfficiency _output_get_7))))
      (:NewEnumerator5
        ;[1 1 1] OnPlayer Light Attack
        (if (CallFunction|IsEnemyAttackingLight? 2e+02)
          (bind _output_get_8 (LocalVariables|SetEfficiency%20Sum (+ (LocalVariables|GetBase%20Efficiency_Ref) (LocalVariables|GetCurrentEfficiency))))
          (LocalVariables|SetCurrentEfficiency _output_get_8)
          (else
            (bind _output_get_9 (LocalVariables|SetEfficiency%20Sum (LocalVariables|GetCurrentEfficiency)))
            (LocalVariables|SetCurrentEfficiency _output_get_9))))
      (:NewEnumerator6
        ;[1 1 1] OnPlayer Heavy Attack
        (if (CallFunction|IsEnemyAttackingHeavy? 2e+02)
          (bind _output_get_10 (LocalVariables|SetEfficiency%20Sum (+ (LocalVariables|GetBase%20Efficiency_Ref) (LocalVariables|GetCurrentEfficiency))))
          (LocalVariables|SetCurrentEfficiency _output_get_10)
          (else
            (bind _output_get_11 (LocalVariables|SetEfficiency%20Sum (LocalVariables|GetCurrentEfficiency)))
            (LocalVariables|SetCurrentEfficiency _output_get_11))))))
  (if (!= _returnvalue 0)
    (LocalVariables|SetFinalEfficiency (/ (LocalVariables|GetEfficiency%20Sum) (Math|Conversions|ToFloat(Integer) _returnvalue))))
  (return (LocalVariables|GetFinalEfficiency)))

(fn GetRandomDeviationValue
  (params (Deviation :type Float%20%28single-precision%29))
  (bind _returnvalue (Math|Float|Absolute(Float) Deviation))
  (bind _returnvalue_2 (Math|Random|RandomFloatinRange 0.0 _returnvalue))
  (bind _returnvalue_3 (Math|Float|Clamp(Float) _returnvalue_2))
  (if (>= (Math|Random|RandomFloatinRange 0.0 1.0) 0.5)
    (LocalVariables|SetDev (- 1.0 _returnvalue_3))
    (else
      (LocalVariables|SetDev (+ _returnvalue_3 1.0))))
  (return (LocalVariables|GetDev)))

(fn UpdateCombatStateChances
  (params (RandomDeviation :type Float%20%28single-precision%29))
  (bind _finalefficiency1 (CallFunction|SetEfficiencybyMethod (Variables|Default|GetAIDefenceStructure) RandomDeviation))
  (bind _finalefficiency1_2 (CallFunction|SetEfficiencybyMethod (Variables|Default|GetAIStrafeStructure) RandomDeviation))
  (bind _finalefficiency1_3 (CallFunction|SetEfficiencybyMethod (Variables|Default|GetAIAttackStructure) RandomDeviation))
  (Utilities|FlowControl|Sequence
    (:then_0
      (Variables|CombatStates|Probabilities|SetDefenceChance (CallFunction|GetGrownEfficiency (Variables|Default|GetAIDefenceStructure) _finalefficiency1)))
    (:then_1
      (Variables|CombatStates|Probabilities|SetStrafeChance (CallFunction|GetGrownEfficiency (Variables|Default|GetAIStrafeStructure) _finalefficiency1_2)))
    (:then_2
      (Variables|CombatStates|Probabilities|SetAttackChance (CallFunction|GetGrownEfficiency (Variables|Default|GetAIAttackStructure) _finalefficiency1_3)))))

(fn GetHealtPercentage
  (bind _healthcomponent (Variables|Default|GethealthComponent))
  (return (/ (Default|GetCurrentValue _healthcomponent) (Default|GetMaxValue _healthcomponent))))

(fn GetOwnerEnemyCharacter
  (bind _returnvalue (Components|GetOwner))
  (if (Utilities|DoesObjectImplementInterface _returnvalue "/Game/Scripts/Blueprints/Interfaces/BP_CharacterInterface.BP_CharacterInterface_C")
    (bind _enemycharacter (Class|BPCharacterInterface|GetMyEnemyCharacter(Message) _returnvalue)))
  (return _enemycharacter))

(fn GetOwnerAiController
  (bind _asbp_aicontroller (Utilities|Casting|CastToBP_AIController (AI|GetAIController (CallFunction|GetOwnerEnemyCharacter))))
  (return _asbp_aicontroller))

(fn IsEnemyAttacking?
  (params (DistanceToCheck :type Float%20%28single-precision%29))
  (bind _returnvalue (Components|GetOwner))
  (bind _returnvalue_2 (Game|GetPlayerCharacter 0))
  (bind _asbp_enemy_master (Utilities|Casting|CastToBP_EnemyMaster _returnvalue))
  (Utilities|IsValid _returnvalue_2
    (:Is%20Valid
      (bind _asbp_character_master (Utilities|Casting|CastToBP_CharacterMaster _returnvalue_2))
      (bind _direction (Default|GetRelativeDirectionbyActor _asbp_enemy_master _asbp_enemy_master _asbp_character_master))
      (bind _output_get (LocalVariables|SetIsForward (Utilities|Select :Index _direction :NewEnumerator0 true :NewEnumerator1 true :NewEnumerator2 true :NewEnumerator3 false :NewEnumerator4 false :NewEnumerator5 false :NewEnumerator6 false :NewEnumerator7 false)))
      (return (and _output_get (and (or (Utilities|Enum|Equal(Enum) (Default|GetAnimationType (Variables|/Game/Scripts/Blueprints/Characters/BP_CharacterMaster.BP_CharacterMaster_C|GetBP_CombatComponent _asbp_character_master) (Variables|/Game/Scripts/Blueprints/Components/Animation/BP_CombatComponent.BP_CombatComponent_C|GetCurrentAnimation (Variables|/Game/Scripts/Blueprints/Characters/BP_CharacterMaster.BP_CharacterMaster_C|GetBP_CombatComponent _asbp_character_master))) "NewEnumerator2") (Utilities|Enum|Equal(Enum) (Default|GetAnimationType (Variables|/Game/Scripts/Blueprints/Characters/BP_CharacterMaster.BP_CharacterMaster_C|GetBP_CombatComponent _asbp_character_master) (Variables|/Game/Scripts/Blueprints/Components/Animation/BP_CombatComponent.BP_CombatComponent_C|GetCurrentAnimation (Variables|/Game/Scripts/Blueprints/Characters/BP_CharacterMaster.BP_CharacterMaster_C|GetBP_CombatComponent _asbp_character_master))) "NewEnumerator3")) (<= (Transformation|GetDistanceTo _asbp_character_master (Components|GetOwner)) DistanceToCheck)))))))

(fn IsEnemyBlocking?
  (bind _returnvalue (Game|GetPlayerCharacter 0))
  (Utilities|IsValid _returnvalue
    (:Is%20Valid
      (bind _asbp_character_master (Utilities|Casting|CastToBP_CharacterMaster _returnvalue))
      (return (Variables|/Game/Scripts/Blueprints/Characters/BP_CharacterMaster.BP_CharacterMaster_C|GetIsBlocking _asbp_character_master)))))

(fn UpdateAttackState
  (UpdateFunctions|AttackState|UpdateAttackStateChance (Variables|CombatStates|GetBehaviorRandomDeviation))
  (LocalVariables|SetMax (GetFunction|AttackState|GetAttackStateSum))
  (LocalVariables|SetRandom (Math|Random|RandomFloatinRange (LocalVariables|GetMin) (LocalVariables|GetMax)))
  (bind _index (CallFunction|CalculateProbabilities (Utilities|Array|MakeArray (Variables|AttackState|GetLightAttacksChance) (Variables|AttackState|GetHeavyAttackChance)) (LocalVariables|GetRandom)))
  (switch int _index
    (:Default
      (Variables|AttackState|SetAttackState "NewEnumerator4"))
    (:0
      (Variables|AttackState|SetAttackState "NewEnumerator4"))
    (:1
      (Variables|AttackState|SetAttackState "NewEnumerator5")))
  (return))

(fn UpdateAttackStateChance
  (params (RandomDeviation :type Float%20%28single-precision%29))
  (bind _finalefficiency1 (CallFunction|SetEfficiencybyMethod (Variables|Default|GetAILightAttackStructure) RandomDeviation))
  (bind _finalefficiency1_2 (CallFunction|SetEfficiencybyMethod (Variables|Default|GetAIHeavyAttackStructure) RandomDeviation))
  (Utilities|FlowControl|Sequence
    (:then_0
      (Variables|AttackState|SetLightAttacksChance (CallFunction|GetGrownEfficiency (Variables|Default|GetAILightAttackStructure) _finalefficiency1)))
    (:then_1
      (Variables|AttackState|SetHeavyAttackChance (CallFunction|GetGrownEfficiency (Variables|Default|GetAIHeavyAttackStructure) _finalefficiency1_2)))))

(fn GetLightAttackChance
  (params (Min :type Float%20%28single-precision%29) (Random :type Float%20%28single-precision%29))
  (return (and (>= Random Min) (< Random (Variables|AttackState|GetLightAttacksChance)))))

(fn GetPercentagebyRange
  (params (NewParam :type Array%20of%20Floats%20%28single-precision%29)))

(fn GetHeavyAttackChance
  (params (Min :type Float%20%28single-precision%29) (Random :type Float%20%28single-precision%29))
  (return (and (>= Random Min) (< Random (Variables|AttackState|GetHeavyAttackChance)))))

(fn UpdateDefenceState
  (UpdateFunctions|DefenceState|UpdateDefenceStateChance (Variables|CombatStates|GetBehaviorRandomDeviation))
  (LocalVariables|SetMax (GetFunction|DefenceState|GetDefenceStateSm))
  (LocalVariables|SetRandom (Math|Random|RandomFloatinRange (LocalVariables|GetMin) (LocalVariables|GetMax)))
  (bind _index (CallFunction|CalculateProbabilities (Utilities|Array|MakeArray (Variables|AttackState|GetDodgeChance) (Variables|AttackState|GetBlockChance)) (LocalVariables|GetRandom)))
  (switch int _index
    (:Default
      (Variables|Default|SetDefenceState "NewEnumerator0"))
    (:0
      (Variables|Default|SetDefenceState "NewEnumerator0"))
    (:1
      (Variables|Default|SetDefenceState "NewEnumerator1")))
  (return))

(fn UpdateDefenceStateChance
  (params (RandomDeviation :type Float%20%28single-precision%29))
  (bind _finalefficiency1 (CallFunction|SetEfficiencybyMethod (Variables|Default|GetAIDodgeStructure) RandomDeviation))
  (bind _finalefficiency1_2 (CallFunction|SetEfficiencybyMethod (Variables|Default|GetAIBlockStructure) RandomDeviation))
  (Utilities|FlowControl|Sequence
    (:then_0
      (Variables|AttackState|SetDodgeChance (CallFunction|GetGrownEfficiency (Variables|Default|GetAIDodgeStructure) _finalefficiency1)))
    (:then_1
      (Variables|AttackState|SetBlockChance (CallFunction|GetGrownEfficiency (Variables|Default|GetAIBlockStructure) _finalefficiency1_2)))))

(fn GetDodgeChance
  (params (Min :type Float%20%28single-precision%29) (Random :type Float%20%28single-precision%29))
  (return (and (>= Random Min) (< Random (Variables|AttackState|GetDodgeChance)))))

(fn GetBlockChance
  (params (Min :type Float%20%28single-precision%29) (Random :type Float%20%28single-precision%29))
  (return (and (>= Random Min) (< Random (Variables|AttackState|GetBlockChance)))))

(fn IsEnemyAttackingLight?
  (params (DistanceToCheck :type Float%20%28single-precision%29))
  (bind _returnvalue (Game|GetPlayerCharacter 0))
  (Utilities|IsValid _returnvalue
    (:Is%20Valid
      (bind _asbp_character_master (Utilities|Casting|CastToBP_CharacterMaster _returnvalue))
      (return (and (Utilities|Enum|Equal(Enum) (Default|GetAnimationType (Variables|/Game/Scripts/Blueprints/Characters/BP_CharacterMaster.BP_CharacterMaster_C|GetBP_CombatComponent _asbp_character_master) (Variables|/Game/Scripts/Blueprints/Components/Animation/BP_CombatComponent.BP_CombatComponent_C|GetCurrentAnimation (Variables|/Game/Scripts/Blueprints/Characters/BP_CharacterMaster.BP_CharacterMaster_C|GetBP_CombatComponent _asbp_character_master))) "NewEnumerator2") (<= (Transformation|GetDistanceTo _asbp_character_master (Components|GetOwner)) DistanceToCheck))))))

(fn IsEnemyAttackingHeavy?
  (params (DistanceToCheck :type Float%20%28single-precision%29))
  (bind _returnvalue (Game|GetPlayerCharacter 0))
  (Utilities|IsValid _returnvalue
    (:Is%20Valid
      (bind _asbp_character_master (Utilities|Casting|CastToBP_CharacterMaster _returnvalue))
      (return (and (Utilities|Enum|Equal(Enum) (Default|GetAnimationType (Variables|/Game/Scripts/Blueprints/Characters/BP_CharacterMaster.BP_CharacterMaster_C|GetBP_CombatComponent _asbp_character_master) (Variables|/Game/Scripts/Blueprints/Components/Animation/BP_CombatComponent.BP_CombatComponent_C|GetCurrentAnimation (Variables|/Game/Scripts/Blueprints/Characters/BP_CharacterMaster.BP_CharacterMaster_C|GetBP_CombatComponent _asbp_character_master))) "NewEnumerator3") (<= (Transformation|GetDistanceTo _asbp_character_master (Components|GetOwner)) DistanceToCheck))))))

(fn GetDefenceStateSm
  (return (+ (Variables|AttackState|GetDodgeChance) (Variables|AttackState|GetBlockChance))))

(fn CalculateProbabilities
  (params (Array :type Array%20of%20Floats%20%28single-precision%29) (Random :type Float%20%28single-precision%29))
  (LocalVariables|SetArray_LocalRef Array)
  (LocalVariables|SetRandomNumber Random)
  (bind (_array_element _array_index) (Utilities|Array|ForEachLoopwithBreak (LocalVariables|GetArray_LocalRef) :!label _label)
    (:LoopBody
      (LocalVariables|SetCurrentIndex _array_index)
      (if (> _array_index 0)
        (LocalVariables|SetArraySum (+ (Utilities|Array|Get(acopy) (LocalVariables|GetArray_LocalRef) (LocalVariables|GetCurrentIndex)) (Utilities|Array|Get(acopy) (LocalVariables|GetArray_LocalRef) (- (LocalVariables|GetCurrentIndex) 1))))
        (else
          (LocalVariables|SetArraySum _array_element)))
      (if (<= (LocalVariables|GetRandomNumber) (LocalVariables|GetArraySum))
        (LocalVariables|SetReturnIndex (LocalVariables|GetCurrentIndex))
        (goto _label Break)))
    (:Completed
      (return (LocalVariables|GetReturnIndex)))))