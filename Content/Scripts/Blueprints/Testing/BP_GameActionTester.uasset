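; Test actor that applies a gameplay action to whatever actor enters its Box trigger.
; Begin overlap runs SingleTargetGameplayAction with the ConsumeHealthAndStamina data on that actor; end overlap does nothing, and a RestoreHealthAndStamina call is left unconnected.
; The construction script gives the Cube a dynamic MI_Dust material driven by the Color and Opacity variables, with Color setting both base and emissive color.
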(event OnComponentBeginOverlap(Box)
  (params (OverlappedComponent :type Primitive%20Component%20Object%20Reference) (OtherActor :type Actor%20Object%20Reference) (OtherComp :type Primitive%20Component%20Object%20Reference) (OtherBodyIndex :type Integer) (bFromSweep :type Boolean) (SweepResult :type Hit%20Result%20Structure%20%28by%20ref%29))
  (CallFunction|SingleTargetGameplayAction OtherActor (Variables|Default|GetConsumeHealthAndStamina) false))

(event OnComponentEndOverlap(Box)
  (params (OverlappedComponent :type Primitive%20Component%20Object%20Reference) (OtherActor :type Actor%20Object%20Reference) (OtherComp :type Primitive%20Component%20Object%20Reference) (OtherBodyIndex :type Integer)))

(event EventBeginPlay)

(event Collision|EventActorBeginOverlap
  (params (OtherActor :type Actor%20Object%20Reference)))

(event EventTick
  (params (DeltaSeconds :type Float%20%28single-precision%29)))

(fn ConstructionScript
  (bind _color (Variables|Default|GetColor))
  (bind _returnvalue (Rendering|Material|CreateDynamicMaterialInstance (Variables|Default|GetCube) 0 "/Game/Scripts/Materials/Instances/Dungeon/Misc/MI_Dust.MI_Dust" "None" :!class /Script/Engine.PrimitiveComponent))
  (bind _output_get (Variables|Default|SetMaterialDynamic _returnvalue))
  (Rendering|Material|SetScalarParameterValue _output_get "Opacity" (Variables|Default|GetOpacity) :!class /Script/Engine.MaterialInstanceDynamic)
  (Rendering|Material|SetVectorParameterValue _output_get "BaseColor" _color :!class /Script/Engine.MaterialInstanceDynamic)
  (Rendering|Material|SetVectorParameterValue _output_get "EmissiveColor" _color :!class /Script/Engine.MaterialInstanceDynamic))