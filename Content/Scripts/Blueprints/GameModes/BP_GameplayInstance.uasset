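; BP_GameplayInstance holds and updates game-wide state for a hero management and dungeon game: resources, hero rosters, week count and checkpoint use.
; Dungeon loot is added to global resources minus the gods' share, which scales with checkpoints used.
; Weekly recovery heals infirmary heroes and restores tavern stamina using building-level curves, returning recovered heroes to the roster.
; Curve-driven experience levels up the selected hero, capped at level 10.
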(fn ResetSelctedHerotoNone
  (bind _structout (Utilities|Struct|SetmembersinSTRUCT_HeroesData (Variables|Default|GetSelectedHero) "NewEnumerator2"))
  (Variables|Default|SetSelectedHero _structout))

(fn GetCurrentResource
  (params (ResourceType :type ENUM_ResourceType%20Enum :default "NewEnumerator0"))
  (switch Utilities|FlowControl|Switch|SwitchonENUM_ResourceType ResourceType
    (:NewEnumerator0
      (LocalVariables|SetCurrent (.currentquantity (Utilities|Array|Get(acopy) (Variables|Default|GetStruct_Resources)))))
    (:NewEnumerator1
      (LocalVariables|SetCurrent (.currentquantity (Utilities|Array|Get(acopy) (Variables|Default|GetStruct_Resources) 1))))
    (:NewEnumerator2
      (LocalVariables|SetCurrent (.currentquantity (Utilities|Array|Get(acopy) (Variables|Default|GetStruct_Resources) 2))))
    (:NewEnumerator3
      (LocalVariables|SetCurrent (.currentquantity (Utilities|Array|Get(acopy) (Variables|Default|GetStruct_Resources) 3)))))
  (return (LocalVariables|GetCurrent)))

(fn GetInnStaminarecovery
  (return (Math|Curves|GetFloatValue (Variables|Inn|GetStaminaRecoveryCurve) (Math|Conversions|ToFloat(Integer) (Variables|Inn|GetInnLevel)))))

(fn SortArraybyDecrescentValueInteger
  (params (Array :type Array%20of%20Integers))
  (bind _newarray (LocalVariables|GetNewArray))
  (for _array_element Array
    (Utilities|Array|Add _newarray _array_element)
    (for (_array_element_2 _array_index) _newarray
      (if (> _array_index 0)
        (if (< (Utilities|Array|Get(acopy) _newarray (- _array_index 1)) _array_element_2)
          (LocalVariables|SetCurrentMax _array_element_2)
          (LocalVariables|SetCurrentMin 0))))))

(fn ResetDungeonResourceArray
  (bind _struct_dungeonresources (Variables|Default|GetStruct_DungeonResources))
  (for (_array_element _array_index) _struct_dungeonresources
    (bind _structout (Utilities|Struct|SetmembersinStruct_Resources _array_element))
    (Utilities|Array|SetArrayElem _struct_dungeonresources _array_index _structout)
    (Utilities|Array|SetArrayElem (Variables|Default|GetStruct_ResourceToGods) _array_index _structout)))

(fn UpdateResourcetoGods
  (params (CheckpointUsed :type Integer) (PercentageMultiplier :type Float%20%28single-precision%29))
  (bind _struct_resourcetogods (Variables|Default|GetStruct_ResourceToGods))
  (LocalVariables|SetPercentage (/ (* CheckpointUsed PercentageMultiplier) 1e+02))
  (for (_array_element _array_index) _struct_resourcetogods
    (bind _structout (Utilities|Struct|SetmembersinStruct_Resources _array_element (Math|Float|Round (* (.currentquantity (Utilities|Array|Get(acopy) (Variables|Default|GetStruct_DungeonResources) _array_index)) (LocalVariables|GetPercentage)))))
    (Utilities|Array|SetArrayElem _struct_resourcetogods _array_index _structout)))

(fn UpdateGlobalResource
  (bind _struct_resources (Variables|Default|GetStruct_Resources))
  (for (_array_element _array_index) _struct_resources
    (bind _structout (Utilities|Struct|SetmembersinStruct_Resources _array_element (+ (.CurrentQuantity (Utilities|Struct|BreakStruct_Resources _array_element)) (Math|Integer|Clamp(Integer) (- (.currentquantity (Utilities|Array|Get(acopy) (Variables|Default|GetStruct_DungeonResources) _array_index)) (.currentquantity (Utilities|Array|Get(acopy) (Variables|Default|GetStruct_ResourceToGods) _array_index))) 0 99999999))))
    (Utilities|Array|SetArrayElem _struct_resources _array_index _structout)))

(fn WeeklyHealthRecovery
  (bind _heroesininfirmary (Variables|Infirmary|GetHeroesInInfirmary))
  (for (_array_element _array_index) (Variables|Infirmary|GetHeroesInInfirmary)
    (LocalVariables|SetCurrentIndex_ _array_index)
    (bind _structout (Utilities|Struct|SetmembersinSTRUCT_HeroesData _array_element (Utilities|Struct|MakeSTRUCT_GameAttribute (.minvalue (.Health (Utilities|Struct|BreakSTRUCT_HeroesData _array_element))) (.maxvalue (.Health (Utilities|Struct|BreakSTRUCT_HeroesData _array_element))) (.startvalue (.Health (Utilities|Struct|BreakSTRUCT_HeroesData _array_element))) (Math|Float|Clamp(Float) (+ (.currentvalue (.Health (Utilities|Struct|BreakSTRUCT_HeroesData _array_element))) (* (.maxvalue (.Health (Utilities|Struct|BreakSTRUCT_HeroesData _array_element))) (CallFunction|GetInfirmaryHealthRecovery))) 0.0 (.maxvalue (.Health (Utilities|Struct|BreakSTRUCT_HeroesData _array_element)))) (.modifierpersecond (.Health (Utilities|Struct|BreakSTRUCT_HeroesData _array_element))) (.bcanbeconsumed (.Health (Utilities|Struct|BreakSTRUCT_HeroesData _array_element))) (.bcanberestored (.Health (Utilities|Struct|BreakSTRUCT_HeroesData _array_element))) 0)))
    (Utilities|Array|SetArrayElem _heroesininfirmary (LocalVariables|GetCurrentIndex_) _structout)
    (if (>= (.currentvalue (.Health (Utilities|Struct|BreakSTRUCT_HeroesData (Utilities|Array|Get(acopy) _heroesininfirmary (LocalVariables|GetCurrentIndex_))))) (.maxvalue (.Health (Utilities|Struct|BreakSTRUCT_HeroesData (Utilities|Array|Get(acopy) _heroesininfirmary (LocalVariables|GetCurrentIndex_))))))
      (bind _structout_2 (Utilities|Struct|SetmembersinSTRUCT_HeroesData (Utilities|Array|Get(acopy) _heroesininfirmary (LocalVariables|GetCurrentIndex_)) "NewEnumerator1"))
      (Utilities|Array|SetArrayElem (Variables|Infirmary|GetHeroesInInfirmary) (LocalVariables|GetCurrentIndex_) _structout_2)
      (Utilities|Array|Add (LocalVariables|GetHeroesToRemove) _structout_2)))
  (for _array_element_2 (LocalVariables|GetHeroesToRemove)
    (Utilities|Array|Add (Variables|Default|GetStruct_Heroes) _array_element_2)
    (Utilities|Array|RemoveItem (Variables|Infirmary|GetHeroesInInfirmary) _array_element_2)))

(fn GetInfirmaryHealthRecovery
  (return (Math|Curves|GetFloatValue (Variables|Infirmary|GetHealthRecoveryCurve) (Math|Conversions|ToFloat(Integer) (Variables|Infirmary|GetInfirmaryLevel)))))

(fn WeeklyStaminaRecovery
  (bind _heroesintavern (Variables|Inn|GetHeroesInTavern))
  (for (_array_element _array_index) (Variables|Inn|GetHeroesInTavern)
    (LocalVariables|SetCurrentIndex_ _array_index)
    (bind _structout (Utilities|Struct|SetmembersinSTRUCT_HeroesData _array_element (Utilities|Struct|MakeSTRUCT_GameAttribute (.minvalue (.Stamina (Utilities|Struct|BreakSTRUCT_HeroesData _array_element))) (.maxvalue (.Stamina (Utilities|Struct|BreakSTRUCT_HeroesData _array_element))) (.startvalue (.Stamina (Utilities|Struct|BreakSTRUCT_HeroesData _array_element))) (Math|Float|Clamp(Float) (+ (.currentvalue (.Stamina (Utilities|Struct|BreakSTRUCT_HeroesData _array_element))) (* (.maxvalue (.Stamina (Utilities|Struct|BreakSTRUCT_HeroesData _array_element))) (CallFunction|GetInnStaminarecovery))) 0.0 (.maxvalue (.Stamina (Utilities|Struct|BreakSTRUCT_HeroesData _array_element)))) (.modifierpersecond (.Stamina (Utilities|Struct|BreakSTRUCT_HeroesData _array_element))) (.bcanbeconsumed (.Stamina (Utilities|Struct|BreakSTRUCT_HeroesData _array_element))) (.bcanberestored (.Stamina (Utilities|Struct|BreakSTRUCT_HeroesData _array_element))) 0)))
    (Utilities|Array|SetArrayElem _heroesintavern (LocalVariables|GetCurrentIndex_) _structout)
    (if (>= (.currentvalue (.Stamina (Utilities|Struct|BreakSTRUCT_HeroesData (Utilities|Array|Get(acopy) _heroesintavern (LocalVariables|GetCurrentIndex_))))) (.maxvalue (.Stamina (Utilities|Struct|BreakSTRUCT_HeroesData (Utilities|Array|Get(acopy) _heroesintavern (LocalVariables|GetCurrentIndex_))))))
      (bind _structout_2 (Utilities|Struct|SetmembersinSTRUCT_HeroesData (Utilities|Array|Get(acopy) _heroesintavern (LocalVariables|GetCurrentIndex_)) "NewEnumerator1"))
      (Utilities|Array|SetArrayElem (Variables|Inn|GetHeroesInTavern) (LocalVariables|GetCurrentIndex_) _structout_2)
      (Utilities|Array|Add (LocalVariables|GetHeroesToRemove) _structout_2)))
  (for _array_element_2 (LocalVariables|GetHeroesToRemove)
    (Utilities|Array|Add (Variables|Default|GetStruct_Heroes) _array_element_2)
    (Utilities|Array|RemoveItem (Variables|Inn|GetHeroesInTavern) _array_element_2)))

(fn IncreaseUsedCheckpoints
  (Variables|Dungeon|SetUsedCheckpoints (+ (Variables|Dungeon|GetUsedCheckpoints) 1)))

(fn ResetCheckpoints
  (Variables|Dungeon|SetUsedCheckpoints 0))

(fn IncreaseGameWeek
  (Variables|Default|SetGameWeek (+ (Variables|Default|GetGameWeek) 1))
  (Variables|Academy|SetVolunteerRecruited false))

(fn GetHeroExpValueRange
  (params (STRUCT_GameAttribute :type STRUCT%20Game%20Attribute%20Structure%20%28by%20ref%29))
  (bind _growthcurve (Utilities|Struct|BreakSTRUCT_GameAttribute STRUCT_GameAttribute))
  (bind (_minvalue _maxvalue) (Class|CurveBase|GetValueRange _growthcurve))
  (return _minvalue _maxvalue))

(fn GetHeroExpLevelRange
  (params (STRUCT_GameAttribute :type STRUCT%20Game%20Attribute%20Structure%20%28by%20ref%29))
  (bind _growthcurve (Utilities|Struct|BreakSTRUCT_GameAttribute STRUCT_GameAttribute))
  (bind (_mintime _maxtime) (Math|Curves|GetTimeRange _growthcurve))
  (return _mintime _maxtime))

(fn SetExperienceCurrentValue
  (params (Hero :type STRUCT%20Heroes%20Data%20Structure) (CurrentValue :type Float%20%28single-precision%29))
  (bind _output_get (LocalVariables|SetLocalHero Hero))
  (bind _structout (Utilities|Struct|SetmembersinSTRUCT_GameAttribute (.Experience (Utilities|Struct|BreakSTRUCT_HeroesData _output_get)) CurrentValue))
  (bind _structout_2 (Utilities|Struct|SetmembersinSTRUCT_HeroesData (Variables|Default|GetSelectedHero) _structout))
  (bind _output_get_2 (LocalVariables|SetLocalHero _structout_2))
  (return _output_get_2))

(fn GetNextLevelExperienceNeeded
  (params (Hero :type STRUCT%20Heroes%20Data%20Structure))
  (bind (_icon _health _stamina _experience _level) (Utilities|Struct|BreakSTRUCT_HeroesData Hero))
  (return (Math|Curves|GetFloatValue (.growthcurve _experience) (Math|Conversions|ToFloat(Integer) (+ _level 1)))))

(fn SetAllHeroesExperienceLimits
  (Utilities|FlowControl|Sequence
    (:then_0
      (for (_array_element _array_index) (Variables|Default|GetStruct_Heroes)
        (bind _structout (Utilities|Struct|SetmembersinSTRUCT_GameAttribute (.Experience (Utilities|Struct|BreakSTRUCT_HeroesData _array_element)) (.MinValue (Experience|GetHeroExpValueRange (.Experience (Utilities|Struct|BreakSTRUCT_HeroesData _array_element)))) (.MaxValue (Experience|GetHeroExpValueRange (.Experience (Utilities|Struct|BreakSTRUCT_HeroesData _array_element))))))
        (bind _structout_2 (Utilities|Struct|SetmembersinSTRUCT_HeroesData (Utilities|Array|Get(acopy) (Variables|Default|GetStruct_Heroes) _array_index) _structout))
        (Utilities|Array|SetArrayElem (Variables|Default|GetStruct_Heroes) _array_index _structout_2)))
    (:then_1
      (for (_array_element_2 _array_index_2) (Variables|Infirmary|GetHeroesInInfirmary)
        (bind _structout_3 (Utilities|Struct|SetmembersinSTRUCT_GameAttribute (.Experience (Utilities|Struct|BreakSTRUCT_HeroesData _array_element_2)) (.MinValue (Experience|GetHeroExpValueRange (.Experience (Utilities|Struct|BreakSTRUCT_HeroesData _array_element_2)))) (.MaxValue (Experience|GetHeroExpValueRange (.Experience (Utilities|Struct|BreakSTRUCT_HeroesData _array_element_2))))))
        (bind _structout_4 (Utilities|Struct|SetmembersinSTRUCT_HeroesData (Utilities|Array|Get(acopy) (Variables|Infirmary|GetHeroesInInfirmary) _array_index_2) _structout_3))
        (Utilities|Array|SetArrayElem (Variables|Infirmary|GetHeroesInInfirmary) _array_index_2 _structout_4)))
    (:then_2
      (for (_array_element_3 _array_index_3) (Variables|Inn|GetHeroesInTavern)
        (bind _structout_5 (Utilities|Struct|SetmembersinSTRUCT_GameAttribute (.Experience (Utilities|Struct|BreakSTRUCT_HeroesData _array_element_3)) (.MinValue (Experience|GetHeroExpValueRange (.Experience (Utilities|Struct|BreakSTRUCT_HeroesData _array_element_3)))) (.MaxValue (Experience|GetHeroExpValueRange (.Experience (Utilities|Struct|BreakSTRUCT_HeroesData _array_element_3))))))
        (bind _structout_6 (Utilities|Struct|SetmembersinSTRUCT_HeroesData (Utilities|Array|Get(acopy) (Variables|Inn|GetHeroesInTavern) _array_index_3) _structout_5))
        (Utilities|Array|SetArrayElem (Variables|Inn|GetHeroesInTavern) _array_index_3 _structout_6)))))

(fn LevelUp?
  (params (Hero :type STRUCT%20Heroes%20Data%20Structure))
  (return (>= (Experience|GetCurrentExperience Hero) (Experience|GetNextLevelExperienceNeeded Hero))))

(fn GetCurrentExperience
  (params (Hero :type STRUCT%20Heroes%20Data%20Structure))
  (return (.currentvalue (.experience Hero))))

(fn UpdateHeroLevels
  (params (Hero :type STRUCT%20Heroes%20Data%20Structure) (ExpToAssign :type Float%20%28single-precision%29))
  (LocalVariables|SetLocalHero Hero)
  (if (Experience|MaxlevelReached? (LocalVariables|GetLocalHero) 10)
    _
    (else
      (bind _newherostruct (Experience|SetExperienceCurrentValue :CurrentValue (+ ExpToAssign (Experience|GetCurrentExperience (LocalVariables|GetLocalHero)))))
      (LocalVariables|SetLocalHero _newherostruct)
      (if (Experience|LevelUp? (LocalVariables|GetLocalHero)) :!label _label
        (bind _newhero (Experience|IncreaseHeroLevel (LocalVariables|GetLocalHero)))
        (LocalVariables|SetLocalHero _newhero)
        (if (Experience|MaxlevelReached? (LocalVariables|GetLocalHero) 10)
          _
          (else
            (goto _label)))
        (else
          (return (LocalVariables|GetLocalHero))))))
  (return (LocalVariables|GetLocalHero)))

(fn IncreaseHeroLevel
  (params (Hero :type STRUCT%20Heroes%20Data%20Structure))
  (bind _structout (Utilities|Struct|SetmembersinSTRUCT_HeroesData Hero (+ (.Level (Utilities|Struct|BreakSTRUCT_HeroesData Hero)) 1)))
  (return _structout))

(fn MaxlevelReached?
  (params (Hero :type STRUCT%20Heroes%20Data%20Structure) (MaxLevel :type Integer))
  (return (>= (.Level (Utilities|Struct|BreakSTRUCT_HeroesData Hero)) MaxLevel)))

(fn UpdateSelectedHeroLevels
  (bind _newhero (Experience|UpdateHeroLevels (Variables|Default|GetSelectedHero) (CallFunction|GetDungeonLevelExperience)))
  (Variables|Default|SetSelectedHero _newhero))

(fn GetDungeonLevelExperience
  (return (Math|Curves|GetFloatValue (Variables|Dungeon|GetDungeonExperienceCurve) (Math|Conversions|ToFloat(Integer) (Variables|Dungeon|GetDungeonLevel)))))

(fn CalculateProbabilities
  (params (Array :type Array%20of%20Floats%20%28single-precision%29) (Random :type Float%20%28single-precision%29))
  (LocalVariables|SetArray_LocalRef Array)
  (LocalVariables|SetRandomNumber Random)
  (bind (_array_element _array_index) (Utilities|Array|ForEachLoopwithBreak (LocalVariables|GetArray_LocalRef) :!label _label)
    (:LoopBody
      (LocalVariables|SetCurrentIndex _array_index)
      (if (> _array_index 0)
        (LocalVariables|SetArraySum (+ (Utilities|Array|Get(acopy) (LocalVariables|GetArray_LocalRef) (LocalVariables|GetCurrentIndex)) (Utilities|Array|Get(acopy) (LocalVariables|GetArray_LocalRef) (- (LocalVariables|GetCurrentIndex) 1))))
        (else
          (LocalVariables|SetArraySum _array_element)))
      (if (<= (LocalVariables|GetRandomNumber) (LocalVariables|GetArraySum))
        (LocalVariables|SetReturnIndex (LocalVariables|GetCurrentIndex))
        (goto _label Break)))
    (:Completed
      (return (LocalVariables|GetReturnIndex)))))