(event Custom|OnInitialChunksLoaded
  (params (Dungeon :type Dungeon%20Object%20Reference))
  ;[1 1 1] Set a flag after the initial chunks are loaded. Our game starts after this. (See ReadToStartMatch function)
  (Variables|Default|SetInitialChunksLoaded true))

(event Custom|BuildDungeonServer
  (bind _returnvalue (Game|Player|GetPlayerPawn 0))
  (Networking|SwitchHasAuthority
    (:Authority
      ;[1 1 1] Grab the Dungeon Actor
      (bind _returnvalue_2 (Actor|GetActorOfClass "/Script/DungeonArchitectRuntime.Dungeon"))
      (bind _output_get (Variables|Default|SetDungeon _returnvalue_2))
      (Utilities|IsValid _output_get
        (:Is%20Valid
          (Utilities|FlowControl|Sequence
            (:then_0
              ;[1 1 1] Set a flag after the initial chunks are loaded. Our game starts after this. (See ReadToStartMatch function)
              (EventDispatchers|BindEventtoOnDungeonBuildComplete (Variables|Default|GetDungeon) (delegate Custom|OnDungeonComplete))
              (EventDispatchers|BindEventtoOnInitialChunksLoaded (Variables|/Script/DungeonArchitectRuntime.Dungeon|GetLevelStreamingModel (Variables|Default|GetDungeon)) (delegate Custom|OnInitialChunksLoaded)))
            (:then_1
              ;[1 1 1] Move the spectate camera to the player start and destroy it.  The initial dungeon will be built around this
              (bind _returnvalue_3 (Actor|GetActorOfClass "/Script/Engine.PlayerStart"))
              (Utilities|IsValid _returnvalue_3
                (:Is%20Valid
                  (Utilities|IsValid _returnvalue
                    (:Is%20Valid
                      (Transformation|Teleport _returnvalue (Transformation|GetActorLocation _returnvalue_3) "0, 0, 0"))
                    (:Is%20Not%20Valid
                      _))
                  (Actor|DestroyActor _returnvalue_3))))
            (:then_2
              ;[1 1 1] Build the dungeon
              (Variables|/Script/DungeonArchitectRuntime.DungeonConfig|SetSeed (Variables|/Script/DungeonArchitectRuntime.Dungeon|GetConfig (Variables|Default|GetDungeon)) (Math|Random|RandomInteger 1000000))
              (Class|Dungeon|BuildDungeon (Variables|Default|GetDungeon)))))
        (:Is%20Not%20Valid
          (Variables|Default|SetInitialChunksLoaded true)
          (Variables|Default|SetDungeonComplete true))))))

(event Custom|OnDungeonComplete
  (params (Dungeon :type Dungeon%20Object%20Reference))
  ;[1 1 1] Set a flag after the initial chunks are loaded. Our game starts after this. (See ReadToStartMatch function)
  (Variables|Default|SetDungeonComplete true))

(event EventBeginPlay
  (CallFunction|BuildDungeonServer))

(fn ConstructionScript)

(fn ReadytoStartMatch
  (if (Networking|IsDedicatedServer)
    (return (> (Utilities|Time|GetTimeSeconds) (Variables|Default|GetDedicatedServerInitialWaitTime)))
    (else
      (return (and (Variables|Default|GetInitialChunksLoaded) (Variables|Default|GetDungeonComplete))))))

(fn ChoosePlayerStart
  (params (Player :type Controller%20Object%20Reference))
  (bind _returnvalue (Actor|GetActorOfClass "/Script/Engine.PlayerStart"))
  (return _returnvalue))