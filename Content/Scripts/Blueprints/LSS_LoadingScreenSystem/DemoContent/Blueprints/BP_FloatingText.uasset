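; BP_FloatingText is a demo actor for the Loading Screen System that bobs vertically and can pulse in scale.
; A Movement timeline starts on BeginPlay and adds a Z offset each update from its Alpha times Bounce.
; With Pulse enabled, the same Alpha drives a slight uniform scale change only while the loop counter is zero.
; The timeline's Loop event increments that counter and resets it after PulseInterval, spacing out the pulses.
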(event EventBeginPlay
  (bind _alpha (Timeline|Movement PlayFromStart)
    (:Update
      ;[1 1 1] Bounce
      (Transformation|AddActorWorldOffset (Math|Vector|MakeVector 0.0 0.0 (* _alpha (Variables|Default|GetBounce))))
      (if (Variables|Default|GetPulse)
        ;[1 1 1] Set Scale
        (if (== (Variables|Default|GetLoops) 0)
          (Transformation|SetActorScale3D (Math|Conversions|ToVector(Float) (Math|Float|MapRangeClamped _alpha 0.95 1.0 0.95 1.0))))))
    (:Loop
      ;[1 1 1] Reset Interval for scale
      (bind _result (Math|Integer|IncrementInt (Variables|Default|GetLoops))
        (:%20%20
          (if (> _result (Variables|Default|GetPulse%20Interval))
            (Variables|Default|SetLoops 0)))))))

(event EventTick
  (params (DeltaSeconds :type Float%20%28single-precision%29)))

(fn ConstructionScript)