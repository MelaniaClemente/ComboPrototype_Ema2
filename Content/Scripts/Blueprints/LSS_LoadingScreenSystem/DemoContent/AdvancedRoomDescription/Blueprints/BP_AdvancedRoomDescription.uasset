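; Demo-room description stand that shows title, subtitle, description and bottom text with a typewriter effect, started on BeginPlay or pawn overlap.
; Construction script wraps text, tints the base and creates dynamic materials.
; Play types items simultaneously through reusable BP_TypewriterInstance child actors or sequentially with sound, while the Glow timeline animates emissive and color, reversing on overlap end.
; A configurable key possesses a found or spawned BP_ShowCaseCamera pawn.
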(event OnComponentBeginOverlap(TypeWriterBox)
  (params (OverlappedComponent :type Primitive%20Component%20Object%20Reference) (OtherActor :type Actor%20Object%20Reference) (OtherComp :type Primitive%20Component%20Object%20Reference) (OtherBodyIndex :type Integer) (bFromSweep :type Boolean) (SweepResult :type Hit%20Result%20Structure%20%28by%20ref%29))
  ;[1 1 1] Activate On OverlapO
  (Utilities|Casting|CastToPawn OtherActor)
  (if (Variables|TypewriterSettings|GetStart%20Typewriter%20On%20Overlap)
    (CallFunction|Play)))

(event OnComponentEndOverlap(TypeWriterBox)
  (params (OverlappedComponent :type Primitive%20Component%20Object%20Reference) (OtherActor :type Actor%20Object%20Reference) (OtherComp :type Primitive%20Component%20Object%20Reference) (OtherBodyIndex :type Integer))
  ;[1 1 1] Deactivate On Overlap
  (Utilities|Casting|CastToPawn OtherActor)
  (CallFunction|ReverseAnimation))

(event Custom|Init%20Text%20Materials)

(event Custom|Play
  ;[1 1 1] Start Effect (Material Animation + Typewriter)
  (Utilities|FlowControl|Sequence
    (:then_0
      (if (Variables|TypewriterSettings|GetOneshot%20Typewriter)
        (Utilities|FlowControl|DoOnce false
          (:Completed
            _)))
      (Utilities|StartTyping))
    (:then_1
      (CallFunction|PlayAnimation))))

(event Custom|Reverse%20Animation
  ;[1 1 1] Animation
  (Components|Timeline|SetPlayRate (Variables|Default|GetGlow) 0.5)
  (bind (_direction _alpha) (Timeline|Glow Reverse)
    (:Update
      (for _array_element (Variables|Private|GetTextObjects)
        (CallFunction|UpdateMaterials (.DynamicMaterialInstance (Utilities|Struct|BreakS_WrappedTextGroup _array_element)) (.TestSettings (Utilities|Struct|BreakS_WrappedTextGroup _array_element)) _alpha)))
    (:Start
      ;[1 1 1] On Anim Start
      (if (and (Utilities|Enum|Equal(Enum) _direction "Forward") (Variables|TypewriterSettings|GetPlay%20Sound%20On%20Activate))
        (Audio|PlaySoundatLocation (Variables|TypewriterSettings|GetActivation%20Sound) (Transformation|GetActorLocation) "0, 0, 0" 1.0 1.0 0.0 0 0 0)))))

(event Custom|Play%20Animation
  ;[1 1 1] Animation
  (Components|Timeline|SetPlayRate (Variables|Default|GetGlow) 0.75)
  (bind (_direction _alpha) (Timeline|Glow Play)
    (:Update
      (for _array_element (Variables|Private|GetTextObjects)
        (CallFunction|UpdateMaterials (.DynamicMaterialInstance (Utilities|Struct|BreakS_WrappedTextGroup _array_element)) (.TestSettings (Utilities|Struct|BreakS_WrappedTextGroup _array_element)) _alpha)))
    (:Start
      ;[1 1 1] On Anim Start
      (if (and (Utilities|Enum|Equal(Enum) _direction "Forward") (Variables|TypewriterSettings|GetPlay%20Sound%20On%20Activate))
        (Audio|PlaySoundatLocation (Variables|TypewriterSettings|GetActivation%20Sound) (Transformation|GetActorLocation) "0, 0, 0" 1.0 1.0 0.0 0 0 0)))))

(event EventBeginPlay
  ;[1 1 1] Begin Play
  (if (Variables|TypewriterSettings|GetAutostart%20Typewriter)
    (CallFunction|Play)))

(event Input|KeyboardEvents|AnyKey
  (params (Key :type Key%20Structure))
  ;[1 1 1] Input Handling
  (:Pressed
    (Utilities|IsKey Key (Variables|CameraPawn|GetInput%20To%20Spawn%20PresentationPawn)
      (:then
        (CallFunction|SpawnCamera)))))

(fn ConstructionScript
  (Utilities|FlowControl|Sequence
    (:then_0
      ;[1 1 1] Texts
      (CallFunction|InitText (Variables|Default|GetTitleTextRender) (Variables|Text|GetTitle%20Text) true)
      (CallFunction|InitText (Variables|Default|GetSubtiteTextRender) (Variables|Text|GetSubtitle%20Text) true)
      (CallFunction|InitText (Variables|Default|GetDescriptionTextRender) (Variables|Text|GetDescription%20Text) true)
      (CallFunction|InitText (Variables|Default|GetBackground%20Description) (Variables|Text|GetDescription%20Text) false)
      (CallFunction|InitText (Variables|Default|GetBottomTextRender) (Variables|Text|GetBottom%20Text) true))
    (:then_1
      ;[1 1 1] Base
      (bind _returnvalue (Rendering|Material|CreateDynamicMaterialInstance (Variables|Default|GetSM_Base) 3 0 "None" :!class /Script/Engine.PrimitiveComponent))
      (Rendering|Material|SetVectorParameterValue _returnvalue "Color" (Variables|StyleSettings|GetStandColor) :!class /Script/Engine.MaterialInstanceDynamic)
      (bind _returnvalue_2 (Rendering|Material|CreateDynamicMaterialInstance (Variables|Default|GetSM_Base_FlatWall) 0 0 "None" :!class /Script/Engine.PrimitiveComponent))
      (Rendering|Material|SetVectorParameterValue _returnvalue_2 "Color" (Variables|StyleSettings|GetStandColor) :!class /Script/Engine.MaterialInstanceDynamic))))

(fn InitText
  (params (Text%20Render :type Text%20Render%20Component%20Object%20Reference) (Text%20Settings :type S%20Wrapped%20Text%20Render%20Structure) (Active%20Object :type Boolean))
  ;[1 1 1] Input
  (bind _output_get (LocalVariables|SetLoc%20TextRender Text%20Render))
  (Utilities|IsValid _output_get
    (:Is%20Valid
      (LocalVariables|SetLoc%20Settings Text%20Settings)
      (LocalVariables|SetLoc%20Active Active%20Object)
      (Utilities|FlowControl|Sequence
        (:then_0
          ;[1 1 1] Set Size And Visibility
          (Rendering|Components|TextRender|SetWorldSize (LocalVariables|GetLoc%20TextRender) (.Size (Utilities|Struct|BreakS_WrappedTextRender (LocalVariables|GetLoc%20Settings))))
          (Rendering|SetVisibility (LocalVariables|GetLoc%20TextRender) (.Visible (Utilities|Struct|BreakS_WrappedTextRender (LocalVariables|GetLoc%20Settings))) false)
          ;[1 1 1] Wrap Text
          (if (.Wrap (Utilities|Struct|BreakS_WrappedTextRender (LocalVariables|GetLoc%20Settings)))
            (bind _output_string (CallFunction|StringWrap (.Text (Utilities|Struct|BreakS_WrappedTextRender (LocalVariables|GetLoc%20Settings))) (.Width (Utilities|Struct|BreakS_WrappedTextRender (LocalVariables|GetLoc%20Settings))) "<br>"))
            (Rendering|Components|TextRender|SetText (LocalVariables|GetLoc%20TextRender) (Utilities|Text|ToText(String) _output_string))
            (else
              (Rendering|Components|TextRender|SetText (LocalVariables|GetLoc%20TextRender) (Utilities|Text|ToText(String) (.Text (Utilities|Struct|BreakS_WrappedTextRender (LocalVariables|GetLoc%20Settings))))))))
        (:then_1
          ;[1 1 1] Create Dynamic Material Instance and reset Params
          (bind _returnvalue (Rendering|Material|CreateDynamicMaterialInstance (LocalVariables|GetLoc%20TextRender) 0 (Rendering|Material|GetMaterial (LocalVariables|GetLoc%20TextRender) 0) "None" :!class /Script/Engine.PrimitiveComponent))
          (bind _output_get_2 (LocalVariables|SetLoc%20DMI _returnvalue))
          (Rendering|Material|SetScalarParameterValue _output_get_2 "Emissive Strength" (* (Math|Curves|GetFloatValue (Utilities|Struct|BreakS_WrappedTextTypeWriter (.TypewriterEffect (Utilities|Struct|BreakS_WrappedTextRender (LocalVariables|GetLoc%20Settings)))) 0.0) 1e+02) :!class /Script/Engine.MaterialInstanceDynamic)
          (Rendering|Material|SetVectorParameterValue _output_get_2 "Color" (Math|Conversions|ToLinearColor(Color) (.Color (Utilities|Struct|BreakS_WrappedTextRender (LocalVariables|GetLoc%20Settings)))) :!class /Script/Engine.MaterialInstanceDynamic))
        (:then_2
          ;[1 1 1] Add to Active Objects (second layer of description will be excluded here)
          (if (LocalVariables|GetLoc%20Active)
            (Utilities|Array|Add (Variables|Private|GetTextObjects) (Utilities|Struct|MakeS_WrappedTextGroup (LocalVariables|GetLoc%20TextRender) (LocalVariables|GetLoc%20DMI) (LocalVariables|GetLoc%20Settings)))))
        (:then_3
          (return))))))

(fn UpdateMaterials
  (params (Dynamic%20Material%20Instance :type Material%20Instance%20Dynamic%20Object%20Reference) (Text%20Settings :type S%20Wrapped%20Text%20Render%20Structure%20%28by%20ref%29) (Alpha :type Float%20%28single-precision%29))
  (bind _output_get (LocalVariables|SetLoc%20DMI Dynamic%20Material%20Instance))
  (Utilities|IsValid _output_get
    (:Is%20Valid
      (LocalVariables|SetLoc%20Text%20Settings Text%20Settings)
      (LocalVariables|SetLoc%20Alpha Alpha)
      (Rendering|Material|SetScalarParameterValue (LocalVariables|GetLoc%20DMI) "Emissive Strength" (* (Math|Curves|GetFloatValue (.GlowCurve (Utilities|Struct|BreakS_WrappedTextTypeWriter (.TypewriterEffect (Utilities|Struct|BreakS_WrappedTextRender (LocalVariables|GetLoc%20Text%20Settings))))) (LocalVariables|GetLoc%20Alpha)) 1e+02) :!class /Script/Engine.MaterialInstanceDynamic)
      (Rendering|Material|SetVectorParameterValue (LocalVariables|GetLoc%20DMI) "Color" (Math|Color|Lerp(LinearColor) (Math|Conversions|ToLinearColor(Color) (.Color (Utilities|Struct|BreakS_WrappedTextRender (LocalVariables|GetLoc%20Text%20Settings)))) (Math|Conversions|ToLinearColor(Color) (.TextColor (Utilities|Struct|BreakS_WrappedTextTypeWriter (.TypewriterEffect (Utilities|Struct|BreakS_WrappedTextRender (LocalVariables|GetLoc%20Text%20Settings)))))) (LocalVariables|GetLoc%20Alpha)) :!class /Script/Engine.MaterialInstanceDynamic))))

(fn GetTypewriterActor
  (params (Item :type S%20Wrapped%20Text%20Group%20Structure%20%28by%20ref%29) (TargetArray :type Array%20of%20S%20Wrapped%20Text%20Group%20Structures) (Index :type Integer))
  (bind _typewriter (Utilities|Struct|BreakS_WrappedTextGroup Item))
  ;[1 1 1] Return stored Actor
  (Utilities|IsValid _typewriter
    (:Is%20Valid
      (return true _typewriter false))
    (:Is%20Not%20Valid
      ;[1 1 1] Create Actor if not found
      (bind _returnvalue (AddComponent|AddChildActorComponent false))
      (ChildActorComponent|SetChildActorClass _returnvalue "/Game/Scripts/Blueprints/LSS_LoadingScreenSystem/DemoContent/AdvancedRoomDescription/Blueprints/Data/BP_TypewriterInstance.BP_TypewriterInstance_C")
      (bind _asbp_typewriter_instance (Utilities|Casting|CastToBP_TypewriterInstance (Variables|/Script/Engine.ChildActorComponent|GetChildActor _returnvalue))
        (:then
          (return true _asbp_typewriter_instance true))
        (:CastFailed
          (return false 0 false))))))

(fn ExecuteTypewriterActor
  (params (Array :type Array%20of%20S%20Wrapped%20Text%20Group%20Structures) (Index :type Integer) (Item :type S%20Wrapped%20Text%20Group%20Structure))
  ;[1 1 1] Input
  (LocalVariables|SetLoc%20Array Array)
  (LocalVariables|SetLoc%20Index Index)
  (LocalVariables|SetLoc%20Item Item)
  ;[1 1 1] Continue if Typewriter Effect Enabled
  (if (Utilities|Struct|BreakS_WrappedTextTypeWriter (Utilities|Struct|BreakS_WrappedTextRender (Utilities|Struct|BreakS_WrappedTextGroup (LocalVariables|GetLoc%20Item))))
    ;[1 1 1] Find or Create Typewriter Actor and Execute
    (bind (_success _asbp_tw_helper _created) (CallFunction|GetTypewriterActor (LocalVariables|GetLoc%20Item) (LocalVariables|GetLoc%20Array) (LocalVariables|GetLoc%20Index)))
    (if _success
      (LocalVariables|SetLoc%20Needs%20Save _created)
      (bind _output_get (LocalVariables|SetLoc%20Typewriter _asbp_tw_helper))
      (Utilities|IsValid _output_get
        (:Is%20Valid
          (Default|Execute (LocalVariables|GetLoc%20Typewriter) (.TextRenderComponent (Utilities|Struct|BreakS_WrappedTextGroup (LocalVariables|GetLoc%20Item))) (.TestSettings (Utilities|Struct|BreakS_WrappedTextGroup (LocalVariables|GetLoc%20Item))))
          ;[1 1 1] Store new Typewriter Actor for reusability
          (if (LocalVariables|GetLoc%20Needs%20Save)
            (Utilities|Array|SetArrayElem Array (LocalVariables|GetLoc%20Index) (Utilities|Struct|MakeS_WrappedTextGroup (.TextRenderComponent (Utilities|Struct|BreakS_WrappedTextGroup (LocalVariables|GetLoc%20Item))) (.DynamicMaterialInstance (Utilities|Struct|BreakS_WrappedTextGroup (LocalVariables|GetLoc%20Item))) (.TestSettings (Utilities|Struct|BreakS_WrappedTextGroup (LocalVariables|GetLoc%20Item))) (LocalVariables|GetLoc%20Typewriter)))))))))

(fn SpawnCamera
  (Utilities|IsValid (Variables|Private|GetCameraPawn)
    (:Is%20Valid
      _)
    (:Is%20Not%20Valid
      ;[1 1 1] Find Camera Pawn In Scene if already created
      (bind _outactors (Actor|GetAllActorsOfClass "/Game/Scripts/Blueprints/LSS_LoadingScreenSystem/DemoContent/AdvancedRoomDescription/Blueprints/BP_ShowCaseCamera.BP_ShowCaseCamera_C"))
      (if (> (Utilities|Array|Length _outactors) 0)
        (Variables|Private|SetCameraPawn (Utilities|Array|Get(acopy) _outactors))
        (else
          ;[1 1 1] Spawn Camera Pawn
          (bind _returnvalue (Game|SpawnActorfromClass "/Game/Scripts/Blueprints/LSS_LoadingScreenSystem/DemoContent/AdvancedRoomDescription/Blueprints/BP_ShowCaseCamera.BP_ShowCaseCamera_C" (Math|Transform|MakeTransform (Transformation|GetActorLocation) (Transformation|GetActorRotation)) "Undefined" self (Game|Player|GetPlayerPawn 0) 0))
          (Variables|Private|SetCameraPawn _returnvalue)))
      ;[1 1 1] Possess Camera Pawn
      (Utilities|IsValid (Variables|Private|GetCameraPawn)
        (:Is%20Valid
          _))))
  (Pawn|Possess (Game|GetPlayerController 0) (Variables|Private|GetCameraPawn)))