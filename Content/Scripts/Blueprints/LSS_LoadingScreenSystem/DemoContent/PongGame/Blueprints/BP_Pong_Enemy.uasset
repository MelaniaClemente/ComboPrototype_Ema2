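; AI opponent paddle for the Pong minigame in the Loading Screen System demo content.
; Each tick it loops over all Pong ball actors and steps along X toward each ball, scaled by paddle speed and delta time, with the offset clamped to ease in when close.
; Bound-check helpers take priority over tracking, snapping the paddle back just inside the play area's X limits when it overshoots.
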(event EventTick
  (params (DeltaSeconds :type Float%20%28single-precision%29))
  (bind _outactors (Actor|GetAllActorsOfClass "/Game/Scripts/Blueprints/LSS_LoadingScreenSystem/DemoContent/PongGame/Blueprints/BP_Pong_Ball.BP_Pong_Ball_C"))
  (for _array_element _outactors
    (|X>1500
      (:then
        (|RestrictLocationA))
      (:else
        (|X>-1500
          (:then
            (|RestrictLocationB))
          (:else
            (|SetLocation _array_element)))))))

(fn ConstructionScript)