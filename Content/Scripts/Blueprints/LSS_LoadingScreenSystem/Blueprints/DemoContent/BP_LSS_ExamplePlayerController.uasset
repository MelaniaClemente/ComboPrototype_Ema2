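; Demo player controller for the Loading Screen System (LSS) examples, handling the info HUD, level selection menu and level changes.
; It binds to the LSS actor's loading events to hide the HUD during loading and restore it afterwards.
; Escape or Tab toggles level selection, and Shift+Alt with number or +/- keys fades out before opening demo maps.
; Extra debug keys cover screenshots, resolution, view reset, pawn count and loaded-level printout.
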(event Custom|Transition%20To%20Level%20Input
  (params (LevelName :type Name))
  ;[1 1 1] Transition to level from anywhere
  (if (and (or (Variables|Default|GetLShiftDown) (Variables|Default|GetRShiftDown)) (or (Variables|Default|GetLAltDown) (Variables|Default|GetRAltDown)))
    (CallFunction|TransitiontoLevel LevelName)))

(event Custom|Transition%20To%20Level
  (params (LevelName :type Name))
  ;[1 1 1] Transition to level from anywhere
  (bind (_fade_time _success) (CallFunction|LSSFadeOut false))
  (if _success
    (Utilities|FlowControl|Delay _fade_time))
  (CallFunction|HideLevelSelection)
  (Game|OpenLevel(byName) LevelName))

(event Custom|Hide%20HUD
  (bind _info_ui (Variables|Default|GetInfo%20UI))
  ;[1 1 1] Display info on HUD ("ESC / Tab" to open level selection)
  (Utilities|IsValid _info_ui
    (:Is%20Valid
      (Widget|RemovefromParent _info_ui))))

(event Custom|Hide%20Level%20Selection
  (bind _ui_ref (Variables|Default|GetUI%20Ref))
  ;[1 1 1] Hide Level Selection
  (Utilities|FlowControl|Sequence
    (:then_0
      (Utilities|IsValid _ui_ref
        (:Is%20Valid
          (Widget|RemovefromParent _ui_ref))))
    (:then_1
      (Input|SetInputModeGameOnly self)
      (Variables|Default|SetbShowMouseCursor false)
      (Variables|Default|SetUI%20Visible false)
      (CallFunction|ShowHUD))))

(event Custom|OnLoadingCompleted_Event_0
  ;[1 1 1] Hide HUD during loading
  (CallFunction|ShowHUD))

(event Custom|OnBeginLoading_Event_0
  ;[1 1 1] Hide HUD during loading
  (CallFunction|HideHUD))

(event Custom|Show%20Level%20Selection
  ;[1 1 1] Show Level Selection
  (bind _loading (CallFunction|LSSinProgress))
  (if (not _loading)
    (Utilities|IsValid (Variables|Default|GetUI%20Ref)
      (:Is%20Valid
        _)
      (:Is%20Not%20Valid
        (bind _returnvalue (UserInterface|CreateWidget "/Game/Scripts/Blueprints/LSS_LoadingScreenSystem/UI/ExampleWidgets/UI_Demo_LevelSelection.UI_Demo_LevelSelection_C" self))
        (bind _output_get (Variables|Default|SetUI%20Ref _returnvalue))))
    (UserInterface|Viewport|AddtoViewport _output_get 0)
    (Variables|Default|SetbShowMouseCursor true)
    (Input|SetInputModeGameandUI self (Variables|Default|GetUI%20Ref) "DoNotLock" true)
    (Variables|Default|SetUI%20Visible true)
    (CallFunction|HideHUD)))

(event Custom|Show%20HUD
  ;[1 1 1] Display info on HUD ("ESC / Tab" to open level selection)
  (if (not (Variables|Default|GetUI%20Visible))
    (Utilities|IsValid (Variables|Default|GetInfo%20UI)
      (:Is%20Valid
        _)
      (:Is%20Not%20Valid
        (bind _returnvalue (UserInterface|CreateWidget "/Game/Scripts/Blueprints/LSS_LoadingScreenSystem/UI/ExampleWidgets/UI_Demo_Default.UI_Demo_Default_C"))
        (Variables|Default|SetInfo%20UI _returnvalue)))
    (UserInterface|Viewport|AddtoViewport (Variables|Default|GetInfo%20UI) 0)))

(event EventBeginPlay
  ;[1 1 1] Display info on HUD ("ESC / Tab" to open level selection)
  (Utilities|FlowControl|Delay 0.2)
  (Utilities|FlowControl|Sequence
    (:then_0
      (bind _loading (CallFunction|LSSinProgress))
      (if (not _loading)
        (CallFunction|ShowHUD)))
    (:then_1
      (bind _lss_actor (CallFunction|GetLSSActor))
      (Utilities|IsValid _lss_actor
        (:Is%20Valid
          (EventDispatchers|AssignOnLoadingCompleted _lss_actor (delegate Custom|OnLoadingCompleted_Event_0))
          (EventDispatchers|AssignOnBeginLoading _lss_actor (delegate Custom|OnBeginLoading_Event_0)))))))

(event Input|KeyboardEvents|Add
  (params (Key :type Key%20Structure))
  ;[1 1 1] Debug Input
  (:Pressed
    (CallFunction|TransitiontoLevelInput "07_02_MiniGameLoadingScreen_Map")))

(event Input|KeyboardEvents|1
  (params (Key :type Key%20Structure))
  ;[1 1 1] Debug Input
  (:Pressed
    (CallFunction|TransitiontoLevelInput "01_BasicSetup_Map")))

(event Input|KeyboardEvents|LeftShift
  (params (Key :type Key%20Structure))
  ;[1 1 1] Debug Input
  (:Pressed
    (Variables|Default|SetLShiftDown true))
  (:Released
    (Variables|Default|SetLShiftDown false)))

(event Input|KeyboardEvents|R
  (params (Key :type Key%20Structure))
  ;[1 1 1] Debug Input
  (:Pressed
    (Development|ExecuteConsoleCommand (select (Variables|Default|GetLAltDown) "r.setRes 1920x1080w" "r.setRes 1920x1080f") 0)))

(event Input|KeyboardEvents|0
  (params (Key :type Key%20Structure))
  ;[1 1 1] Debug Input
  (:Pressed
    (CallFunction|TransitiontoLevelInput "10_AlternativeEventOrder_Map")))

(event Input|KeyboardEvents|T
  (params (Key :type Key%20Structure))
  (bind _returnvalue (Game|GetPlayerController 0))
  ;[1 1 1] Debug Input
  (:Pressed
    (Pawn|SetControlRotation _returnvalue (Math|Rotator|MakeRotator 0.0 0.0 (.yaw (Pawn|GetControlRotation _returnvalue :!class /Script/Engine.Controller))))))

(event Input|KeyboardEvents|Subtract
  (params (Key :type Key%20Structure))
  ;[1 1 1] Debug Input
  (:Pressed
    (CallFunction|TransitiontoLevelInput "11_OpenLevel")))

(event Input|KeyboardEvents|Escape
  (params (Key :type Key%20Structure))
  ;[1 1 1] Toggle Level Selection
  (:Pressed
    (if (Widget|IsVisible (Variables|Default|GetUI%20Ref))
      (CallFunction|HideLevelSelection)
      (else
        (CallFunction|ShowLevelSelection)))))

(event Input|KeyboardEvents|Tab
  (params (Key :type Key%20Structure))
  (bind _ui_ref (Variables|Default|GetUI%20Ref))
  ;[1 1 1] Toggle Level Selection
  (:Pressed
    (Utilities|IsValid _ui_ref
      (:Is%20Valid
        (if (Widget|IsVisible _ui_ref)
          (CallFunction|HideLevelSelection)
          (else
            (CallFunction|ShowLevelSelection :!label _label))))
      (:Is%20Not%20Valid
        (goto _label)))))

(event Input|KeyboardEvents|3
  (params (Key :type Key%20Structure))
  ;[1 1 1] Debug Input
  (:Pressed
    (CallFunction|TransitiontoLevelInput "03_SaveReferenceOptimization_Map")))

(event Input|KeyboardEvents|Z
  (params (Key :type Key%20Structure))
  ;[1 1 1] Debug Input
  (:Pressed
    (bind _loaded_levels (CallFunction|LSSGetAllLoadedLevels))
    (for _array_element _loaded_levels
      (Development|PrintString (Utilities|String|ToString(Name) _array_element)))))

(event Input|KeyboardEvents|2
  (params (Key :type Key%20Structure))
  ;[1 1 1] Debug Input
  (:Pressed
    (CallFunction|TransitiontoLevelInput "02_BlueprintSetup_Map")))

(event Input|KeyboardEvents|P
  (params (Key :type Key%20Structure))
  ;[1 1 1] Debug Input
  (:Pressed
    (Development|ExecuteConsoleCommand "bugscreenshot 2" 0)))

(event Input|KeyboardEvents|X
  (params (Key :type Key%20Structure))
  ;[1 1 1] Debug Input
  (:Pressed
    (bind _outactors (Actor|GetAllActorsOfClass "/Script/Engine.Pawn"))
    (Development|PrintString (Utilities|String|ToString(Integer) (Utilities|Array|Length _outactors)))))

(event Input|KeyboardEvents|RightShift
  (params (Key :type Key%20Structure))
  ;[1 1 1] Debug Input
  (:Pressed
    (Variables|Default|SetRShiftDown true))
  (:Released
    (Variables|Default|SetRShiftDown false)))

(event Input|KeyboardEvents|4
  (params (Key :type Key%20Structure))
  ;[1 1 1] Debug Input
  (:Pressed
    (CallFunction|TransitiontoLevelInput "04_MultipleLoadingScreens_Map")))

(event Input|KeyboardEvents|5
  (params (Key :type Key%20Structure))
  ;[1 1 1] Debug Input
  (:Pressed
    (CallFunction|TransitiontoLevelInput "05_LevelPersistence_Map")))

(event Input|KeyboardEvents|LeftAlt
  (params (Key :type Key%20Structure))
  ;[1 1 1] Debug Input
  (:Pressed
    (Variables|Default|SetLAltDown true))
  (:Released
    (Variables|Default|SetLAltDown false)))

(event Input|KeyboardEvents|6
  (params (Key :type Key%20Structure))
  ;[1 1 1] Debug Input
  (:Pressed
    (CallFunction|TransitiontoLevelInput "06_AdvancedEventHandling_Map")))

(event Input|KeyboardEvents|7
  (params (Key :type Key%20Structure))
  ;[1 1 1] Debug Input
  (:Pressed
    (CallFunction|TransitiontoLevelInput "07_MiniGameLoadingScreen_Map")))

(event Input|KeyboardEvents|8
  (params (Key :type Key%20Structure))
  ;[1 1 1] Debug Input
  (:Pressed
    (CallFunction|TransitiontoLevelInput "08_MainMenu_Map")))

(event Input|KeyboardEvents|RightAlt
  (params (Key :type Key%20Structure))
  ;[1 1 1] Debug Input
  (:Pressed
    (Variables|Default|SetRAltDown true))
  (:Released
    (Variables|Default|SetRAltDown false)))

(event Input|KeyboardEvents|9
  (params (Key :type Key%20Structure))
  ;[1 1 1] Debug Input
  (:Pressed
    (CallFunction|TransitiontoLevelInput "09_UserInterface_Map")))

(fn ConstructionScript)