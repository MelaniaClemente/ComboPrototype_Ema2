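; Base projectile actor that damages characters on static mesh overlap, ignoring its shooter and destroying itself on teammates (unless team checks are off) or non-characters.
; Blocking characters hit from the front arcs take block-reduced damage; other hits deal normal damage, each spawning its effect before delayed destruction.
; Construction adds a sphere, box or capsule collider when no mesh is set.
; The impulse launch function is disconnected and does nothing.
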(event OnComponentBeginOverlap(StaticMesh)
  (params (OverlappedComponent :type Primitive%20Component%20Object%20Reference) (OtherActor :type Actor%20Object%20Reference) (OtherComp :type Primitive%20Component%20Object%20Reference) (OtherBodyIndex :type Integer) (bFromSweep :type Boolean) (SweepResult :type Hit%20Result%20Structure%20%28by%20ref%29))
  (bind _onhitgameplayactions (Variables|Default|GetOnHitGameplayActions))
  (if (!= OtherActor (Variables|Default|GetOwnerShooter))
    (bind _asbp_character_master (Utilities|Casting|CastToBP_CharacterMaster OtherActor)
      (:then
        (Variables|Default|SetHittedCharacter _asbp_character_master)
        (if (Variables|Default|GetIgnoreTeamID)
          (if (Variables|/Game/Scripts/Blueprints/Characters/BP_CharacterMaster.BP_CharacterMaster_C|GetIsBlocking (Variables|Default|GetHittedCharacter)) :!label _label
            (bind _direction (Default|GetRelativeDirectionbyActor (Variables|Default|GetHittedCharacter) self (Variables|Default|GetHittedCharacter)))
            (switch Utilities|FlowControl|Switch|SwitchonENUM_Directions _direction
              (:NewEnumerator0
                (Utilities|IsValid (Variables|Default|GetHittedCharacter) :!label _label_2
                  (:Is%20Valid
                    (CallFunction|SingleTargetAttack (Variables|Default|GetHittedCharacter) _onhitgameplayactions (Variables|Default|GetOwnerAttackTypeMultiplier) (Variables|Default|GetOwnerWeaponTypeMultiplier) (Default|GetBlockDamageReduction (Variables|Default|GetHittedCharacter)) (Variables|Default|GetOwnerBaseDamage) true)
                    (Game|SpawnActorfromClass (Variables|Effects|GetBlockedGameplayEffect) (Math|Transform|MakeTransform (Transformation|GetActorLocation (Variables|Default|GetHittedCharacter)) (Math|Random|RandomRotator false) "1,1,1") "AlwaysSpawn" 0 0))))
              (:NewEnumerator1
                (goto _label_2))
              (:NewEnumerator2
                (goto _label_2))
              (:NewEnumerator3
                (Utilities|IsValid (Variables|Default|GetHittedCharacter) :!label _label_3
                  (:Is%20Valid
                    (CallFunction|SingleTargetAttack (Variables|Default|GetHittedCharacter) _onhitgameplayactions (Variables|Default|GetOwnerAttackTypeMultiplier) (Variables|Default|GetOwnerWeaponTypeMultiplier) 1.0 (Variables|Default|GetOwnerBaseDamage) false)
                    (Game|SpawnActorfromClass (Variables|Effects|GetHitCharacterGameplayEffect) (Math|Transform|MakeTransform (Transformation|GetActorLocation (Variables|Default|GetHittedCharacter)) (Math|Random|RandomRotator false) "1,1,1") "AlwaysSpawn" 0 0))))
              (:NewEnumerator4
                (goto _label_3))
              (:NewEnumerator5
                (goto _label_3))
              (:NewEnumerator6
                (goto _label_3))
              (:NewEnumerator7
                (goto _label_3)))
            (else
              (goto _label_3)))
          (Utilities|FlowControl|Delay 1.0)
          (Actor|DestroyActor)
          (else
            (bind _id (Default|GetTeamID (Variables|Default|GetHittedCharacter)))
            (if (!= _id (Variables|Default|GetTeamID))
              (goto _label)
              (else
                (Actor|DestroyActor :!label _label_4))))))
      (:CastFailed
        (goto _label_4)))))

(event EventBeginPlay)

(event Collision|EventActorBeginOverlap
  (params (OtherActor :type Actor%20Object%20Reference)))

(event EventTick
  (params (DeltaSeconds :type Float%20%28single-precision%29)))

(fn ConstructionScript
  (Utilities|IsValid (Variables|/Script/Engine.StaticMeshComponent|GetStaticMesh (Variables|Default|GetStaticMesh))
    (:Is%20Valid
      (Variables|Collision|SetUseMeshCollision true))
    (:Is%20Not%20Valid
      (Variables|Collision|SetUseMeshCollision false)
      (switch Utilities|FlowControl|Switch|SwitchonENUM_ColliderType (Variables|Collision|GetPrimitiveColliderType)
        (:NewEnumerator0
          (bind _returnvalue (AddComponent|AddSphereComponent false))
          (bind _output_get (Variables|Default|SetSphereCollider _returnvalue))
          (Transformation|AttachComponentToComponent _output_get (Variables|Default|GetStaticMesh) "None" "KeepRelative" "KeepRelative" "KeepRelative" true)
          (Components|Sphere|SetSphereRadius (Variables|Default|GetSphereCollider) (Variables|Collision|GetSphereCollider_radius) true))
        (:NewEnumerator1
          (bind _returnvalue_2 (AddComponent|AddBoxComponent false))
          (bind _output_get_2 (Variables|Default|SetBoxCollider _returnvalue_2))
          (Transformation|AttachComponentToComponent _output_get_2 (Variables|Default|GetStaticMesh) "None" "KeepRelative" "KeepRelative" "KeepRelative" true)
          (Components|Box|SetBoxExtent (Variables|Default|GetBoxCollider) (Variables|Collision|GetBoxCollider_Dimension) true))
        (:NewEnumerator2
          (bind _returnvalue_3 (AddComponent|AddCapsuleComponent false))
          (bind _output_get_3 (Variables|Default|SetCapsuleCollider _returnvalue_3))
          (Transformation|AttachComponentToComponent _output_get_3 (Variables|Default|GetStaticMesh) "None" "KeepRelative" "KeepRelative" "KeepRelative" true)
          (Components|Capsule|SetCapsuleRadius (Variables|Default|GetCapsuleCollider) (Variables|Collision|GetSphereCollider_radius) true)
          (Components|Capsule|SetCapsuleHalfHeight (Variables|Default|GetCapsuleCollider) (Variables|Collision|GetCapsuleCollider_HalfHeight) true))))))

(fn SpawnGameplayEffect
  (bind _returnvalue (Game|SpawnActorfromClass (Variables|Effects|GetSpawnGameplayEffectClass) (Transformation|GetActorTransform) "AlwaysSpawn" self 0))
  (Variables|Effects|SetEffectActor _returnvalue))

(fn ActivateProjectileImpulse
  (params (Direction :type Vector) (ImpulseStrenght :type Float%20%28single-precision%29) (bVelChange :type Boolean)))

(fn EnableMeshOverlap
  (Collision|SetCollisionResponsetoAllChannels (Variables|Default|GetStaticMesh) "ECR_Overlap"))