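; Checkpoint actor in the saving system that supplies a respawn transform for a character and can blow itself apart.
; GetRespawnLocationAndRotation traces down from the RespawnLocation component and, on a hit, lifts the point by the character's capsule half-height, keeping only the component's relative yaw.
; The Autodestruction event enables physics on the DestructibleComponent, shatters it with radius damage, then destroys the actor after a short delay.
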(event Custom|Autodestruction
  (Physics|SetSimulatePhysics (Variables|Default|GetDestructibleComponent) true)
  (Class|DestructibleComponent|ApplyRadiusDamage (Variables|Default|GetDestructibleComponent) 1e+05 (Transformation|GetActorLocation) 1e+03 2.5e+03 true)
  (Utilities|FlowControl|Delay 3.0)
  (Actor|DestroyActor))

(event EventBeginPlay)

(event Collision|EventActorBeginOverlap
  (params (OtherActor :type Actor%20Object%20Reference)))

(event EventTick
  (params (DeltaSeconds :type Float%20%28single-precision%29)))

(event Game|Damage|EventAnyDamage
  (params (Damage :type Float%20%28single-precision%29) (DamageType :type Damage%20Type%20Object%20Reference) (InstigatedBy :type Controller%20Object%20Reference) (DamageCauser :type Actor%20Object%20Reference)))

(fn ConstructionScript)

(fn GetRespawnLocationandRotation
  (params (Character :type Character%20Object%20Reference))
  (bind _respawnlocation (Variables|Default|GetRespawnLocation))
  (bind _respawnlocation_2 (Variables|Default|GetRespawnLocation))
  (bind _returnvalue (Transformation|GetWorldLocation _respawnlocation))
  (bind _returnvalue_2 (Transformation|GetWorldLocation _respawnlocation_2))
  (LocalVariables|SetRespawnRot (Math|Rotator|MakeRotator 0.0 0.0 (.yaw (Variables|/Script/Engine.SceneComponent|GetRelativeRotation _respawnlocation_2))))
  (LocalVariables|SetRespawnLoc _returnvalue_2)
  (bind (_outhit _returnvalue_3) (Collision|LineTraceByChannel _returnvalue_2 (- (Transformation|GetWorldLocation (Variables|Default|GetRespawnLocation)) "0, 0,5000.000000") "TraceTypeQuery1" false 0 "None"))
  (if _returnvalue_3
    (LocalVariables|SetRespawnLoc (Math|Vector|MakeVector (.x _returnvalue) (.y _returnvalue) (+ (.Z (Math|Vector|BreakVector (.Location (Collision|BreakHitResult _outhit)))) (Components|Capsule|GetScaledCapsuleHalfHeight (Variables|/Script/Engine.Character|GetCapsuleComponent Character))))))
  (return (LocalVariables|GetRespawnLoc) (LocalVariables|GetRespawnRot)))