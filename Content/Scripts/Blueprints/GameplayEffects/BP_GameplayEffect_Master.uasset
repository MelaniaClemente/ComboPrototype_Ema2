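; Master one-shot gameplay effect actor bundling Cascade and Niagara particles, sound, hit stop, camera shake and gamepad vibration.
; Construction applies the GameplayEffect struct to the components and hit-stop curve; its data table lookup is disconnected.
; BeginPlay fires shake and vibration, while Tick triggers a timeline that lerps global time dilation for hit stop.
; Completion flags, preset for unused parts, let Tick destroy the actor once particles, audio and hit stop finish.
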(event OnSystemFinished(ParticleSystem)
  (params (PSystem :type Particle%20System%20Component%20Object%20Reference))
  (Variables|Default|SetPS_Ended true))

(event OnAudioFinished(Audio)
  (Variables|Default|SetAudio_Ended true))

(event OnSystemFinished(NiagaraParticleSystem)
  (params (PSystem :type Niagara%20Component%20Object%20Reference))
  (Variables|Default|SetNiagara_Ended true))

(event Custom|Hit&StopEffect
  (if (and (not (Variables|Default|GetHit&Stop_Ended)) (>= (Class|GameplayStatics|GetGlobalTimeDilation) 1.0))
    (bind _hit_stoptrack (Timeline|Hit&Stop PlayFromStart)
      (:Update
        (Utilities|Time|SetGlobalTimeDilation (Math|Float|Lerp 1.0 (CallFunction|GetMaxTimeDilation) _hit_stoptrack)))
      (:Finished
        (Variables|Default|SetHit&Stop_Ended true)))
    (else
      (Variables|Default|SetHit&Stop_Ended true))))

(event EventBeginPlay
  (bind (_return _gameplay_effect_vibration_intensity _gameplay_effect_vibration_duration) (CallFunction|GetVibrationEnabled))
  (bind _returnvalue (Game|GetPlayerController 0))
  (bind (_return_2 _gameplay_effect_camera_shake_class) (CallFunction|GetCameraShakeEnabled))
  (Utilities|FlowControl|Sequence
    (:then_0
      (Utilities|IsValid (Variables|/Script/Engine.ParticleSystemComponent|GetTemplate (Variables|Default|GetParticleSystem))
        (:Is%20Not%20Valid
          (Variables|Default|SetPS_Ended true))))
    (:then_1
      (Utilities|IsValid (Variables|/Script/Engine.AudioComponent|GetSound (Variables|Default|GetAudio))
        (:Is%20Not%20Valid
          (Variables|Default|SetAudio_Ended true))))
    (:then_2
      (if (not (CallFunction|GetHitandStopEnabled))
        (Variables|Default|SetHit&Stop_Ended true)))
    (:then_3
      (if _return_2
        (Camera|PlayWorldCameraShake _gameplay_effect_camera_shake_class (Transformation|GetActorLocation) 1e+03 1e+05)))
    (:then_4
      (if (and _return (Utilities|DoesObjectImplementInterface _returnvalue "/Game/Scripts/Blueprints/Interfaces/BP_CharacterInterface.BP_CharacterInterface_C"))
        (bind _myplayercontroller (Class|BPCharacterInterface|GetMyPlayerController(Message) _returnvalue))
        (Game|Feedback|PlayDynamicForceFeedback _myplayercontroller _gameplay_effect_vibration_intensity _gameplay_effect_vibration_duration true true true true)))
    (:then_5
      (Utilities|IsValid (AssetData|GetAsset (Variables|Default|GetNiagaraParticleSystem))
        (:Is%20Not%20Valid
          (Variables|Default|SetNiagara_Ended true))))))

(event EventTick
  (params (DeltaSeconds :type Float%20%28single-precision%29))
  (Utilities|FlowControl|Sequence
    (:then_0
      (if (and (== (Class|GameplayStatics|GetGlobalTimeDilation) 1.0) (CallFunction|GetHitandStopEnabled))
        (Utilities|FlowControl|DoOnce false
          (:Completed
            (CallFunction|Hit&StopEffect)))))
    (:then_1
      (if (Math|Boolean|ANDBoolean (Variables|Default|GetPS_Ended) (Variables|Default|GetAudio_Ended) (Variables|Default|GetHit&Stop_Ended) (Variables|Default|GetNiagara_Ended))
        (Actor|DestroyActor)))))

(fn ConstructionScript
  (bind _gameplayeffect (Variables|Effects|GetGameplayEffect))
  (bind _audio (Variables|Default|GetAudio))
  (Effects|Components|ParticleSystem|SetTemplate (Variables|Default|GetParticleSystem) (.particlesystem _gameplayeffect))
  (Audio|Components|Audio|SetSound _audio (.sound _gameplayeffect))
  (Audio|Components|Audio|SetVolumeMultiplier _audio (.volumemultiplier _gameplayeffect) :!class /Script/Engine.AudioComponent)
  (Audio|Components|Audio|SetPitchMultiplier _audio (.pitchmultiplier _gameplayeffect))
  (Class|TimelineComponent|SetFloatCurve (Variables|Default|GetHit&Stop) (.hitstopcurve _gameplayeffect) "Hit&StopTrack")
  (Class|NiagaraComponent|SetAsset (Variables|Default|GetNiagaraParticleSystem) (.niagaraparticlesystem (Variables|Effects|GetGameplayEffect))))

(fn GetTimeDilationMultiplier
  (return (.hitstopmultiplier (Variables|Effects|GetGameplayEffect))))

(fn GetHitandStopEnabled
  (return (.hitstop (Variables|Effects|GetGameplayEffect))))

(fn GetMaxTimeDilation
  (return (.maxtimedilationvalue (Variables|Effects|GetGameplayEffect))))

(fn GetCameraShakeEnabled
  (bind _gameplayeffect (Variables|Effects|GetGameplayEffect))
  (return (.camerashake _gameplayeffect) (.camerashakeclass _gameplayeffect)))

(fn GetVibrationEnabled
  (bind _gameplayeffect (Variables|Effects|GetGameplayEffect))
  (return (.gamepadvibration _gameplayeffect) (.vibrationintensity _gameplayeffect) (.vibrationduration _gameplayeffect)))