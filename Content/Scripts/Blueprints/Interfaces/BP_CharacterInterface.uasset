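; Blueprint interface for characters, exposing typed references, team identity and aggro without requiring callers to cast.
; Getter functions return the player character, character master, master anim instance, player controller and enemy character.
; GetTeamID returns an enum team value, while IncrementAggro, DecrementAggro and GetTargetAggro define a per-actor threat contract.
; The functions hold no logic here, leaving behavior to implementing classes.
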(fn GetMyPlayerCharacter
  (return 0))

(fn GetMyCharacterMaster
  (return 0))

(fn GetMyMasterAnimInstance
  (return 0))

(fn GetMyPlayerController
  (return 0))

(fn GetMyEnemyCharacter
  (return 0))

(fn GetTeamID
  (return "NewEnumerator0"))

(fn IncrementAggro
  (params (Increment :type Integer) (Actor :type Actor%20Object%20Reference)))

(fn DecrementAggro
  (params (Decrement :type Integer) (Actor :type Actor%20Object%20Reference)))

(fn GetTargetAggro
  (return 0))