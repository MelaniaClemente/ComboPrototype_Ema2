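; Interactable double door that swings open once, with audio, when OpenInteraction fires.
; It flips the swing angle if the player's relative direction is on a left side, then a timeline rotates both leaves in opposite yaw.
; On finish, it tints the emissive color of dynamic materials created at BeginPlay and broadcasts the final rotations, color and interaction type through OnDoorOpening.
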(event EventBeginPlay
  (bind _rightdoor (Variables|Default|GetRightDoor))
  (bind _leftdoor (Variables|Default|GetLeftDoor))
  (|CallParentFunction)
  (bind _returnvalue (Rendering|Material|CreateDynamicMaterialInstance _rightdoor 0 (Rendering|Material|GetMaterial _rightdoor 0) "None" :!class /Script/Engine.PrimitiveComponent))
  (bind _output_get (Variables|Default|SetLeftDoorMat _returnvalue))
  (Rendering|Material|SetMaterial _rightdoor 0 _output_get)
  (bind _returnvalue_2 (Rendering|Material|CreateDynamicMaterialInstance _leftdoor 0 (Rendering|Material|GetMaterial _leftdoor 0) "None" :!class /Script/Engine.PrimitiveComponent))
  (bind _output_get_2 (Variables|Default|SetRightDoorMat _returnvalue_2))
  (Rendering|Material|SetMaterial _leftdoor 0 _output_get_2))

(event Collision|EventActorBeginOverlap
  (params (OtherActor :type Actor%20Object%20Reference))
  (|CallParentFunction OtherActor) ; This node is disabled and will not be called.\nDrag off pins to build functionality.
)

(event EventTick
  (params (DeltaSeconds :type Float%20%28single-precision%29))
  (|CallParentFunction DeltaSeconds))

(event EventOpenInteraction
  (bind _doorcolor (Variables|Default|GetDoorColor))
  (Utilities|FlowControl|DoOnce false
    (:Completed
      (Variables|Default|SetInteractionType "NewEnumerator2")
      (Audio|Components|Audio|Play (Variables|Default|GetAudio) 0.0)
      (CallFunction|UpdateRotationAnglebyCharacterDirection)
      (bind _newtrack_0 (Timeline|OpenDoorTimeline PlayFromStart)
        (:Update
          (Transformation|SetRelativeRotation (Variables|Default|GetLeftDoor) (Math|Rotator|MakeRotator 0.0 0.0 (Math|Float|Lerp 0.0 (* (Variables|Default|GetLastRotationAngle) -1.0) _newtrack_0)) false false)
          (Transformation|SetRelativeRotation (Variables|Default|GetRightDoor) (Math|Rotator|MakeRotator 0.0 0.0 (Math|Float|Lerp 0.0 (Variables|Default|GetLastRotationAngle) _newtrack_0)) false false))
        (:Finished
          (Rendering|Material|SetVectorParameterValue (Variables|Default|GetLeftDoorMat) "EmissiveColor" _doorcolor :!class /Script/Engine.MaterialInstanceDynamic)
          (Rendering|Material|SetVectorParameterValue (Variables|Default|GetRightDoorMat) "EmissiveColor" _doorcolor :!class /Script/Engine.MaterialInstanceDynamic)
          (Default|CallOnDoorOpening (Variables|/Script/Engine.SceneComponent|GetRelativeRotation (Variables|Default|GetLeftDoor)) (Variables|/Script/Engine.SceneComponent|GetRelativeRotation (Variables|Default|GetRightDoor)) (Variables|Default|GetDoorColor) (Variables|Default|GetInteractionType)))))))

(event EventOnSnapDataLoaded)

(fn ConstructionScript
  (|CallParentFunction))

(fn InvertLastRotationAngle
  (Variables|Default|SetLastRotationAngle (* (Variables|Default|GetLastRotationAngle) -1.0)))

(fn UpdateRotationAnglebyCharacterDirection
  (bind _asbp_player_character (Utilities|Casting|CastToBP_PlayerCharacter (Game|GetPlayerCharacter 0)))
  (bind _direction (Default|GetRelativeDirectionbyActor _asbp_player_character _asbp_player_character self))
  (switch Utilities|FlowControl|Switch|SwitchonENUM_Directions _direction
    (:NewEnumerator1
      _)
    (:NewEnumerator3
      _)
    (:NewEnumerator5
      _))
  (CallFunction|InvertLastRotationAngle))