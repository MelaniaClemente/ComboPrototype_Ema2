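; Double door actor for level design that swings both leaves open, one time only, when its OpenInteraction event fires.
; A DoOnce gate switches InteractionType to another enum state and plays OpenDoorTimeline.
; The timeline track lerps the relative yaw of LeftDoor and RightDoor from zero to LastRotationAngle in opposite directions.
; The event graph has no close or reset path.
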(event EventBeginPlay
  (|CallParentFunction) ; This node is disabled and will not be called.\nDrag off pins to build functionality.
)

(event Collision|EventActorBeginOverlap
  (params (OtherActor :type Actor%20Object%20Reference))
  (|CallParentFunction OtherActor) ; This node is disabled and will not be called.\nDrag off pins to build functionality.
)

(event EventTick
  (params (DeltaSeconds :type Float%20%28single-precision%29))
  (|CallParentFunction DeltaSeconds) ; This node is disabled and will not be called.\nDrag off pins to build functionality.
)

(event EventOpenInteraction
  (Utilities|FlowControl|DoOnce false
    (:Completed
      (Variables|Default|SetInteractionType "NewEnumerator2")
      (bind _newtrack_0 (Timeline|OpenDoorTimeline Play)
        (:Update
          (Transformation|SetRelativeRotation (Variables|Default|GetLeftDoor) (Math|Rotator|MakeRotator 0.0 0.0 (Math|Float|Lerp 0.0 (* (Variables|Default|GetLastRotationAngle) -1.0) _newtrack_0)) false false)
          (Transformation|SetRelativeRotation (Variables|Default|GetRightDoor) (Math|Rotator|MakeRotator 0.0 0.0 (Math|Float|Lerp 0.0 (Variables|Default|GetLastRotationAngle) _newtrack_0)) false false))))))

(fn ConstructionScript
  (|CallParentFunction))