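; BP_TreasureChest is an interactable treasure chest that opens once and spawns a pickup.
; OnInteractions changes the interaction type, plays audio, deactivates the particle system and runs a timeline that lerps the cover's roll toward LastRotationAngle.
; The timeline's first update spawns BP_PickUpable at PickUpableSpawnLocation.
; The construction script offsets the base along Y by the negated trigger box dimension.
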(event EventBeginPlay
  (|CallParentFunction))

(event Collision|EventActorBeginOverlap
  (params (OtherActor :type Actor%20Object%20Reference))
  (|CallParentFunction OtherActor) ; This node is disabled and will not be called.\nDrag off pins to build functionality.
)

(event EventTick
  (params (DeltaSeconds :type Float%20%28single-precision%29))
  (|CallParentFunction DeltaSeconds) ; This node is disabled and will not be called.\nDrag off pins to build functionality.
)

(event EventOnInteractions
  (bind _cover (Variables|Default|GetCover))
  (bind _relativerotation (Variables|/Script/Engine.SceneComponent|GetRelativeRotation _cover))
  (Utilities|FlowControl|DoOnce false
    (:Completed
      (Variables|Default|SetInteractionType "NewEnumerator2")
      (Audio|Components|Audio|Play (Variables|Default|GetAudio) 0.0)
      (Components|Activation|SetActive (Variables|Default|GetParticleSystem) false false)
      (bind _newtrack_0 (Timeline|OpenChestMovement Play)
        (:Update
          (Transformation|SetRelativeRotation _cover (Math|Rotator|MakeRotator (Math|Float|Lerp (.roll _relativerotation) (Variables|Default|GetLastRotationAngle) _newtrack_0) (.pitch _relativerotation) (.yaw _relativerotation)) false false)
          (Utilities|FlowControl|DoOnce false
            (:Completed
              (Game|SpawnActorfromClass "/Game/Scripts/Blueprints/LevelDesignHelper/Interaction/BP_PickUpable.BP_PickUpable_C" (Transformation|GetWorldTransform (Variables|Default|GetPickUpableSpawnLocation)) "AlwaysSpawn" 0 0))))))))

(fn ConstructionScript
  (|CallParentFunction)
  (Transformation|SetRelativeLocation (Variables|Default|GetBasament) (Math|Vector|MakeVector 0.0 (* (.y (Variables|Default|GetTriggerBoxDimension)) -1.0) 0.0) false false))