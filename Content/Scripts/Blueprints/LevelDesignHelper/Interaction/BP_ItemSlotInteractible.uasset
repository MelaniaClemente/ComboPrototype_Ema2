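; BP_ItemSlotInteractible is a level-design interactible that lets the player open an item slot UI for combinations.
; ItemInteraction has BP_PlayerConroller create the slot widget for this actor when its ItemInteractionWidget is not valid.
; BeginPlay binds inherited delegates: end overlap removes the player's widget, and combination match calls CombinationMatched.
; CombinationMatched only prints the matched index or an invalid-combination message, with -1 meaning invalid.
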(event Custom|RemoveWidget
  (params (OtherActor :type Actor%20Object%20Reference))
  (bind _asbp_player_character (Utilities|Casting|CastToBP_PlayerCharacter OtherActor))
  (bind _asbp_player_conroller (Utilities|Casting|CastToBP_PlayerConroller (Pawn|GetController _asbp_player_character)))
  (Default|RemoveItemSlotWidget _asbp_player_conroller))

(event Custom|CombinationMatched
  (params (CombinationIndex :type Integer))
  (switch int CombinationIndex
    (:Default
      (Development|PrintString (Utilities|String|Append "MatchedCombination: " (Utilities|String|ToString(Integer) CombinationIndex))))
    (:-1
      (Development|PrintString "Unvalid Combination"))))

(event EventBeginPlay
  (|CallParentFunction)
  (EventDispatchers|BindEventtoMyEndEndOverlap (delegate Custom|RemoveWidget))
  (EventDispatchers|BindEventtoOnCombinationMatch (delegate Custom|CombinationMatched)))

(event Collision|EventActorBeginOverlap
  (params (OtherActor :type Actor%20Object%20Reference))
  (|CallParentFunction OtherActor) ; This node is disabled and will not be called.\nDrag off pins to build functionality.
)

(event EventTick
  (params (DeltaSeconds :type Float%20%28single-precision%29))
  (|CallParentFunction DeltaSeconds) ; This node is disabled and will not be called.\nDrag off pins to build functionality.
)

(event EventItemInteraction
  (Development|PrintString "TuMadre")
  (bind _asbp_player_conroller (Utilities|Casting|CastToBP_PlayerConroller (Game|GetPlayerController 0)))
  (Utilities|IsValid (Variables|/Game/Scripts/Blueprints/Controllers/Player/BP_PlayerConroller.BP_PlayerConroller_C|GetItemInteractionWidget _asbp_player_conroller)
    (:Is%20Not%20Valid
      (Default|InitializeItemSlotWidget _asbp_player_conroller self))))

(fn ConstructionScript
  (|CallParentFunction))