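; Base interactable actor that registers itself with the player's interaction controller on trigger overlap and exposes Pick Up, Open and Pray interactions.
; The construction script configures a sphere, box or capsule trigger, adding it if missing.
; Overlaps reach the controller through BP_PlayerInteractionsInterface, setting the current actor and type; exiting clears the actor without checking it is self.
; OnInteractions dispatches by InteractionType to empty events.
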(event OnComponentBeginOverlap(SphereTrigger)
  (params (OverlappedComponent :type Primitive%20Component%20Object%20Reference) (OtherActor :type Actor%20Object%20Reference) (OtherComp :type Primitive%20Component%20Object%20Reference) (OtherBodyIndex :type Integer) (bFromSweep :type Boolean) (SweepResult :type Hit%20Result%20Structure%20%28by%20ref%29))
  ;[0 0 0] Interaction Events
  (CallFunction|ProcessonOverlap OtherActor))

(event OnComponentEndOverlap(SphereTrigger)
  (params (OverlappedComponent :type Primitive%20Component%20Object%20Reference) (OtherActor :type Actor%20Object%20Reference) (OtherComp :type Primitive%20Component%20Object%20Reference) (OtherBodyIndex :type Integer))
  ;[0 0 0] Interaction Events
  (CallFunction|ProcessEndOverlap OtherActor))

(event OnComponentBeginOverlap(CapsuleTrigger)
  (params (OverlappedComponent :type Primitive%20Component%20Object%20Reference) (OtherActor :type Actor%20Object%20Reference) (OtherComp :type Primitive%20Component%20Object%20Reference) (OtherBodyIndex :type Integer) (bFromSweep :type Boolean) (SweepResult :type Hit%20Result%20Structure%20%28by%20ref%29))
  ;[0 0 0] Interaction Events
  (CallFunction|ProcessonOverlap OtherActor))

(event OnComponentEndOverlap(CapsuleTrigger)
  (params (OverlappedComponent :type Primitive%20Component%20Object%20Reference) (OtherActor :type Actor%20Object%20Reference) (OtherComp :type Primitive%20Component%20Object%20Reference) (OtherBodyIndex :type Integer))
  ;[0 0 0] Interaction Events
  (CallFunction|ProcessEndOverlap OtherActor))

(event OnComponentBeginOverlap(BoxTrigger)
  (params (OverlappedComponent :type Primitive%20Component%20Object%20Reference) (OtherActor :type Actor%20Object%20Reference) (OtherComp :type Primitive%20Component%20Object%20Reference) (OtherBodyIndex :type Integer) (bFromSweep :type Boolean) (SweepResult :type Hit%20Result%20Structure%20%28by%20ref%29))
  ;[0 0 0] Interaction Events
  (CallFunction|ProcessonOverlap OtherActor))

(event OnComponentEndOverlap(BoxTrigger)
  (params (OverlappedComponent :type Primitive%20Component%20Object%20Reference) (OtherActor :type Actor%20Object%20Reference) (OtherComp :type Primitive%20Component%20Object%20Reference) (OtherBodyIndex :type Integer))
  ;[0 0 0] Interaction Events
  (CallFunction|ProcessEndOverlap OtherActor))

(event Custom|ProcessOnOverlap
  (params (Other%20Actor :type Actor%20Object%20Reference))
  ;[0 0 0] Interaction Events
  (if (Utilities|Enum|NotEqual(Enum) (Variables|Interaction|GetInteractionType) "NewEnumerator2")
    (if (and (Utilities|DoesObjectImplementInterface Other%20Actor "/Game/Scripts/Blueprints/Interfaces/BP_PlayerInteractionsInterface.BP_PlayerInteractionsInterface_C") (Utilities|IsValid Other%20Actor))
      (bind _controller (Class|BPPlayerInteractionsInterface|GetInteractionController(Message) Other%20Actor))
      (Utilities|IsValid _controller
        (:Is%20Valid
          (if (or (!= (Variables|/Game/Scripts/Blueprints/Controllers/Player/BP_PlayerConroller.BP_PlayerConroller_C|GetCurrentInteractiveActor _controller) self) (not (Utilities|IsValid (Variables|/Game/Scripts/Blueprints/Controllers/Player/BP_PlayerConroller.BP_PlayerConroller_C|GetCurrentInteractiveActor _controller))))
            (Variables|/Game/Scripts/Blueprints/Controllers/Player/BP_PlayerConroller.BP_PlayerConroller_C|SetCurrentInteractiveActor _controller self)
            (Variables|/Game/Scripts/Blueprints/Controllers/Player/BP_PlayerConroller.BP_PlayerConroller_C|SetCurrentInteractionType _controller (Variables|Interaction|GetInteractionType))))))))

(event Custom|ProcessEndOverlap
  (params (Other%20Actor :type Actor%20Object%20Reference))
  ;[0 0 0] Interaction Events
  (if (Utilities|Enum|NotEqual(Enum) (Variables|Interaction|GetInteractionType) "NewEnumerator2")
    (if (Utilities|DoesObjectImplementInterface Other%20Actor "/Game/Scripts/Blueprints/Interfaces/BP_PlayerInteractionsInterface.BP_PlayerInteractionsInterface_C")
      (bind _controller (Class|BPPlayerInteractionsInterface|GetInteractionController(Message) Other%20Actor))
      (Utilities|IsValid _controller
        (:Is%20Valid
          (Variables|/Game/Scripts/Blueprints/Controllers/Player/BP_PlayerConroller.BP_PlayerConroller_C|SetCurrentInteractiveActor _controller 0)
          (Variables|/Game/Scripts/Blueprints/Controllers/Player/BP_PlayerConroller.BP_PlayerConroller_C|SetCurrentInteractionType _controller (Variables|Interaction|GetInteractionType)))))))

(event EventBeginPlay)

(event Collision|EventActorBeginOverlap
  (params (OtherActor :type Actor%20Object%20Reference)))

(event EventTick
  (params (DeltaSeconds :type Float%20%28single-precision%29)))

(event EventOnInteractions
  (switch Utilities|FlowControl|Switch|SwitchonENUM_InteractionType (Variables|Interaction|GetInteractionType)
    (:NewEnumerator0
      (CallFunction|PickUpInteraction))
    (:NewEnumerator1
      (CallFunction|OpenInteraction))
    (:NewEnumerator3
      (CallFunction|PrayInteraction))))

(event EventOpenInteraction)

(event EventPickUpInteraction)

(event EventPrayInteraction)

(event EventOnSnapDataLoaded)

(fn ConstructionScript
  (switch Utilities|FlowControl|Switch|SwitchonENUM_ColliderType (Variables|Trigger|GetColliderType)
    (:NewEnumerator0
      (Utilities|IsValid (Variables|Default|GetSphereTrigger)
        (:Is%20Valid
          _)
        (:Is%20Not%20Valid
          (bind _returnvalue (AddComponent|AddSphereComponent false))
          (bind _output_get (Variables|Default|SetSphereTrigger _returnvalue))
          (Utilities|IsValid _output_get
            (:Is%20Valid
              _))))
      (Components|Sphere|SetSphereRadius _output_get (Variables|Trigger|GetTriggerRadius) true)
      (Collision|SetCollisionResponsetoAllChannels (Variables|Default|GetSphereTrigger) "ECR_Overlap")
      (Collision|SetCollisionResponsetoChannel (Variables|Default|GetSphereTrigger) "ECC_PhysicsBody" "ECR_Ignore")
      (Development|SetHiddeninGame (Variables|Default|GetSphereTrigger) (Variables|Trigger|GetTriggerHiddenIngame) false)
      (Transformation|SetRelativeLocation (Variables|Default|GetSphereTrigger) (Variables|Trigger|GetTriggerOffset) false false))
    (:NewEnumerator1
      (Utilities|IsValid (Variables|Default|GetBoxTrigger)
        (:Is%20Valid
          _)
        (:Is%20Not%20Valid
          (bind _returnvalue_2 (AddComponent|AddBoxComponent false))
          (bind _output_get_2 (Variables|Default|SetBoxTrigger _returnvalue_2))
          (Utilities|IsValid _output_get_2
            (:Is%20Valid
              _))))
      (Components|Box|SetBoxExtent _output_get_2 (Variables|Trigger|GetTriggerBoxDimension) true)
      (Collision|SetCollisionResponsetoAllChannels (Variables|Default|GetBoxTrigger) "ECR_Overlap")
      (Collision|SetCollisionResponsetoChannel (Variables|Default|GetBoxTrigger) "ECC_PhysicsBody" "ECR_Ignore")
      (Development|SetHiddeninGame (Variables|Default|GetBoxTrigger) (Variables|Trigger|GetTriggerHiddenIngame) false)
      (Transformation|SetRelativeLocation (Variables|Default|GetBoxTrigger) (Variables|Trigger|GetTriggerOffset) false false))
    (:NewEnumerator2
      (Utilities|IsValid (Variables|Default|GetCapsuleTrigger)
        (:Is%20Valid
          _)
        (:Is%20Not%20Valid
          (bind _returnvalue_3 (AddComponent|AddCapsuleComponent false))
          (bind _output_get_3 (Variables|Default|SetCapsuleTrigger _returnvalue_3))
          (Utilities|IsValid _output_get_3
            (:Is%20Valid
              _))))
      (Components|Capsule|SetCapsuleRadius _output_get_3 (Variables|Trigger|GetTriggerRadius) true)
      (Components|Capsule|SetCapsuleHalfHeight (Variables|Default|GetCapsuleTrigger) (Variables|Trigger|GetTriggerHalfHeight) true)
      (Collision|SetCollisionResponsetoAllChannels (Variables|Default|GetCapsuleTrigger) "ECR_Overlap")
      (Collision|SetCollisionResponsetoChannel (Variables|Default|GetCapsuleTrigger) "ECC_PhysicsBody" "ECR_Ignore")
      (Development|SetHiddeninGame (Variables|Default|GetCapsuleTrigger) (Variables|Trigger|GetTriggerHiddenIngame) false)
      (Transformation|SetRelativeLocation (Variables|Default|GetCapsuleTrigger) (Variables|Trigger|GetTriggerOffset) false false))))

(fn DebugInteractionMessage
  (params (InteractioEventCalled :type String))
  (Development|PrintString (Utilities|String|MakeLiteralString (Utilities|String|Append (Utilities|GetDisplayName self) ": " "is calling the Interaction event for " InteractioEventCalled))))

(fn GetInteractionController
  (return 0))