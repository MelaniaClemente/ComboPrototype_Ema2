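; Pickup actor that grants loot on interaction: usually a random resource, otherwise a Gogo diary unlock.
; Resources get a type-based random quantity, are added to the player controller and synced to the game instance.
; The diary branch marks locked GogoDiary entries unlocked, though the all-unlocked check reads a separate GogosDiary array.
; Both branches show a loot notification, play a UI sound and destroy the actor after a short timer.
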(event Custom|SelfKill
  (Actor|DestroyActor))

(event EventBeginPlay
  (|CallParentFunction) ; This node is disabled and will not be called.\nDrag off pins to build functionality.
)

(event Collision|EventActorBeginOverlap
  (params (OtherActor :type Actor%20Object%20Reference))
  (|CallParentFunction OtherActor) ; This node is disabled and will not be called.\nDrag off pins to build functionality.
)

(event EventTick
  (params (DeltaSeconds :type Float%20%28single-precision%29))
  (|CallParentFunction DeltaSeconds) ; This node is disabled and will not be called.\nDrag off pins to build functionality.
)

(event EventPickUpInteraction
  (bind _asbp_player_conroller (Utilities|Casting|CastToBP_PlayerConroller (Game|GetPlayerController 0)))
  (Variables|Default|SetControllerRef _asbp_player_conroller)
  (Variables|Default|SetInteractionType "NewEnumerator2")
  (switch Utilities|FlowControl|Switch|SwitchonENUM_DropType (CallFunction|GenerateRandomDropType 0.9)
    (:NewEnumerator0
      (bind _output_get (Variables|Default|SetResourceDropped (CallFunction|DropRandomResource)))
      (Default|LootNotification (Variables|Default|GetControllerRef) "NewEnumerator0" (.type _output_get) "NewEnumerator3" (.currentquantity _output_get))
      (Default|PlayUISound (Variables|Default|GetControllerRef) "/Game/Assets/Sounds/Dungeon/MISC/Cues/CUE_Coins.CUE_Coins" 1.0 1.0 0.0)
      (for (_array_element _array_index) (Variables|/Game/Scripts/Blueprints/Controllers/Player/BP_PlayerConroller.BP_PlayerConroller_C|GetCurrentResources (Variables|Default|GetControllerRef))
        (if (== (.type (Variables|Default|GetResourceDropped)) (.type _array_element))
          (bind _structout (Utilities|Struct|SetmembersinStruct_Resources_new (Utilities|Array|Get(acopy) (Variables|/Game/Scripts/Blueprints/Controllers/Player/BP_PlayerConroller.BP_PlayerConroller_C|GetCurrentResources (Variables|Default|GetControllerRef)) _array_index) (+ (.CurrentQuantity (Utilities|Struct|BreakStruct_Resources_new (Utilities|Array|Get(acopy) (Variables|/Game/Scripts/Blueprints/Controllers/Player/BP_PlayerConroller.BP_PlayerConroller_C|GetCurrentResources (Variables|Default|GetControllerRef)) _array_index))) (.currentquantity (Variables|Default|GetResourceDropped)))))
          (Utilities|Array|SetArrayElem (Variables|/Game/Scripts/Blueprints/Controllers/Player/BP_PlayerConroller.BP_PlayerConroller_C|GetCurrentResources (Variables|Default|GetControllerRef)) _array_index _structout)))
      (Default|UpdateConsumablesinGameInstance (Variables|Default|GetControllerRef)))
    (:NewEnumerator1
      (bind _unlockedpage (CallFunction|UnlockRandomDiary))
      (Default|LootNotification (Variables|Default|GetControllerRef) "NewEnumerator1" "NewEnumerator0" "NewEnumerator3" (+ _unlockedpage 1))
      (Default|PlayUISound (Variables|Default|GetControllerRef) "/Game/Assets/Sounds/Dungeon/MISC/Cues/CUE_Paper.CUE_Paper" 1.0 1.0 0.0)))
  (Utilities|Time|SetTimerbyEvent (delegate Custom|SelfKill) 0.5))

(event EventOnSnapDataLoaded)

(fn ConstructionScript
  (|CallParentFunction))

(fn DropRandomResource
  (bind _output_get (LocalVariables|SetRandomResourceType (Utilities|RandomItem (Utilities|Array|MakeArray "NewEnumerator0" "NewEnumerator1" "NewEnumerator2" "NewEnumerator3"))))
  (LocalVariables|SetRandomQuantity (Utilities|Select :Index _output_get :NewEnumerator0 (Math|Random|RandomIntegerinRange 70 245) :NewEnumerator1 (Math|Random|RandomIntegerinRange 3 7) :NewEnumerator2 (Math|Random|RandomIntegerinRange 15 25) :NewEnumerator3 (Math|Random|RandomIntegerinRange 3 7)))
  (bind _structout (Utilities|Struct|SetmembersinStruct_Resources_new (LocalVariables|GetRandomResource) (LocalVariables|GetRandomResourceType) (LocalVariables|GetRandomQuantity) 999999))
  (bind _output_get_2 (LocalVariables|SetRandomResource _structout))
  (return _output_get_2))

(fn GenerateRandomDropType
  (params (ResourcePercentage :type Float%20%28single-precision%29))
  (if (CallFunction|UnlockedAllDiaries?)
    (LocalVariables|SetDrop "NewEnumerator0")
    (elif (< (Math|Random|RandomFloatinRange 0.0 1.0) ResourcePercentage)
      (LocalVariables|SetDrop "NewEnumerator0")
      (else
        (LocalVariables|SetDrop "NewEnumerator1"))))
  (return (LocalVariables|GetDrop)))

(fn UnlockRandomDiary
  (bind _asbp_gameplay_instance (Utilities|Casting|CastToBP_GameplayInstance (Game|GetGameInstance)))
  (LocalVariables|SetGameInstanceLocal _asbp_gameplay_instance)
  (bind _output_get (LocalVariables|SetLocalUnlockedDiaries (.unlocked (Variables|/Game/Scripts/Blueprints/GameModes/BP_GameplayInstance.BP_GameplayInstance_C|GetGogoDiary (LocalVariables|GetGameInstanceLocal)))))
  (for (_array_element _array_index) _output_get
    (if (not _array_element)
      (Utilities|Array|SetArrayElem (LocalVariables|GetLocalUnlockedDiaries) _array_index true)
      (LocalVariables|SetUnlockedPart _array_index)
      (bind _structout (Utilities|Struct|SetmembersinStruct_NarrativeDocument (Variables|/Game/Scripts/Blueprints/GameModes/BP_GameplayInstance.BP_GameplayInstance_C|GetGogoDiary (LocalVariables|GetGameInstanceLocal)) (LocalVariables|GetLocalUnlockedDiaries)))
      (Variables|/Game/Scripts/Blueprints/GameModes/BP_GameplayInstance.BP_GameplayInstance_C|SetGogoDiary (LocalVariables|GetGameInstanceLocal) _structout))))

(fn UnlockedAllDiaries?
  (bind _asbp_gameplay_instance (Utilities|Casting|CastToBP_GameplayInstance (Game|GetGameInstance)))
  (for _array_element (Variables|/Game/Scripts/Blueprints/GameModes/BP_GameplayInstance.BP_GameplayInstance_C|GetGogo'sDiary _asbp_gameplay_instance)
    (bind _output_get (LocalVariables|SetRet (.unlocked _array_element)))
    (if (not _output_get)
      (return (LocalVariables|GetRet))))
  (return (LocalVariables|GetRet)))