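; Item-slot interactable mushroom that rolls a random color (except Orange), which sets its material, name, description and gas effect.
; Valid combinations drop reagents, with some also granting a color-based consumable, then fade it to spent Orange, restored on snapshot load.
; Invalid combinations shake it via material wind parameters and release gas.
; Tick applies the color's fatigue or health action after a delay, once per overlap; Red and Green define none.
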(event OnComponentBeginOverlap(Capsule)
  (params (OverlappedComponent :type Primitive%20Component%20Object%20Reference) (OtherActor :type Actor%20Object%20Reference) (OtherComp :type Primitive%20Component%20Object%20Reference) (OtherBodyIndex :type Integer) (bFromSweep :type Boolean) (SweepResult :type Hit%20Result%20Structure%20%28by%20ref%29))
  (bind _asbp_player_character (Utilities|Casting|CastToBP_PlayerCharacter OtherActor))
  (bind _output_get (Variables|Default|SetOverlappedActor _asbp_player_character))
  (CallFunction|SetGameplayActionbyColor _output_get))

(event OnComponentEndOverlap(Capsule)
  (params (OverlappedComponent :type Primitive%20Component%20Object%20Reference) (OtherActor :type Actor%20Object%20Reference) (OtherComp :type Primitive%20Component%20Object%20Reference) (OtherBodyIndex :type Integer))
  (Utilities|Casting|CastToBP_PlayerCharacter OtherActor)
  (Variables|Default|SetOverlappedActor 0))

(event Custom|CombinationResults
  (params (CombinationIndex :type Integer))
  (bind _controllerref_0 (Variables|Default|GetControllerRef_0))
  (Utilities|IsValid (Variables|/Game/Scripts/Blueprints/Controllers/Player/BP_PlayerConroller.BP_PlayerConroller_C|GetItemInteractionWidget (Variables|Default|GetControllerRef_0))
    (:Is%20Valid
      (Development|PrintString (Utilities|String|ToString(Integer) CombinationIndex))
      (switch int CombinationIndex
        (:Default
          (Development|PrintString "Unvalid Combination" :!label _label)
          (CallFunction|Shake)
          (CallFunction|ActiveGas)
          (CallFunction|SpendCombinationConsumables)
          (Default|RemoveItemSlotWidget (Variables|Default|GetControllerRef_0) :!label _label_2))
        (:-1
          (goto _label))
        (:0
          (Development|PrintString "No Interaction")
          (Default|RemoveItemSlotWidget (Variables|Default|GetControllerRef_0)))
        (:1
          (CallFunction|SpendCombinationConsumables)
          (CallFunction|DropReagents)
          (CallFunction|EndInteraction)
          (goto _label_2))
        (:2
          (CallFunction|SpendCombinationConsumables)
          (switch Utilities|FlowControl|Switch|SwitchonEnum_Colors (Variables|Default|GetColor)
            (:NewEnumerator0
              (Default|AddConsumable _controllerref_0 "NewEnumerator1" 1))
            (:NewEnumerator1
              (Default|AddConsumable _controllerref_0 "NewEnumerator2" 1))
            (:NewEnumerator2
              _)
            (:NewEnumerator3
              _)
            (:NewEnumerator5
              _))
          (CallFunction|DropReagents)
          (CallFunction|EndInteraction)
          (goto _label_2))))))

(event Custom|EndInteraction
  (bind (_color_a1 _color_b1 _color_c1 _emissive_color1) (CallFunction|GetColorbyEnum "NewEnumerator4"))
  (Variables|Default|SetInteractionType "NewEnumerator2")
  (bind (_direction _coloralpha _windalpha) (Timeline|ColorTimeline Play)
    (:Update
      (CallFunction|SetMushRoomColors (Variables|Default|GetDynamicMaterial) (Math|Color|Lerp(LinearColor) (.Color%20A1 (CallFunction|GetColorbyEnum (Variables|Default|GetColor))) _color_a1 _coloralpha) (Math|Color|Lerp(LinearColor) (.Color%20B1 (CallFunction|GetColorbyEnum (Variables|Default|GetColor))) _color_b1 _coloralpha) (Math|Color|Lerp(LinearColor) (.Color%20C1 (CallFunction|GetColorbyEnum (Variables|Default|GetColor))) _color_c1 _coloralpha) (Math|Color|Lerp(LinearColor) (.Emissive%20Color1 (CallFunction|GetColorbyEnum (Variables|Default|GetColor))) _emissive_color1 _coloralpha))
      (CallFunction|SetWindIntensity (Math|Float|Lerp 0.15 0.3 _windalpha) (Math|Float|Lerp 0.15 0.3 _windalpha)))
    (:Finished
      (Variables|Default|SetColor "NewEnumerator4"))))

(event Custom|Shake
  (bind _windalpha (Timeline|ShakeTimeline PlayFromStart)
    (:Update
      (CallFunction|SetWindIntensity (Math|Float|Lerp 0.15 0.3 _windalpha) (Math|Float|Lerp 0.15 0.3 _windalpha)))))

(event EventBeginPlay
  (|CallParentFunction)
  (bind _asbp_player_conroller (Utilities|Casting|CastToBP_PlayerConroller (Game|GetPlayerController 0)))
  (Variables|Default|SetControllerRef_0 _asbp_player_conroller)
  (if (Utilities|Enum|NotEqual(Enum) (Variables|Default|GetInteractionType) "NewEnumerator2")
    (CallFunction|InitializeColor)
    (else
      (Variables|Default|SetColor "NewEnumerator4")))
  (EventDispatchers|BindEventtoOnCombinationMatch (delegate Custom|CombinationResults)))

(event Collision|EventActorBeginOverlap
  (params (OtherActor :type Actor%20Object%20Reference))
  (|CallParentFunction OtherActor))

(event EventTick
  (params (DeltaSeconds :type Float%20%28single-precision%29))
  (bind _overlappedactor (Variables|Default|GetOverlappedActor))
  (bind _gas (Variables|Default|GetGas))
  (bind _overlappedactor_2 (Variables|Default|GetOverlappedActor))
  (bind _returnvalue (Utilities|IsValid _overlappedactor))
  (bind _returnvalue_2 (Components|Activation|IsActive _gas))
  (bind _returnvalue_3 (and _returnvalue _returnvalue_2))
  (|CallParentFunction DeltaSeconds)
  (if _returnvalue_3
    (Utilities|FlowControl|DoOnce _returnvalue_3 :!label _label
      (:Completed
        (Utilities|FlowControl|Delay 0.5)
        (Utilities|IsValid _overlappedactor_2
          (:Is%20Valid
            (CallFunction|SingleTargetGameplayAction _overlappedactor_2 (Variables|Default|GetGasGameplayAction) false)))))
    (else
      (goto _label Reset))))

(event EventOnSnapDataLoaded
  (if (Utilities|Enum|Equal(Enum) (Variables|Default|GetInteractionType) "NewEnumerator2")
    (Variables|Default|SetColor "NewEnumerator4")
    (CallFunction|UpdateTextbyColor)
    (CallFunction|SetGasTemplatebyColor)
    (CallFunction|SetMaterialbyColor)))

(fn ConstructionScript
  (|CallParentFunction))

(fn UpdateTextbyColor
  (bind _color (Variables|Default|GetColor))
  (bind _returnvalue (Utilities|String|EnumtoString _color))
  (bind _returnvalue_2 (Utilities|Select :Index _color :NewEnumerator0 ", some say they have healing effects." :NewEnumerator1 ", or as invigorating medicines." :NewEnumerator2 "." :NewEnumerator3 "." :NewEnumerator4 "." :NewEnumerator5 "."))
  (bind _returnvalue_3 (Utilities|String|Append _returnvalue_2 ""))
  (bind _returnvalue_4 (Utilities|String|Append "A strange " _returnvalue " mushroom, typically grows in humid undergrounds." " 
" "Its pigments are often used as alchemical reagents" _returnvalue_3))
  (bind _returnvalue_5 (Utilities|Text|ToText(String) _returnvalue_4))
  (Variables|Default|SetItemName (Utilities|Text|ToText(String) (Utilities|String|Append (Utilities|String|EnumtoString (Variables|Default|GetColor)) " " "Obnoxy")))
  (Development|PrintString (Utilities|String|ToString(Text) _returnvalue_5))
  (Variables|Default|SetItemDescription _returnvalue_5))

(fn SetMaterialbyColor
  (bind _staticmesh (Variables|Default|GetStaticMesh))
  (bind _color (Variables|Default|GetColor))
  (bind (_color_a1 _color_b1 _color_c1 _emissive_color1) (CallFunction|GetColorbyEnum _color))
  (bind _returnvalue (Rendering|Material|CreateDynamicMaterialInstance _staticmesh 0 "/Game/Scripts/Materials/Instances/CustomOpaque/Misc/MI_Mushroom_Small_CustomColor.MI_Mushroom_Small_CustomColor" "None" :!class /Script/Engine.PrimitiveComponent))
  (bind _output_get (Variables|Default|SetDynamicMaterial _returnvalue))
  (Rendering|Material|SetMaterial _staticmesh 0 _output_get)
  (CallFunction|SetMushRoomColors (Variables|Default|GetDynamicMaterial) _color_a1 _color_b1 _color_c1 _emissive_color1))

(fn SpawnSmoke)

(fn InitializeColor
  (CallFunction|SetRandomColor)
  (CallFunction|SetMaterialbyColor)
  (CallFunction|SetGasTemplatebyColor)
  (CallFunction|UpdateTextbyColor))

(fn SetGasTemplatebyColor
  (Effects|Components|ParticleSystem|SetTemplate (Variables|Default|GetGas) (Utilities|Select :Index (Variables|Default|GetColor) :NewEnumerator0 "/Game/Assets/Particles/Nature/Smokes/PS_MushroomSmoke_Red.PS_MushroomSmoke_Red" :NewEnumerator1 "/Game/Assets/Particles/Nature/Smokes/PS_MushroomSmoke_Green.PS_MushroomSmoke_Green" :NewEnumerator2 "/Game/Assets/Particles/Nature/Smokes/PS_MushroomSmoke_Blue.PS_MushroomSmoke_Blue" :NewEnumerator3 "/Game/Assets/Particles/Nature/Smokes/PS_MushroomSmoke_Yellow.PS_MushroomSmoke_Yellow" :NewEnumerator4 "/Game/Assets/Particles/Nature/Smokes/PS_MushroomSmoke_Orange.PS_MushroomSmoke_Orange" :NewEnumerator5 "/Game/Assets/Particles/Nature/Smokes/PS_MushroomSmoke_Purple.PS_MushroomSmoke_Purple")))

(fn ActiveGas
  (Components|Activation|SetActive (Variables|Default|GetGas) true false))

(fn SetGameplayActionbyColor
  (params (Character :type BP%20Player%20Character%20Object%20Reference))
  (bind _array (Utilities|Array|MakeArray "NewEnumerator0"))
  (bind _array_2 (Utilities|Array|MakeArray "NewEnumerator3"))
  (bind _fatiguecomponent (Variables|/Game/Scripts/Blueprints/Characters/BP_PlayerCharacter.BP_PlayerCharacter_C|GetFatigueComponent Character))
  (bind _bp_healthcomponent (Variables|/Game/Scripts/Blueprints/Characters/BP_CharacterMaster.BP_CharacterMaster_C|GetBP_HealthComponent Character))
  (bind _maxvalue (Default|GetMaxValue _fatiguecomponent))
  (bind _maxvalue_2 (Default|GetMaxValue _bp_healthcomponent))
  (bind _returnvalue (* _maxvalue 0.05))
  (bind _returnvalue_2 (* _maxvalue_2 0.05))
  (bind _array_3 (Utilities|Array|MakeArray _returnvalue))
  (bind _array_4 (Utilities|Array|MakeArray _returnvalue_2))
  (bind _struct_gameactions_new (Utilities|Struct|MakeSTRUCT_GameActions_new "NewEnumerator3" _array _array_4))
  (bind _struct_gameactions_new_2 (Utilities|Struct|MakeSTRUCT_GameActions_new "NewEnumerator4" _array_2 _array_3))
  (Variables|Default|SetGasGameplayAction (Utilities|Select :Index (Variables|Default|GetColor) :NewEnumerator0 "" :NewEnumerator1 "" :NewEnumerator2 _struct_gameactions_new_2 :NewEnumerator3 _struct_gameactions_new_2 :NewEnumerator4 _struct_gameactions_new :NewEnumerator5 _struct_gameactions_new)))

(fn SetMushRoomColors
  (params (Material :type Material%20Instance%20Dynamic%20Object%20Reference) (Color%20A :type Linear%20Color%20Structure) (Color%20B :type Linear%20Color%20Structure) (Color%20C :type Linear%20Color%20Structure) (EmissiveColor :type Linear%20Color%20Structure))
  (Rendering|Material|SetVectorParameterValue Material "BaseColor_A" Color%20A :!class /Script/Engine.MaterialInstanceDynamic)
  (Rendering|Material|SetVectorParameterValue Material "BaseColor_B" Color%20B :!class /Script/Engine.MaterialInstanceDynamic)
  (Rendering|Material|SetVectorParameterValue Material "BaseColor_C" Color%20C :!class /Script/Engine.MaterialInstanceDynamic)
  (Rendering|Material|SetVectorParameterValue Material "EmissiveColor" EmissiveColor :!class /Script/Engine.MaterialInstanceDynamic))

(fn GetColorbyEnum
  (params (Color :type Enum_Colors%20Enum :default "NewEnumerator0"))
  (LocalVariables|SetColorEnum Color)
  (LocalVariables|SetColor%20A (Utilities|Select :Index (LocalVariables|GetColorEnum) :NewEnumerator0 "(R=0.130136,G=0.023153,B=0.030713,A=1.000000)" :NewEnumerator1 "(R=0.027321,G=0.124772,B=0.046665,A=1.000000)" :NewEnumerator2 "(R=0.004526,G=0.035100,B=0.078187,A=1.000000)" :NewEnumerator3 "(R=0.166667,G=0.125289,B=0.005844,A=1.000000)" :NewEnumerator4 "(R=0.025187,G=0.017878,B=0.012725,A=1.000000)" :NewEnumerator5 "(R=0.029557,G=0.017642,B=0.040915,A=1.000000)"))
  (LocalVariables|SetColor%20B (Utilities|Select :Index (LocalVariables|GetColorEnum) :NewEnumerator0 "(R=0.630757,G=0.052563,B=0.091348,A=1.000000)" :NewEnumerator1 "(R=0.156250,G=0.666667,B=0.263597,A=1.000000)" :NewEnumerator2 "(R=0.023950,G=0.223971,B=0.412543,A=1.000000)" :NewEnumerator3 "(R=0.545725,G=0.456411,B=0.109462,A=1.000000)" :NewEnumerator4 "(R=0.234375,G=0.154741,B=0.098877,A=1.000000)" :NewEnumerator5 "(R=0.215861,G=0.127438,B=0.296138,A=1.000000)"))
  (LocalVariables|SetColor%20C (Utilities|Select :Index (LocalVariables|GetColorEnum) :NewEnumerator0 "(R=0.630757,G=0.203682,B=0.232330,A=1.000000)" :NewEnumerator1 "(R=0.239583,G=1.000000,B=0.399508,A=1.000000)" :NewEnumerator2 "(R=0.000000,G=0.068478,B=0.412543,A=1.000000)" :NewEnumerator3 "(R=0.545725,G=0.456411,B=0.109462,A=1.000000)" :NewEnumerator4 "(R=0.244792,G=0.160870,B=0.101997,A=1.000000)" :NewEnumerator5 "(R=0.215861,G=0.127438,B=0.296138,A=1.000000)"))
  (LocalVariables|SetEmissive%20Color (Utilities|Select :Index (LocalVariables|GetColorEnum) :NewEnumerator0 "(R=0.630757,G=0.223393,B=0.250718,A=1.000000)" :NewEnumerator1 "(R=0.458333,G=1.000000,B=0.572253,A=1.000000)" :NewEnumerator2 "(R=0.097165,G=0.307856,B=0.412543,A=1.000000)" :NewEnumerator3 "(R=0.545725,G=0.485790,B=0.252966,A=1.000000)" :NewEnumerator4 "(R=0.250000,G=0.189545,B=0.147135,A=1.000000)" :NewEnumerator5 "(R=0.261642,G=0.223646,B=0.296138,A=1.000000)"))
  (return (LocalVariables|GetColor%20A) (LocalVariables|GetColor%20B) (LocalVariables|GetColor%20C) (LocalVariables|GetEmissive%20Color)))

(fn DropReagents
  (bind _controllerref_0 (Variables|Default|GetControllerRef_0))
  (Default|AddResource _controllerref_0 "NewEnumerator3" (.currentquantity (Default|GetRandomResource _controllerref_0 (Utilities|Array|MakeArray "NewEnumerator3")))))

(fn SetRandomColor
  (Variables|Default|SetColor (Utilities|RandomItem (Utilities|Array|MakeArray "NewEnumerator0" "NewEnumerator1" "NewEnumerator2" "NewEnumerator3" "NewEnumerator5"))))

(fn SetWindIntensity
  (params (WindIntensity :type Float%20%28single-precision%29) (WindSpeed :type Float%20%28single-precision%29))
  (bind _dynamicmaterial (Variables|Default|GetDynamicMaterial))
  (Utilities|IsValid _dynamicmaterial
    (:Is%20Valid
      (Rendering|Material|SetScalarParameterValue _dynamicmaterial "WindIntensity (S)" WindIntensity :!class /Script/Engine.MaterialInstanceDynamic)
      (Rendering|Material|SetScalarParameterValue _dynamicmaterial "WindSpeed (S)" WindSpeed :!class /Script/Engine.MaterialInstanceDynamic))))