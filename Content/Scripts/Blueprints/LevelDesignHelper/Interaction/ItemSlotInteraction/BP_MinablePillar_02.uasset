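; Minable "Mining Vein" pillar interactable that rewards the player with gems when the correct item-slot combination is used on it.
; On a combination match it spends the slotted consumables and removes the slot widget; index -1 only consumes, while other non-matching indices print "No Interaction".
; A successful match adds a random gem quantity, then radius damage fractures the destructible mesh with debris sound before a timer destroys the actor.
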(event OnComponentFracture(Pillar)
  (params (HitPoint :type Vector%20%28by%20ref%29 :default "0, 0, 0") (HitDirection :type Vector%20%28by%20ref%29 :default "0, 0, 0"))
  (Audio|PlaySoundatLocation "/Game/Assets/Sounds/Dungeon/Craft_and_Environment/Cues/CUE_StoneDebris.CUE_StoneDebris" HitPoint "0, 0, 0" 1.0 1.0 0.0 0 0 0))

(event Custom|FractureMesh
  (Variables|Default|SetInteractionType "NewEnumerator2")
  (Class|DestructibleComponent|ApplyRadiusDamage (Variables|Default|GetPillar) 5.0 (Transformation|GetWorldLocation (Variables|Default|GetPillar)) 2.5e+02 2.5e+02 false)
  (Utilities|Time|SetTimerbyEvent (delegate Custom|Suicide) 2.5))

(event Custom|Suicide
  (Actor|DestroyActor))

(event Custom|CombinationMatch
  (params (CombinationIndex :type Integer))
  (Utilities|IsValid (Variables|/Game/Scripts/Blueprints/Controllers/Player/BP_PlayerConroller.BP_PlayerConroller_C|GetItemInteractionWidget (Variables|Default|GetControllerRef_0))
    (:Is%20Valid
      (switch int CombinationIndex
        (:Default
          (Development|PrintString "No Interaction" :!label _label)
          (Default|RemoveItemSlotWidget (Variables|Default|GetControllerRef_0)))
        (:-1
          (CallFunction|SpendConsumable)
          (Default|RemoveItemSlotWidget (Variables|Default|GetControllerRef_0)))
        (:0
          (goto _label))
        (:1
          (CallFunction|SpendConsumable)
          (Default|RemoveItemSlotWidget (Variables|Default|GetControllerRef_0))
          (CallFunction|DropGems)
          (CallFunction|FractureMesh))))))

(event EventBeginPlay
  (|CallParentFunction)
  (bind _asbp_player_conroller (Utilities|Casting|CastToBP_PlayerConroller (Game|GetPlayerController 0)))
  (Variables|Default|SetControllerRef_0 _asbp_player_conroller)
  (CallFunction|UpdateTexts)
  (EventDispatchers|BindEventtoOnCombinationMatch (delegate Custom|CombinationMatch)))

(event Collision|EventActorBeginOverlap
  (params (OtherActor :type Actor%20Object%20Reference))
  (|CallParentFunction OtherActor) ; This node is disabled and will not be called.\nDrag off pins to build functionality.
)

(event EventTick
  (params (DeltaSeconds :type Float%20%28single-precision%29))
  (|CallParentFunction DeltaSeconds) ; This node is disabled and will not be called.\nDrag off pins to build functionality.
)

(fn ConstructionScript
  (|CallParentFunction))

(fn SpendConsumable
  (bind _playercontrollerref (Variables|Default|GetPlayerControllerRef))
  (Utilities|IsValid _playercontrollerref
    (:Is%20Valid
      (for _array_element (Variables|/Game/Scripts/Blueprints/UI/BPW_ItemInterractionWidget.BPW_ItemInterractionWidget_C|GetCombination (Variables|/Game/Scripts/Blueprints/Controllers/Player/BP_PlayerConroller.BP_PlayerConroller_C|GetItemInteractionWidget _playercontrollerref))
        (Default|SpendConsumable (Variables|Default|GetPlayerControllerRef) _array_element 1)))))

(fn DropGems
  (bind _controllerref_0 (Variables|Default|GetControllerRef_0))
  (Default|AddResource _controllerref_0 "NewEnumerator2" (.currentquantity (Default|GetRandomResource _controllerref_0 (Utilities|Array|MakeArray "NewEnumerator3")))))

(fn UpdateTexts
  (Variables|Default|SetItemName "Mining Vein")
  (Variables|Default|SetItemDescription "Varius shiny and colored vains nestle in the stone forming many small crystals. They seem to be very precious."))