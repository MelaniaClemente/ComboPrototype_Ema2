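; Master Blueprint for item-slot interactibles, which open a widget where the player combines consumables.
; ItemInteraction has the player controller create the slot widget and fills in name, description and slot count, while Tick removes it once no interactive actor is current.
; SpendCombinationConsumables charges one of each consumable in the widget's combination.
; CombinationMatched only prints the result; its binding and the end-overlap removal binding are never executed here.
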(event Custom|RemoveWidget
  (params (OtherActor :type Actor%20Object%20Reference))
  (bind _asbp_player_character (Utilities|Casting|CastToBP_PlayerCharacter OtherActor))
  (bind _asbp_player_conroller (Utilities|Casting|CastToBP_PlayerConroller (Pawn|GetController _asbp_player_character)))
  (Default|RemoveItemSlotWidget _asbp_player_conroller))

(event Custom|CombinationMatched
  (params (CombinationIndex :type Integer))
  (switch int CombinationIndex
    (:Default
      (Development|PrintString (Utilities|String|Append "MatchedCombination: " (Utilities|String|ToString(Integer) CombinationIndex))))
    (:-1
      (Development|PrintString "Unvalid Combination"))))

(event EventBeginPlay
  (|CallParentFunction)
  (bind _asbp_player_conroller (Utilities|Casting|CastToBP_PlayerConroller (Game|GetPlayerController 0)))
  (Variables|Default|SetPlayerControllerRef _asbp_player_conroller))

(event Collision|EventActorBeginOverlap
  (params (OtherActor :type Actor%20Object%20Reference))
  (|CallParentFunction OtherActor) ; This node is disabled and will not be called.\nDrag off pins to build functionality.
)

(event EventTick
  (params (DeltaSeconds :type Float%20%28single-precision%29))
  (bind _playercontrollerref (Variables|Default|GetPlayerControllerRef))
  (|CallParentFunction DeltaSeconds)
  (Utilities|IsValid (Variables|/Game/Scripts/Blueprints/Controllers/Player/BP_PlayerConroller.BP_PlayerConroller_C|GetCurrentInteractiveActor (Variables|Default|GetPlayerControllerRef))
    (:Is%20Not%20Valid
      (Utilities|IsValid (Variables|/Game/Scripts/Blueprints/Controllers/Player/BP_PlayerConroller.BP_PlayerConroller_C|GetItemInteractionWidget _playercontrollerref)
        (:Is%20Valid
          (Default|RemoveItemSlotWidget _playercontrollerref))))))

(event EventItemInteraction
  (bind _playercontrollerref (Variables|Default|GetPlayerControllerRef))
  (bind _iteminteractionwidget (Variables|/Game/Scripts/Blueprints/Controllers/Player/BP_PlayerConroller.BP_PlayerConroller_C|GetItemInteractionWidget _playercontrollerref))
  (Utilities|IsValid (Variables|/Game/Scripts/Blueprints/Controllers/Player/BP_PlayerConroller.BP_PlayerConroller_C|GetItemInteractionWidget _playercontrollerref)
    (:Is%20Not%20Valid
      (Default|InitializeItemSlotWidget _playercontrollerref self)
      (Default|SetTexts _iteminteractionwidget (Variables|WidgetTexts|GetItemName) (Variables|WidgetTexts|GetItemDescription))
      (Variables|/Game/Scripts/Blueprints/UI/BPW_ItemInterractionWidget.BPW_ItemInterractionWidget_C|SetNumberOfSlots _iteminteractionwidget (Variables|Interaction|GetConsumableSlots))
      (Default|Initialization _iteminteractionwidget))))

(fn ConstructionScript
  (|CallParentFunction))

(fn SpendCombinationConsumables
  (bind _playercontrollerref (Variables|Default|GetPlayerControllerRef))
  (Utilities|IsValid _playercontrollerref
    (:Is%20Valid
      (for _array_element (Variables|/Game/Scripts/Blueprints/UI/BPW_ItemInterractionWidget.BPW_ItemInterractionWidget_C|GetCombination (Variables|/Game/Scripts/Blueprints/Controllers/Player/BP_PlayerConroller.BP_PlayerConroller_C|GetItemInteractionWidget _playercontrollerref))
        (Default|SpendConsumable (Variables|Default|GetPlayerControllerRef) _array_element 1)))))