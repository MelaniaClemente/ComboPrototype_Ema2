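; BP_CheckpointBrazier is an interactable brazier that the player lights by praying, spending a checkpoint consumable to make it their current checkpoint.
; PrayInteraction checks the controller's consumables, then sets the checkpoint, clears the interaction type and plays a sound, or notifies when none remain.
; A looping timer refreshes player references and matches fire and loop sound to the interaction type.
; GetRespawnLocationAndRotation traces down to place the capsule on the ground, keeping only yaw.
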(event Custom|UpdateParticle
  (bind _fire (Variables|Default|GetFire))
  (bind _fireloopsound (Variables|Default|GetFireLoopSound))
  (CallFunction|UpdateReferences)
  (switch Utilities|FlowControl|Switch|SwitchonENUM_InteractionType (Variables|Default|GetInteractionType)
    (:NewEnumerator2
      (Components|Activation|SetActive _fire true false)
      (Components|Activation|SetActive _fireloopsound true false))
    (:NewEnumerator3
      (Components|Activation|SetActive _fire false false)
      (Components|Activation|SetActive _fireloopsound false false))))

(event EventBeginPlay
  (|CallParentFunction)
  (Utilities|Time|SetTimerbyEvent (delegate Custom|UpdateParticle) 0.1 true))

(event Collision|EventActorBeginOverlap
  (params (OtherActor :type Actor%20Object%20Reference))
  (|CallParentFunction OtherActor) ; This node is disabled and will not be called.\nDrag off pins to build functionality.
)

(event EventTick
  (params (DeltaSeconds :type Float%20%28single-precision%29))
  (|CallParentFunction DeltaSeconds) ; This node is disabled and will not be called.\nDrag off pins to build functionality.
)

(event EventPrayInteraction
  (bind _characterref (Variables|Default|GetCharacterRef))
  (bind _controllerref (Variables|Default|GetControllerRef))
  (Variables|Default|SetNumberOfCheckpoint 0)
  (Utilities|IsValid _controllerref
    (:Is%20Valid
      (for _array_element (Variables|/Game/Scripts/Blueprints/Controllers/Player/BP_PlayerConroller.BP_PlayerConroller_C|GetConsumablesArray _controllerref)
        (if (Utilities|Enum|Equal(Enum) (.type _array_element) "NewEnumerator0")
          (bind _output_get (Variables|Default|SetNumberOfCheckpoint (.currentquantity _array_element)))
          (Development|PrintString (Utilities|String|ToString(Integer) _output_get))))
      (if (> (Variables|Default|GetNumberOfCheckpoint) 0)
        (Utilities|IsValid _characterref
          (:Is%20Valid
            (bind _success (CallFunction|UseConsumableCheckpoint))
            (if _success
              (Variables|/Game/Scripts/Blueprints/Characters/BP_PlayerCharacter.BP_PlayerCharacter_C|SetCurrentCheckpoint _characterref self)
              (Variables|Default|SetInteractionType "NewEnumerator2")
              (Audio|Components|Audio|Play (Variables|Default|GetActivationSound) 0.0)
              (Default|CheckpointActivatedNotification (Variables|Default|GetControllerRef))))
          (:Is%20Not%20Valid
            (Development|PrintString "Hello")))
        (else
          (Default|NoCheckpointNotification (Variables|Default|GetControllerRef)))))))

(fn ConstructionScript
  (|CallParentFunction))

(fn UpdateReferences
  (bind _returnvalue (Game|GetPlayerController 0))
  (if (Utilities|DoesObjectImplementInterface _returnvalue "/Game/Scripts/Blueprints/Interfaces/BP_CharacterInterface.BP_CharacterInterface_C")
    (bind _myplayercontroller (Class|BPCharacterInterface|GetMyPlayerController(Message) _returnvalue))
    (Variables|Default|SetControllerRef _myplayercontroller))
  (bind _asbp_player_character (Utilities|Casting|CastToBP_PlayerCharacter (Game|GetPlayerCharacter 0))
    (:then
      (Variables|Default|SetCharacterRef _asbp_player_character))
    (:CastFailed
      (Development|PrintString "Hello"))))

(fn GetRespawnLocationandRotation
  (params (Character :type Character%20Object%20Reference))
  (bind _spawnlocationandrotation (Variables|Default|GetSpawnLocationAndRotation))
  (bind _spawnlocationandrotation_2 (Variables|Default|GetSpawnLocationAndRotation))
  (bind _returnvalue (Transformation|GetWorldLocation _spawnlocationandrotation_2))
  (bind _returnvalue_2 (Transformation|GetWorldLocation _spawnlocationandrotation))
  (Variables|Default|SetRespawnRot (Math|Rotator|MakeRotator 0.0 0.0 (.yaw (Transformation|GetWorldRotation _spawnlocationandrotation))))
  (LocalVariables|SetRespawnLoc _returnvalue_2)
  (bind (_outhit _returnvalue_3) (Collision|LineTraceByChannel _returnvalue_2 (- (Transformation|GetWorldLocation (Variables|Default|GetSpawnLocationAndRotation)) "0, 0,5000.000000") "TraceTypeQuery1" false 0 "None"))
  (if _returnvalue_3
    (LocalVariables|SetRespawnLoc (Math|Vector|MakeVector (.x _returnvalue) (.y _returnvalue) (+ (.Z (Math|Vector|BreakVector (.Location (Collision|BreakHitResult _outhit)))) (Components|Capsule|GetScaledCapsuleHalfHeight (Variables|/Script/Engine.Character|GetCapsuleComponent Character))))))
  (return (LocalVariables|GetRespawnLoc) (Variables|Default|GetRespawnRot)))

(fn UseConsumableCheckpoint
  (bind _controllerref (Variables|Default|GetControllerRef))
  (bind _success (Default|UseConsumable _controllerref 0 true))
  (if _success
    (Default|SetConsumableQuantity _controllerref (- (.currentquantity (Utilities|Array|Get(acopy) (Variables|/Game/Scripts/Blueprints/Controllers/Player/BP_PlayerConroller.BP_PlayerConroller_C|GetConsumablesArray _controllerref))) 1))
    (return _success)))