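; BP_DecalMaster is a level-design helper actor that places a configurable decal in the world.
; Its construction script applies the chosen material to the decal component and creates a dynamic material instance from it.
; It then pushes exposed PBR textures and scalar tuning values for normals, specular, contrast, desaturation and opacity into that instance.
; The event graph holds no runtime logic.
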(event EventBeginPlay)

(event Collision|EventActorBeginOverlap
  (params (OtherActor :type Actor%20Object%20Reference)))

(event EventTick
  (params (DeltaSeconds :type Float%20%28single-precision%29)))

(fn ConstructionScript
  (bind _decal (Variables|Default|GetDecal))
  (Rendering|Components|Decal|SetDecalMaterial _decal (Variables|DecalMaterial|GetMaterial))
  (bind _returnvalue (Rendering|Material|CreateDynamicMaterialInstance _decal :!class /Script/Engine.DecalComponent))
  (Variables|Default|SetDecalMaterial _returnvalue)
  (Utilities|FlowControl|Sequence
    (:then_0
      (Rendering|Material|SetTextureParameterValue (Variables|Default|GetDecalMaterial) "BaseColorMap" (Variables|Textures|GetBaseColorTexture))
      (Rendering|Material|SetTextureParameterValue (Variables|Default|GetDecalMaterial) "RoughnessMap" (Variables|Textures|GetRoughnessTexture))
      (Rendering|Material|SetTextureParameterValue (Variables|Default|GetDecalMaterial) "MetallicMap" (Variables|Textures|GetMetallicTexture))
      (Rendering|Material|SetTextureParameterValue (Variables|Default|GetDecalMaterial) "OpacityMap" (Variables|Textures|GetOpacityTexture))
      (Rendering|Material|SetTextureParameterValue (Variables|Default|GetDecalMaterial) "NormalMap" (Variables|Textures|GetNormalTexture)))
    (:then_1
      (Rendering|Material|SetScalarParameterValue (Variables|Default|GetDecalMaterial) "NormalStrenght" (Variables|ScalarParameters|GetNormalStrenght) :!class /Script/Engine.MaterialInstanceDynamic)
      (Rendering|Material|SetScalarParameterValue (Variables|Default|GetDecalMaterial) "Specular" (Variables|ScalarParameters|GetSpecular) :!class /Script/Engine.MaterialInstanceDynamic)
      (Rendering|Material|SetScalarParameterValue (Variables|Default|GetDecalMaterial) "Contrast" (Variables|ScalarParameters|GetContrast) :!class /Script/Engine.MaterialInstanceDynamic)
      (Rendering|Material|SetScalarParameterValue (Variables|Default|GetDecalMaterial) "Desaturation" (Variables|ScalarParameters|GetDesaturation) :!class /Script/Engine.MaterialInstanceDynamic)
      (Rendering|Material|SetScalarParameterValue (Variables|Default|GetDecalMaterial) "OpacityMultiplier" (Variables|ScalarParameters|GetOpacityMultiplier) :!class /Script/Engine.MaterialInstanceDynamic))))