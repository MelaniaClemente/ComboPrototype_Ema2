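; BP_Torch is a torch actor that scales its point light's cost by distance to the player.
; Each tick it measures distance to BP_PlayerCharacter, picks one of four distance bands and computes a clamped blend alpha.
; The nearest tier enables shadows and lerps radius, radius-based intensity and volumetric scattering.
; Tier two disables shadows and lerps radius, tier three switches mobility to Static, and tier four only zeroes the alpha.
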(event EventBeginPlay
  (CallFunction|InitializePlayerCharacter))

(event Collision|EventActorBeginOverlap
  (params (OtherActor :type Actor%20Object%20Reference)))

(event EventTick
  (params (DeltaSeconds :type Float%20%28single-precision%29))
  (Variables|Default|SetCurrentDistance (CallFunction|GetDistancefromPlayer))
  (if (>= (Variables|Default|GetCurrentDistance) 0.0)
    (Utilities|CurrentTier
      (:Tier%201
        (Utilities|CalculateDistanceAlphabyTier :!label _label
          (:Tier%201
            (CallFunction|OptimizetoTier1))
          (:Tier%202
            (CallFunction|OptimizetoTier2))
          (:Tier%203
            (CallFunction|OptimizetoTier3))))
      (:Tier%202
        (goto _label Tier2))
      (:Tier%203
        (goto _label Tier3))
      (:Tier%204
        (goto _label Tier4)))
    (else
      (CallFunction|InitializePlayerCharacter))))

(fn ConstructionScript)

(fn GetDistancefromPlayer
  (Utilities|IsValid (Variables|Default|GetPlayerRef)
    (:Is%20Valid
      (LocalVariables|SetDist (Transformation|GetDistanceTo (Variables|Default|GetPlayerRef) self)))
    (:Is%20Not%20Valid
      (LocalVariables|SetDist -1.0)))
  (return (LocalVariables|GetDist)))

(fn InitializePlayerCharacter
  (bind _asbp_player_character (Utilities|Casting|CastToBP_PlayerCharacter (Game|GetPlayerCharacter 0)))
  (Variables|Default|SetPlayerRef _asbp_player_character))

(fn OptimizetoTier1
  (bind _pointlight (Variables|Default|GetPointLight))
  (Transformation|SetMobility (Variables|Default|GetDefaultSceneRoot) "Movable")
  (Transformation|SetMobility _pointlight "Movable")
  (Rendering|Components|Light|SetCastShadows _pointlight true)
  (Rendering|Lighting|SetAttenuationRadius _pointlight (Math|Float|Lerp (Variables|Default|GetTier1MaxRadius) (Variables|Default|GetTier2MaxRadius) (Variables|Default|GetAlphaDistance)))
  (Rendering|Components|Light|SetIntensity _pointlight (* (Variables|/Script/Engine.LocalLightComponent|GetAttenuationRadius _pointlight) (Variables|Default|GetIntensityMultiplier)))
  (Class|LightComponent|SetVolumetricScatteringIntensity (Variables|Default|GetPointLight) (Math|Float|Lerp (Variables|Default|GetMinVolumetricScattering) (Variables|Default|GetMaxVolumetricScattering) (Variables|Default|GetAlphaDistance))))

(fn OptimizetoTier2
  (bind _pointlight (Variables|Default|GetPointLight))
  (Rendering|Components|Light|SetCastShadows _pointlight false)
  (Transformation|SetMobility (Variables|Default|GetDefaultSceneRoot) "Movable")
  (Transformation|SetMobility _pointlight "Movable")
  (Rendering|Lighting|SetAttenuationRadius (Variables|Default|GetPointLight) (Math|Float|Lerp (Variables|Default|GetTier2MaxRadius) (Variables|Default|GetTier3MaxRadius) (Variables|Default|GetAlphaDistance))))

(fn OptimizetoTier3
  (Transformation|SetMobility (Variables|Default|GetDefaultSceneRoot) "Static")
  (Transformation|SetMobility (Variables|Default|GetPointLight) "Static"))