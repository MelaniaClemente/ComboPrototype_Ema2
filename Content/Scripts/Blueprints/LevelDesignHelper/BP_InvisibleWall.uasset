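; BP_InvisibleWall is a level design helper wall that opens or blocks depending on whether a door is found.
; On BeginPlay it binds to the DoorQuerier's query-completed event.
; A valid door makes the Wall ignore all collision channels and hide, while no door makes it block and show.
; The collision response and visibility are stored in variables and reapplied when snap data loads.
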(event Custom|UpdateCollisions
  (params (Door :type BP%20My%20Door%20Object%20Reference))
  (bind _wall (Variables|Default|GetWall))
  (Utilities|IsValid Door
    (:Is%20Valid
      (Variables|Default|SetCollision%20Response "ECR_Ignore")
      (Variables|Default|SetVisibility false))
    (:Is%20Not%20Valid
      (Variables|Default|SetCollision%20Response "ECR_Block")
      (Variables|Default|SetVisibility true)))
  (Collision|SetCollisionResponsetoAllChannels _wall (Variables|Default|GetCollision%20Response))
  (Development|SetHiddeninGame _wall (not (Variables|Default|GetVisibility)) false)
  (Rendering|SetVisibility _wall (Variables|Default|GetVisibility) false))

(event EventBeginPlay
  (Utilities|IsValid (Variables|Default|GetDoorQuerier)
    (:Is%20Valid
      (EventDispatchers|BindEventtoQueryCompleted (Variables|Default|GetDoorQuerier) (delegate Custom|UpdateCollisions)))))

(event Collision|EventActorBeginOverlap
  (params (OtherActor :type Actor%20Object%20Reference)))

(event EventTick
  (params (DeltaSeconds :type Float%20%28single-precision%29)))

(event EventOnSnapDataLoaded
  (bind _wall (Variables|Default|GetWall))
  (Collision|SetCollisionResponsetoAllChannels _wall (Variables|Default|GetCollision%20Response))
  (Development|SetHiddeninGame _wall (not (Variables|Default|GetVisibility)) false)
  (Rendering|SetVisibility _wall (Variables|Default|GetVisibility) false))

(fn ConstructionScript)