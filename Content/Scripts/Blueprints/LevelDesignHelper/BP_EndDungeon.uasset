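; BP_EndDungeon is a trigger actor that ends a dungeon run when the player character overlaps its Collider.
; It saves the character's Health and Stamina attributes into the SelectedHero struct on BP_GameplayInstance, carrying them across the level change.
; It then has the player controller show the completion notification, fades the camera to black after timed delays and opens MAP_DungeonEnd.
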(event OnComponentBeginOverlap(Collider)
  (params (OverlappedComponent :type Primitive%20Component%20Object%20Reference) (OtherActor :type Actor%20Object%20Reference) (OtherComp :type Primitive%20Component%20Object%20Reference) (OtherBodyIndex :type Integer) (bFromSweep :type Boolean) (SweepResult :type Hit%20Result%20Structure%20%28by%20ref%29))
  (bind _asbp_player_character (Utilities|Casting|CastToBP_PlayerCharacter OtherActor))
  (bind _asbp_player_conroller (Utilities|Casting|CastToBP_PlayerConroller (Pawn|GetController _asbp_player_character)))
  (bind _asbp_gameplay_instance (Utilities|Casting|CastToBP_GameplayInstance (Game|GetGameInstance)))
  (bind _structout (Utilities|Struct|SetmembersinSTRUCT_HeroesData (Variables|/Game/Scripts/Blueprints/GameModes/BP_GameplayInstance.BP_GameplayInstance_C|GetSelectedHero _asbp_gameplay_instance) (Variables|/Game/Scripts/Blueprints/Components/GameParameters/BP_CharacterParametersComponent.BP_CharacterParametersComponent_C|GetGameAttribute (Variables|/Game/Scripts/Blueprints/Characters/BP_CharacterMaster.BP_CharacterMaster_C|GetBP_HealthComponent _asbp_player_character)) (Variables|/Game/Scripts/Blueprints/Components/GameParameters/BP_CharacterParametersComponent.BP_CharacterParametersComponent_C|GetGameAttribute (Variables|/Game/Scripts/Blueprints/Characters/BP_PlayerCharacter.BP_PlayerCharacter_C|GetStaminaComponent _asbp_player_character))))
  (Variables|/Game/Scripts/Blueprints/GameModes/BP_GameplayInstance.BP_GameplayInstance_C|SetSelectedHero _asbp_gameplay_instance _structout)
  (Default|DungeonCompletedNotification _asbp_player_conroller)
  (Utilities|FlowControl|Delay 1.5)
  (CameraFades|StartCameraFade (Game|GetPlayerCameraManager 0) 0.0 1.0 2.0 "(R=0.000000,G=0.000000,B=0.000000,A=1.000000)" false false)
  (Utilities|FlowControl|Delay 2.0)
  (Game|OpenLevel(byName) "MAP_DungeonEnd"))

(event EventBeginPlay)

(event Collision|EventActorBeginOverlap
  (params (OtherActor :type Actor%20Object%20Reference)))

(event EventTick
  (params (DeltaSeconds :type Float%20%28single-precision%29)))

(fn ConstructionScript)