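; Room door manager for dungeons that applies data from door querier objects to the doors they reference.
; UpdateDoorState runs two seconds after BeginPlay, or after OnSnapDataLoaded clears the door list, registering each valid door once.
; UpdateDoor copies the querier's interaction type, leaf rotations and emissive color onto the door.
; On-screen debug prints in Italian report the door count and applied data.
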(event Custom|UpdateDoorState
  (for _array_element (Variables|Default|GetDoorsQuerier)
    (Utilities|IsValid _array_element
      (:Is%20Valid
        (if (not (Utilities|Array|ContainsItem (Variables|Default|GetDoors) (Variables|/Game/Scripts/Blueprints/LevelDesignHelper/Dungeon/BP_DoorQuerier.BP_DoorQuerier_C|GetDoorQueried _array_element)))
          (Utilities|IsValid (Variables|/Game/Scripts/Blueprints/LevelDesignHelper/Dungeon/BP_DoorQuerier.BP_DoorQuerier_C|GetDoorQueried _array_element)
            (:Is%20Valid
              (Utilities|Array|Add (Variables|Default|GetDoors) (Variables|/Game/Scripts/Blueprints/LevelDesignHelper/Dungeon/BP_DoorQuerier.BP_DoorQuerier_C|GetDoorQueried _array_element))
              (CallFunction|UpdateDoor _array_element)))))))
  (Development|PrintString (Utilities|String|Append " Il door manager rinominato " (Utilities|GetDisplayName self) " ha " (Utilities|String|ToString(Integer) (Utilities|Array|Length (Variables|Default|GetDoors))) " porte in lista") true true "(R=0.000000,G=0.660000,B=1.000000,A=1.000000)" 1e+01))

(event EventBeginPlay
  (Utilities|FlowControl|Delay 2.0)
  (CallFunction|UpdateDoorState))

(event Collision|EventActorBeginOverlap
  (params (OtherActor :type Actor%20Object%20Reference)))

(event EventTick
  (params (DeltaSeconds :type Float%20%28single-precision%29)))

(event EventOnSnapDataLoaded
  (Utilities|Array|Clear (Variables|Default|GetDoors))
  (Utilities|FlowControl|Delay 2.0)
  (CallFunction|UpdateDoorState))

(fn ConstructionScript)

(fn UpdateDoor
  (params (DoorQuerier :type BP%20Door%20Querier%20Object%20Reference))
  (bind (_leftdoorrotation _rightdoorrotation _doorcolor _doorinteraction) (Default|GetDoorData DoorQuerier))
  (bind _doorqueried (Variables|/Game/Scripts/Blueprints/LevelDesignHelper/Dungeon/BP_DoorQuerier.BP_DoorQuerier_C|GetDoorQueried DoorQuerier))
  (Variables|/Game/Scripts/Blueprints/LevelDesignHelper/Interaction/BP_InteractibleObject_Master.BP_InteractibleObject_Master_C|SetInteractionType _doorqueried _doorinteraction)
  (Transformation|SetRelativeRotation (Variables|/Game/Scripts/Blueprints/LevelDesignHelper/Interaction/BP_MyDoor.BP_MyDoor_C|GetLeftDoor _doorqueried) _leftdoorrotation false false)
  (Transformation|SetRelativeRotation (Variables|/Game/Scripts/Blueprints/LevelDesignHelper/Interaction/BP_MyDoor.BP_MyDoor_C|GetRightDoor _doorqueried) _rightdoorrotation false false)
  (Rendering|Material|SetVectorParameterValue (Variables|/Game/Scripts/Blueprints/LevelDesignHelper/Interaction/BP_MyDoor.BP_MyDoor_C|GetLeftDoorMat _doorqueried) "EmissiveColor" _doorcolor :!class /Script/Engine.MaterialInstanceDynamic)
  (Rendering|Material|SetVectorParameterValue (Variables|/Game/Scripts/Blueprints/LevelDesignHelper/Interaction/BP_MyDoor.BP_MyDoor_C|GetRightDoorMat _doorqueried) "EmissiveColor" _doorcolor :!class /Script/Engine.MaterialInstanceDynamic)
  (Development|PrintString (Utilities|String|Append (Utilities|GetDisplayName self) "  ha caricato sulla porta " (Utilities|GetDisplayName _doorqueried) " i seguenti dati: " " Rotazione " (Utilities|String|ToString(Rotator) _leftdoorrotation) " Colore " (Utilities|String|ToString(Integer) _doorcolor) " Tipo di interazione" (Utilities|String|EnumtoString _doorinteraction)) true true "(R=0.000000,G=1.000000,B=0.001143,A=1.000000)" 15.0))