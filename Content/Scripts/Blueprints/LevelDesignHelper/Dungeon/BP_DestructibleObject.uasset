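; BP_DestructibleObject is a breakable dungeon prop that fractures when hit fast enough, with radius damage scaled by the hitting actor's speed.
; UpdateDestructionEffect applies the mesh and fracture effects at construction and play.
; On fracture it plays sound, may spawn a pickup, recursively enables physics on TracedActors, then destroys itself after a delay.
; The UpperTracing box trace that fills TracedActors has no live caller here.
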(event OnComponentHit(Destructible)
  (params (HitComponent :type Primitive%20Component%20Object%20Reference) (OtherActor :type Actor%20Object%20Reference) (OtherComp :type Primitive%20Component%20Object%20Reference) (NormalImpulse :type Vector :default "0, 0, 0") (Hit :type Hit%20Result%20Structure%20%28by%20ref%29))
  (bind _returnvalue (Transformation|GetVelocity OtherActor))
  (bind _returnvalue_2 (Math|Vector|VectorLength _returnvalue))
  (Variables|Default|SetHitLocation (.Location (Collision|BreakHitResult Hit)))
  (if (> _returnvalue_2 (Variables|Destruction|GetSpeedTollerance))
    (Class|DestructibleComponent|ApplyRadiusDamage (Variables|Default|GetDestructible) (* (/ _returnvalue_2 5e+02) (Variables|Destruction|GetDamageMultiplier)) (Variables|Default|GetHitLocation) (Variables|Destruction|GetDamageRadius) (Variables|Destruction|GetImpulseStrenght) false)))

(event OnComponentFracture(Destructible)
  (params (HitPoint :type Vector%20%28by%20ref%29 :default "0, 0, 0") (HitDirection :type Vector%20%28by%20ref%29 :default "0, 0, 0"))
  (Audio|PlaySoundatLocation (Variables|Destruction|GetFractureSoundEffect) (Transformation|GetActorLocation) "0, 0, 0" 1.0 1.0 0.0 0 0 0)
  (CallFunction|SetPhysicalSimulationonUpperObjects)
  (CallFunction|GenerateRandomSpawn)
  (Utilities|FlowControl|Delay (Variables|Destruction|GetAutoDestructionTimer))
  (Actor|DestroyActor))

(event EventBeginPlay
  (CallFunction|UpdateDestructionEffect))

(event Collision|EventActorBeginOverlap
  (params (OtherActor :type Actor%20Object%20Reference)))

(event EventTick
  (params (DeltaSeconds :type Float%20%28single-precision%29)))

(event EventOnSnapDataLoaded
  (CallFunction|UpdateDestructionEffect))

(fn ConstructionScript
  (CallFunction|UpdateDestructionEffect))

(fn UpdateDestructionEffect
  (bind _destructible (Variables|Default|GetDestructible))
  (bind _fractureeffects (Variables|/Script/ApexDestruction.DestructibleComponent|GetFractureEffects _destructible))
  (Class|DestructibleComponent|SetDestructibleMesh _destructible (Variables|Destruction|GetDestructibleMesh))
  (Variables|/Script/ApexDestruction.DestructibleComponent|SetLargeChunkThreshold _destructible (Variables|Destruction|GetLargeChunkThreshold))
  (for (_array_element _array_index) _fractureeffects
    (bind _structout (Utilities|Struct|SetmembersinFractureEffect _array_element (Variables|Destruction|GetFractureParticleEffect) (Variables|Destruction|GetFractureSoundEffect)))
    (Utilities|Array|SetArrayElem _fractureeffects _array_index _structout)))

(fn SetPhysicalSimulationonUpperObjects
  (for _array_element (Variables|UpperObjectDetection|GetTracedActors)
    (Utilities|FlowControl|Sequence
      (:then_0
        (for _array_element_2 (Actor|GetComponentsByClass _array_element "/Script/Engine.StaticMeshComponent")
          (Utilities|IsValid _array_element_2
            (:Is%20Valid
              (Transformation|SetMobility _array_element_2 "Movable")
              (Collision|SetCollisionResponsetoChannel _array_element_2 "ECC_Pawn" "ECR_Ignore")
              (Physics|SetSimulatePhysics _array_element_2 true)))))
      (:then_1
        (bind _asbp_destructible_object (Utilities|Casting|CastToBP_DestructibleObject _array_element))
        (Utilities|IsValid (Variables|BP_DestructibleObject_C|GetDestructible _asbp_destructible_object)
          (:Is%20Valid
            (Transformation|SetMobility (Variables|BP_DestructibleObject_C|GetDestructible _asbp_destructible_object) "Movable")
            (Physics|SetSimulatePhysics (Variables|BP_DestructibleObject_C|GetDestructible _asbp_destructible_object) true)
            (CallFunction|SetPhysicalSimulationonUpperObjects _asbp_destructible_object)))))))

(fn UpperTracing
  (params (TraceChannel :type ETraceTypeQuery%20Enum :default "TraceTypeQuery1") (DrawDebugType :type EDrawDebugTrace%20Enum :default "None"))
  (bind _destructible (Variables|Default|GetDestructible))
  (bind (_origin _boxextent) (Collision|GetComponentBounds _destructible))
  (bind _returnvalue (+ _origin "0, 0,50.000000"))
  (bind _outhits (Class|KismetSystemLibrary|BoxTraceMulti _returnvalue (+ _returnvalue (Math|Vector|MakeVector 0.0 0.0 (Variables|UpperObjectDetection|GetTraceVerticalOffset))) (* _boxextent 0.75) "0, 0, 0" TraceChannel false 0 DrawDebugType false))
  (for _array_element _outhits
    (Utilities|IsValid (.hitactor _array_element)
      (:Is%20Valid
        (Utilities|Array|Add (Variables|UpperObjectDetection|GetTracedActors) (.hitactor _array_element))))))

(fn GenerateRandomSpawn
  (if (Variables|Default|GetSpawnEnabled?)
    (LocalVariables|SetPerc (Math|Random|RandomFloatinRange 0.0 1.0))
    (if (<= (LocalVariables|GetPerc) 0.15)
      (Game|SpawnActorfromClass "/Game/Scripts/Blueprints/LevelDesignHelper/Interaction/BP_PickUpable.BP_PickUpable_C" (Transformation|GetActorTransform) "Undefined" 0 0))))