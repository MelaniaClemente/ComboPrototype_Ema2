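; Dungeon helper actor that finds the closest BP_MyDoor within MaxDistance and records that door's opening data.
; On BeginPlay and when snap data loads, it waits briefly, scans all doors by distance and binds to the chosen door's OnDoorOpening dispatcher.
; Each opening event caches both leaf rotations, door color and interaction type, which GetDoorData exposes.
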(event Custom|OnDoorOpening_Event_0
  (params (LeftDoorRelativeRotation :type Rotator) (RightDoorRelativeRotation :type Rotator) (DoorColor :type Linear%20Color%20Structure) (InteractionType :type ENUM_InteractionType%20Enum :default "NewEnumerator2"))
  (Variables|Default|SetLeftDoorRotation LeftDoorRelativeRotation)
  (Variables|Default|SetRightDoorRotation RightDoorRelativeRotation)
  (Variables|Default|SetDoorColor DoorColor)
  (Variables|Default|SetDoorInteraction InteractionType))

(event Custom|SearchClosestDoor
  (Utilities|FlowControl|Delay 0.2)
  (bind _outactors (Actor|GetAllActorsOfClass "/Game/Scripts/Blueprints/LevelDesignHelper/Interaction/BP_MyDoor.BP_MyDoor_C"))
  (if (> (Utilities|Array|Length _outactors) 0)
    (bind _closestdoor (CallFunction|CheckDoorDistances _outactors))
    (Utilities|IsValid _closestdoor
      (:Is%20Valid
        (bind _output_get (Variables|Default|SetDoorQueried _closestdoor))
        (EventDispatchers|AssignOnDoorOpening _output_get (delegate Custom|OnDoorOpening_Event_0))))))

(event Custom|DoorResearch
  (CallFunction|SearchClosestDoor))

(event EventBeginPlay
  (CallFunction|DoorResearch))

(event Collision|EventActorBeginOverlap
  (params (OtherActor :type Actor%20Object%20Reference)))

(event EventTick
  (params (DeltaSeconds :type Float%20%28single-precision%29)))

(event EventOnSnapDataLoaded
  (CallFunction|DoorResearch))

(fn ConstructionScript)

(fn CheckDoorDistances
  (params (Array :type Array%20of%20BP%20My%20Door%20Object%20References))
  (LocalVariables|SetDistance (Variables|Default|GetMaxDistance))
  (for (_array_element _array_index) Array
    (if (< (Transformation|GetDistanceTo _array_element self) (LocalVariables|GetDistance))
      (LocalVariables|SetDistance (Transformation|GetDistanceTo _array_element self))
      (LocalVariables|SetDoor _array_element)
      (LocalVariables|SetIndex _array_index)))
  (return (LocalVariables|GetDoor) (LocalVariables|GetIndex) (LocalVariables|GetDistance)))

(fn GetDoorData
  (return (Variables|Default|GetLeftDoorRotation) (Variables|Default|GetRightDoorRotation) (Variables|Default|GetDoorColor) (Variables|Default|GetDoorInteraction)))

(fn PrintDebugMessage
  (bind _doorqueried (Variables|Default|GetDoorQueried)
    (:then
      (Development|PrintString (Utilities|String|Append "Caricamento: " (Utilities|GetDisplayName self) "ha caricato i dati sulla " (Utilities|GetDisplayName _doorqueried)) true true "(R=1.000000,G=0.794904,B=0.000000,A=1.000000)" 1e+01))
    (:else)))