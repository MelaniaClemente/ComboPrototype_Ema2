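; BP_AxeTrap is a child trap Blueprint that times a sound to the swing of its axe mesh.
; Each Tick it compares the mesh's absolute relative rotation to MaxAngle with a small tolerance and sets a flag at the peak.
; When the rotation next nears three quarters of that angle, it plays the Audio component if idle and clears the flag.
; The swing itself is not driven here, and the PlaySound event is empty.
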(event Custom|PlaySound)

(event EventBeginPlay
  (|CallParentFunction))

(event Collision|EventActorBeginOverlap
  (params (OtherActor :type Actor%20Object%20Reference))
  (|CallParentFunction OtherActor) ; This node is disabled and will not be called.\nDrag off pins to build functionality.
)

(event EventTick
  (params (DeltaSeconds :type Float%20%28single-precision%29))
  (bind _staticmesh (Variables|Default|GetStaticMesh))
  (bind _staticmesh_2 (Variables|Default|GetStaticMesh))
  (bind _relativerotation (Variables|/Script/Engine.SceneComponent|GetRelativeRotation _staticmesh))
  (bind _relativerotation_2 (Variables|/Script/Engine.SceneComponent|GetRelativeRotation _staticmesh_2))
  (|CallParentFunction DeltaSeconds)
  (Utilities|FlowControl|Sequence
    (:then_0
      ;[1 1 1] Check If it has reached the max angle
      (if (Math|Rotator|Equal(Rotator) (Math|Rotator|MakeRotator (Math|Float|Absolute(Float) (.roll _relativerotation)) (Math|Float|Absolute(Float) (.pitch _relativerotation)) (Math|Float|Absolute(Float) (.yaw _relativerotation))) (Variables|Default|GetMaxAngle) 1.0)
        (Variables|Default|SetMaxAngleReached true)))
    (:then_1
      ;[1 1 1] Play sound when descendent
      (if (Math|Boolean|ANDBoolean (Math|Rotator|Equal(Rotator) (Math|Rotator|MakeRotator (Math|Float|Absolute(Float) (.roll _relativerotation_2)) (Math|Float|Absolute(Float) (.pitch _relativerotation_2)) (Math|Float|Absolute(Float) (.yaw _relativerotation_2))) (* (Variables|Default|GetMaxAngle) 0.75) 1.0) (not (Audio|Components|Audio|IsPlaying (Variables|Default|GetAudio))) (Variables|Default|GetMaxAngleReached))
        (Audio|Components|Audio|Play (Variables|Default|GetAudio) 0.0)
        (Variables|Default|SetMaxAngleReached false)))))

(fn ConstructionScript
  (|CallParentFunction))