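; Configurable base trap actor whose moving mesh damages overlapping characters by a percentage of max health and triggers hit reactions.
; The construction script configures movement timelines and builds an optional sphere, box or capsule trigger.
; Activation and deactivation follow type settings, such as trigger overlap or movement end, with delayed toggling.
; Tick switches mesh collision by state and, while active, drives constant or cosine pendulum rotation plus curve or spline movement.
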(event OnComponentBeginOverlap(StaticMesh)
  (params (OverlappedComponent :type Primitive%20Component%20Object%20Reference) (OtherActor :type Actor%20Object%20Reference) (OtherComp :type Primitive%20Component%20Object%20Reference) (OtherBodyIndex :type Integer) (bFromSweep :type Boolean) (SweepResult :type Hit%20Result%20Structure%20%28by%20ref%29))
  ;[0 0 0] MeshOverlap
  (bind _asskeletal_mesh_component (Utilities|Casting|CastToSkeletalMeshComponent OtherComp))
  (bind _asbp_character_master (Utilities|Casting|CastToBP_CharacterMaster (Components|GetOwner _asskeletal_mesh_component)))
  (Variables|Gameplay|SetOverlappedCharacter _asbp_character_master)
  (Utilities|FlowControl|DoOnce false
    (:Completed
      (CallFunction|UpdatePercentageDamage _asbp_character_master)
      (CallFunction|SingleTargetGameplayAction _asbp_character_master (Variables|Gameplay|GetOverlapActions) false)
      (Default|PlayHitReactionAnimation (Variables|/Game/Scripts/Blueprints/Characters/BP_CharacterMaster.BP_CharacterMaster_C|GetBP_CombatComponent _asbp_character_master) (Variables|Gameplay|GetOverlappedCharacter) self "NewEnumerator0")
      (Default|SpawnHitReactionTraps (Variables|Gameplay|GetOverlappedCharacter) "NewEnumerator2" (Transformation|GetActorLocation (Variables|Gameplay|GetOverlappedCharacter)) (Math|Random|RandomRotator true)))))

(event OnComponentEndOverlap(StaticMesh)
  (params (OverlappedComponent :type Primitive%20Component%20Object%20Reference) (OtherActor :type Actor%20Object%20Reference) (OtherComp :type Primitive%20Component%20Object%20Reference) (OtherBodyIndex :type Integer))
  ;[0 0 0] MeshOverlap
  (if (== OtherActor (Variables|Gameplay|GetOverlappedCharacter))
    (Variables|Gameplay|SetOverlappedCharacter 0)
    (Utilities|FlowControl|DoOnce false) ; enters at Reset
  ))

(event OnComponentBeginOverlap(CapsuleTrigger)
  (params (OverlappedComponent :type Primitive%20Component%20Object%20Reference) (OtherActor :type Actor%20Object%20Reference) (OtherComp :type Primitive%20Component%20Object%20Reference) (OtherBodyIndex :type Integer) (bFromSweep :type Boolean) (SweepResult :type Hit%20Result%20Structure%20%28by%20ref%29))
  ;[0 0 0] TriggersOverlap
)

(event OnComponentBeginOverlap(SphereTrigger)
  (params (OverlappedComponent :type Primitive%20Component%20Object%20Reference) (OtherActor :type Actor%20Object%20Reference) (OtherComp :type Primitive%20Component%20Object%20Reference) (OtherBodyIndex :type Integer) (bFromSweep :type Boolean) (SweepResult :type Hit%20Result%20Structure%20%28by%20ref%29))
  ;[0 0 0] TriggersOverlap
)

(event OnComponentBeginOverlap(BoxTrigger)
  (params (OverlappedComponent :type Primitive%20Component%20Object%20Reference) (OtherActor :type Actor%20Object%20Reference) (OtherComp :type Primitive%20Component%20Object%20Reference) (OtherBodyIndex :type Integer) (bFromSweep :type Boolean) (SweepResult :type Hit%20Result%20Structure%20%28by%20ref%29))
  ;[0 0 0] TriggersOverlap
)

(event OnComponentEndOverlap(BoxTrigger)
  (params (OverlappedComponent :type Primitive%20Component%20Object%20Reference) (OtherActor :type Actor%20Object%20Reference) (OtherComp :type Primitive%20Component%20Object%20Reference) (OtherBodyIndex :type Integer))
  ;[0 0 0] TriggersOverlap
)

(event OnComponentEndOverlap(CapsuleTrigger)
  (params (OverlappedComponent :type Primitive%20Component%20Object%20Reference) (OtherActor :type Actor%20Object%20Reference) (OtherComp :type Primitive%20Component%20Object%20Reference) (OtherBodyIndex :type Integer))
  ;[0 0 0] TriggersOverlap
)

(event OnComponentEndOverlap(SphereTrigger)
  (params (OverlappedComponent :type Primitive%20Component%20Object%20Reference) (OtherActor :type Actor%20Object%20Reference) (OtherComp :type Primitive%20Component%20Object%20Reference) (OtherBodyIndex :type Integer))
  ;[0 0 0] TriggersOverlap
)

(event Custom|Reverse%20CurveTimeline
  (bind _startlocation (Variables|LinearMovement|Curve|GetStartLocation))
  ;[0 0 0] Timelines
  (bind _locationlerpcurve (Timeline|CurveLocationTimeline Reverse)
    (:Update
      (Transformation|SetRelativeLocation (Variables|Default|GetStaticMesh) (Math|Vector|Lerp(Vector) _startlocation (+ _startlocation (Variables|LinearMovement|Curve|GetLocationOffset)) _locationlerpcurve) false false))
    (:Finished
      (Default|CallOnLinearMovementEnd))))

(event Custom|PlayCurveTimeline
  (bind _startlocation (Variables|LinearMovement|Curve|GetStartLocation))
  ;[0 0 0] Timelines
  (bind _locationlerpcurve (Timeline|CurveLocationTimeline Play)
    (:Update
      (Transformation|SetRelativeLocation (Variables|Default|GetStaticMesh) (Math|Vector|Lerp(Vector) _startlocation (+ _startlocation (Variables|LinearMovement|Curve|GetLocationOffset)) _locationlerpcurve) false false))
    (:Finished
      (Default|CallOnLinearMovementEnd))))

(event Custom|TrapOn
  ;[0 0 0] Activation
  (switch Utilities|FlowControl|Switch|SwitchonENUM_TrapActivationType (Variables|Activation|GetActivationType)
    (:NewEnumerator0
      (Variables|Activation|SetActivated false))
    (:NewEnumerator1
      (CallFunction|ToogleActivation true))
    (:NewEnumerator2
      (CallFunction|BindActivationonBeginOverlap (delegate Custom|ActivateOnTriggerBeginOverlap)))
    (:NewEnumerator3
      (EventDispatchers|BindEventtoOnLinearMovementEnd (delegate Custom|ActivateOnLinearMovementEnd)))))

(event Custom|ActivateOnTriggerBeginOverlap
  (params (OverlappedComponent :type Primitive%20Component%20Object%20Reference) (OtherActor :type Actor%20Object%20Reference) (OtherComp :type Primitive%20Component%20Object%20Reference) (OtherBodyIndex :type Integer) (bFromSweep :type Boolean) (SweepResult :type Hit%20Result%20Structure%20%28by%20ref%29))
  ;[0 0 0] Activation
  (CallFunction|ProcessTriggerBeginOverlap OtherActor OtherComp))

(event Custom|ActivateOnLinearMovementEnd
  ;[0 0 0] Activation
  (CallFunction|ToogleActivation true))

(event Custom|TrapOff
  ;[0 0 0] Activation
  (switch Utilities|FlowControl|Switch|SwitchonENUM_TrapActivationType (Variables|Activation|GetDeactivationType)
    (:NewEnumerator2
      (Default|CallOnDeactivation)
      (CallFunction|BindActivationonEndOverlap (delegate Custom|DeactivateOnTriggerEndOverlap)))
    (:NewEnumerator3
      (Default|CallOnDeactivation)
      (EventDispatchers|BindEventtoOnLinearMovementEnd (delegate Custom|DeactivateOnLinearMovementEnd)))))

(event Custom|DeactivateOnTriggerEndOverlap
  (params (OverlappedComponent :type Primitive%20Component%20Object%20Reference) (OtherActor :type Actor%20Object%20Reference) (OtherComp :type Primitive%20Component%20Object%20Reference) (OtherBodyIndex :type Integer))
  ;[0 0 0] Activation
  (CallFunction|ProcessTriggerEndOverlap OtherActor OtherComp))

(event Custom|DeactivateOnLinearMovementEnd
  ;[0 0 0] Activation
  (Variables|Activation|SetActivated false))

(event Custom|PlaySplineTimeline
  (bind _splinemovmement (Variables|Default|GetSplineMovmement))
  ;[0 0 0] Timelines
  (bind _splinecurve (Timeline|SplineMovmentTimeline Play)
    (:Update
      (Transformation|SetRelativeLocation (Variables|Default|GetStaticMesh) (Spline|GetLocationatDistanceAlongSpline _splinemovmement (Math|Float|Lerp 0.0 (Spline|GetSplineLength _splinemovmement) _splinecurve) "Local") false false))
    (:Finished
      (Default|CallOnLinearMovementEnd))))

(event Custom|StopCurveTimeline
  (bind _startlocation (Variables|LinearMovement|Curve|GetStartLocation))
  ;[0 0 0] Timelines
  (bind _locationlerpcurve (Timeline|CurveLocationTimeline Stop)
    (:Update
      (Transformation|SetRelativeLocation (Variables|Default|GetStaticMesh) (Math|Vector|Lerp(Vector) _startlocation (+ _startlocation (Variables|LinearMovement|Curve|GetLocationOffset)) _locationlerpcurve) false false))
    (:Finished
      (Default|CallOnLinearMovementEnd))))

(event Custom|ToogleActivation
  (params (Activated :type Boolean))
  ;[0 0 0] Activation
  (Utilities|FlowControl|RetriggerableDelay (Variables|Activation|GetActivationDelay))
  (bind _output_get (Variables|Activation|SetActivated Activated))
  (if _output_get
    (Default|CallOnActivation)))

(event Custom|ReverseSplineTimeline
  (bind _splinemovmement (Variables|Default|GetSplineMovmement))
  ;[0 0 0] Timelines
  (bind _splinecurve (Timeline|SplineMovmentTimeline Reverse)
    (:Update
      (Transformation|SetRelativeLocation (Variables|Default|GetStaticMesh) (Spline|GetLocationatDistanceAlongSpline _splinemovmement (Math|Float|Lerp 0.0 (Spline|GetSplineLength _splinemovmement) _splinecurve) "Local") false false))
    (:Finished
      (Default|CallOnLinearMovementEnd))))

(event Custom|PlayFromStartCurveTimeline
  (bind _startlocation (Variables|LinearMovement|Curve|GetStartLocation))
  ;[0 0 0] Timelines
  (bind _locationlerpcurve (Timeline|CurveLocationTimeline PlayFromStart)
    (:Update
      (Transformation|SetRelativeLocation (Variables|Default|GetStaticMesh) (Math|Vector|Lerp(Vector) _startlocation (+ _startlocation (Variables|LinearMovement|Curve|GetLocationOffset)) _locationlerpcurve) false false))
    (:Finished
      (Default|CallOnLinearMovementEnd))))

(event Custom|Play%20from%20startSplineTimeline
  (bind _splinemovmement (Variables|Default|GetSplineMovmement))
  ;[0 0 0] Timelines
  (bind _splinecurve (Timeline|SplineMovmentTimeline PlayFromStart)
    (:Update
      (Transformation|SetRelativeLocation (Variables|Default|GetStaticMesh) (Spline|GetLocationatDistanceAlongSpline _splinemovmement (Math|Float|Lerp 0.0 (Spline|GetSplineLength _splinemovmement) _splinecurve) "Local") false false))
    (:Finished
      (Default|CallOnLinearMovementEnd))))

(event Custom|StopSplineTimenline
  (bind _splinemovmement (Variables|Default|GetSplineMovmement))
  ;[0 0 0] Timelines
  (bind _splinecurve (Timeline|SplineMovmentTimeline Stop)
    (:Update
      (Transformation|SetRelativeLocation (Variables|Default|GetStaticMesh) (Spline|GetLocationatDistanceAlongSpline _splinemovmement (Math|Float|Lerp 0.0 (Spline|GetSplineLength _splinemovmement) _splinecurve) "Local") false false))
    (:Finished
      (Default|CallOnLinearMovementEnd))))

(event EventBeginPlay
  ;[0 0 0] BeginPlay
  (Variables|LinearMovement|Curve|SetStartLocation (Variables|/Script/Engine.SceneComponent|GetRelativeLocation (Variables|Default|GetStaticMesh)))
  (CallFunction|Trapon)
  (CallFunction|TrapOff))

(event Collision|EventActorBeginOverlap
  (params (OtherActor :type Actor%20Object%20Reference)))

(event EventTick
  (params (DeltaSeconds :type Float%20%28single-precision%29))
  ;[0 0 0] Tick
  (CallFunction|UpdateMeshCollisionResponse (Variables|Collision|GetCollisionWhenActive) (Variables|Collision|GetCollisionWhenInactive))
  (if (Variables|Activation|GetActivated)
    (CallFunction|UpdateRotation DeltaSeconds)
    (CallFunction|UpdateLinearMovement)))

(fn ConstructionScript
  (bind _triggeroffset (Variables|Activation|Trigger|GetTriggerOffset))
  (CallFunction|SetCurveTimelineParameters)
  (CallFunction|SetSplineCurveParameters)
  (switch Utilities|FlowControl|Switch|SwitchonENUM_TrapActivationType (Variables|Activation|GetActivationType)
    (:NewEnumerator0
      (Variables|Activation|SetActivated false))
    (:NewEnumerator1
      (Variables|Activation|SetActivated true))
    (:NewEnumerator2
      (switch Utilities|FlowControl|Switch|SwitchonENUM_ColliderType (Variables|Activation|Trigger|GetTriggerType)
        (:NewEnumerator0
          (Utilities|IsValid (Variables|Default|GetSphereTrigger)
            (:Is%20Valid
              _)
            (:Is%20Not%20Valid
              (bind _returnvalue (AddComponent|AddSphereComponent false _triggeroffset))
              (bind _output_get (Variables|Default|SetSphereTrigger _returnvalue))))
          (Components|Sphere|SetSphereRadius _output_get (Variables|Activation|Trigger|GetTriggerRadius) true)
          (Collision|SetCollisionResponsetoAllChannels (Variables|Default|GetSphereTrigger) "ECR_Overlap")
          (Development|SetHiddeninGame (Variables|Default|GetSphereTrigger) (Variables|Activation|Trigger|GetTriggerHiddenIngame) false)
          (Variables|/Script/Engine.PrimitiveComponent|SetbGenerateOverlapEvents (Variables|Default|GetSphereTrigger) true))
        (:NewEnumerator1
          (Utilities|IsValid (Variables|Default|GetBoxTrigger)
            (:Is%20Valid
              _)
            (:Is%20Not%20Valid
              (bind _returnvalue_2 (AddComponent|AddBoxComponent false _triggeroffset))
              (bind _output_get_2 (Variables|Default|SetBoxTrigger _returnvalue_2))))
          (Components|Box|SetBoxExtent _output_get_2 (Variables|Activation|Trigger|GetTriggerBoxDimension) true)
          (Collision|SetCollisionResponsetoAllChannels (Variables|Default|GetBoxTrigger) "ECR_Overlap")
          (Development|SetHiddeninGame (Variables|Default|GetBoxTrigger) (Variables|Activation|Trigger|GetTriggerHiddenIngame) false)
          (Variables|/Script/Engine.PrimitiveComponent|SetbGenerateOverlapEvents (Variables|Default|GetBoxTrigger) true))
        (:NewEnumerator2
          (Utilities|IsValid (Variables|Default|GetCapsuleTrigger)
            (:Is%20Valid
              _)
            (:Is%20Not%20Valid
              (bind _returnvalue_3 (AddComponent|AddCapsuleComponent false _triggeroffset))
              (bind _output_get_3 (Variables|Default|SetCapsuleTrigger _returnvalue_3))))
          (Components|Capsule|SetCapsuleRadius _output_get_3 (Variables|Activation|Trigger|GetTriggerRadius) true)
          (Components|Capsule|SetCapsuleHalfHeight (Variables|Default|GetCapsuleTrigger) (Variables|Activation|Trigger|GetTriggerHalfHeight) true)
          (Collision|SetCollisionResponsetoAllChannels (Variables|Default|GetCapsuleTrigger) "ECR_Overlap")
          (Development|SetHiddeninGame (Variables|Default|GetCapsuleTrigger) (Variables|Activation|Trigger|GetTriggerHiddenIngame) false)
          (Variables|/Script/Engine.PrimitiveComponent|SetbGenerateOverlapEvents (Variables|Default|GetCapsuleTrigger) true))))))

(fn GetPendulumRotation
  (bind _returnvalue (CallFunction|GetPendolumPhase))
  (bind _maxangle (Variables|Rotation|Pendulum|GetMaxAngle))
  (return (Math|Rotator|MakeRotator (* (.roll _maxangle) (.roll _returnvalue)) (* (.pitch _maxangle) (.pitch _returnvalue)) (* (.yaw _maxangle) (.yaw _returnvalue)))))

(fn InitializeRotatingMovement
  (switch Utilities|FlowControl|Switch|SwitchonENUM_RotationType (Variables|Rotation|GetRotationType)
    (:NewEnumerator2
      (Variables|Rotation|SetStartingAngle (Variables|/Script/Engine.SceneComponent|GetRelativeRotation (Variables|Default|GetStaticMesh))))))

(fn SetCurveTimelineParameters
  (bind _curvelocationtimeline (Variables|Default|GetCurveLocationTimeline))
  (Components|Timeline|SetPlayRate _curvelocationtimeline (Variables|LinearMovement|Curve|GetCurveSpeed))
  (Class|TimelineComponent|SetFloatCurve _curvelocationtimeline (Variables|LinearMovement|Curve|GetMovementCurve) "LocationLerpCurve")
  (Components|Timeline|SetLooping _curvelocationtimeline (Variables|LinearMovement|Curve|GetCurveLooping)))

(fn SetSplineCurveParameters
  (Components|Timeline|SetPlayRate (Variables|Default|GetSplineMovmentTimeline) (Variables|LinearMovement|Spline|GetSplineSpeed))
  (Class|TimelineComponent|SetFloatCurve (Variables|Default|GetSplineMovmentTimeline) (Variables|LinearMovement|Spline|GetSplineCurve) "SplineCurve")
  (Components|Timeline|SetLooping (Variables|Default|GetSplineMovmentTimeline) (Variables|LinearMovement|Spline|GetSplineLoop)))

(fn UpdateRotation
  (params (Delta%20Second :type Float%20%28single-precision%29))
  (bind _staticmesh (Variables|Default|GetStaticMesh))
  (switch Utilities|FlowControl|Switch|SwitchonENUM_RotationType (Variables|Rotation|GetRotationType)
    (:NewEnumerator1
      (Transformation|SetRelativeRotation _staticmesh (Math|Rotator|CombineRotators (Variables|/Script/Engine.SceneComponent|GetRelativeRotation _staticmesh) (* (Variables|Rotation|GetMaxRotationSpeed) Delta%20Second)) false false))
    (:NewEnumerator2
      (Transformation|SetRelativeRotation (Variables|Default|GetStaticMesh) (CallFunction|GetPendulumRotation) false false))))

(fn UpdateLinearMovement
  (switch Utilities|FlowControl|Switch|SwitchonENUM_LinearMovementType (Variables|LinearMovement|GetMovementType)
    (:NewEnumerator1
      (if (not (Audio|Components|Audio|IsPlaying (Variables|Default|GetSplineMovmentTimeline)))
        (if (Variables|LinearMovement|Spline|GetSplineLoop)
          (CallFunction|PlaySplineTimeline)
          (else
            (CallFunction|PlayfromStartSplineTimeline)))))
    (:NewEnumerator2
      (if (not (Audio|Components|Audio|IsPlaying (Variables|Default|GetCurveLocationTimeline)))
        (if (Variables|LinearMovement|Curve|GetCurveLooping)
          (CallFunction|PlayCurveTimeline)
          (else
            (CallFunction|PlayfromStartCurveTimeline)))))))

(fn ProcessTriggerBeginOverlap
  (params (Object :type Object%20Object%20Reference) (CapsuleComponent :type Object%20Object%20Reference))
  (Utilities|Casting|CastToBP_CharacterMaster Object)
  (Utilities|Casting|CastToCapsuleComponent CapsuleComponent)
  (CallFunction|ToogleActivation true)
  (Default|CallOnTriggerBeginOverlap))

(fn ProcessTriggerEndOverlap
  (params (Object :type Object%20Object%20Reference) (Component :type Object%20Object%20Reference))
  (Utilities|Casting|CastToBP_CharacterMaster Object)
  (Utilities|Casting|CastToCapsuleComponent Component)
  (CallFunction|ToogleActivation false)
  (Default|CallOnTriggerEndOverlap))

(fn UpdateMeshCollisionResponse
  (params (OnActivationResponse :type ECollisionResponse%20Enum :default "ECR_Ignore") (OnDeactivationResponse :type ECollisionResponse%20Enum :default "ECR_Ignore"))
  (bind _staticmesh (Variables|Default|GetStaticMesh))
  (if (Variables|Activation|GetActivated)
    (Collision|SetCollisionResponsetoAllChannels _staticmesh OnActivationResponse)
    (else
      (Collision|SetCollisionResponsetoAllChannels _staticmesh OnDeactivationResponse))))

(fn HasAValidTrigger?
  (bind _boxtrigger (Variables|Default|GetBoxTrigger))
  (bind _capsuletrigger (Variables|Default|GetCapsuleTrigger))
  (bind _spheretrigger (Variables|Default|GetSphereTrigger))
  (return (Math|Boolean|ORBoolean (Utilities|IsValid _boxtrigger) (Utilities|IsValid _capsuletrigger) (Utilities|IsValid _spheretrigger)) _boxtrigger _capsuletrigger _spheretrigger))

(fn GetPendolumPhase
  (bind _returnvalue (Utilities|Time|GetTimeSeconds))
  (bind _maxrotationspeed (Variables|Rotation|GetMaxRotationSpeed))
  (bind _startingangle (Variables|Rotation|GetStartingAngle))
  (bind _returnvalue_2 (* _maxrotationspeed _returnvalue))
  (return (Math|Rotator|MakeRotator (Math|Trig|Cos(Degrees) (+ (.roll _startingangle) (.roll _returnvalue_2))) (Math|Trig|Cos(Degrees) (+ (.pitch _startingangle) (.pitch _returnvalue_2))) (Math|Trig|Cos(Degrees) (+ (.yaw _startingangle) (.yaw _returnvalue_2))))))

(fn ApplyPendulumAcceleration
  (bind _maxrotationspeed (Variables|Rotation|GetMaxRotationSpeed))
  (bind _rotationaccelerationcurve (Variables|Rotation|Pendulum|GetRotationAccelerationCurve))
  (bind _staticmesh (Variables|Default|GetStaticMesh))
  (bind _relativerotation (Variables|/Script/Engine.SceneComponent|GetRelativeRotation _staticmesh))
  (Variables|Rotation|SetCurrentRotationSpeed (Math|Rotator|MakeRotator (* (.roll _maxrotationspeed) (Math|Curves|GetFloatValue _rotationaccelerationcurve (Math|Trig|Sin(Degrees) (.roll _relativerotation)))) (* (.pitch _maxrotationspeed) (Math|Curves|GetFloatValue _rotationaccelerationcurve (Math|Trig|Sin(Degrees) (.pitch _relativerotation)))) (* (.yaw _maxrotationspeed) (Math|Curves|GetFloatValue _rotationaccelerationcurve (Math|Trig|Sin(Degrees) (.yaw _relativerotation)))))))

(fn BindActivationonBeginOverlap
  (params (Event :type Delegate%20%28by%20ref%29))
  (bind _boxtrigger (Variables|Default|GetBoxTrigger))
  (bind _capsuletrigger (Variables|Default|GetCapsuleTrigger))
  (bind _spheretrigger (Variables|Default|GetSphereTrigger))
  (Utilities|IsValid _boxtrigger
    (:Is%20Valid
      (Collision|BindEventtoOnComponentBeginOverlap _boxtrigger Event))
    (:Is%20Not%20Valid
      (Utilities|IsValid _capsuletrigger
        (:Is%20Valid
          (Collision|BindEventtoOnComponentBeginOverlap _capsuletrigger Event))
        (:Is%20Not%20Valid
          (Utilities|IsValid _spheretrigger
            (:Is%20Valid
              (Collision|BindEventtoOnComponentBeginOverlap _spheretrigger Event))))))))

(fn BindActivationonEndOverlap
  (params (Event :type Delegate%20%28by%20ref%29))
  (bind _boxtrigger (Variables|Default|GetBoxTrigger))
  (bind _capsuletrigger (Variables|Default|GetCapsuleTrigger))
  (bind _spheretrigger (Variables|Default|GetSphereTrigger))
  (Utilities|IsValid _boxtrigger
    (:Is%20Valid
      (Collision|BindEventtoOnComponentEndOverlap _boxtrigger Event))
    (:Is%20Not%20Valid
      (Utilities|IsValid _capsuletrigger
        (:Is%20Valid
          (Collision|BindEventtoOnComponentEndOverlap _capsuletrigger Event))
        (:Is%20Not%20Valid
          (Utilities|IsValid _spheretrigger
            (:Is%20Valid
              (Collision|BindEventtoOnComponentEndOverlap _spheretrigger Event))))))))

(fn UpdatePercentageDamage
  (params (self2 :type BP%20Character%20Master%20Object%20Reference))
  (bind _structout (Utilities|Struct|SetmembersinSTRUCT_GameActions_new (Variables|Gameplay|GetOverlapActions) (Utilities|Array|MakeArray (* (.maxvalue (Variables|/Game/Scripts/Blueprints/Components/GameParameters/BP_CharacterParametersComponent.BP_CharacterParametersComponent_C|GetGameAttribute (Variables|/Game/Scripts/Blueprints/Characters/BP_CharacterMaster.BP_CharacterMaster_C|GetBP_HealthComponent self2))) (Variables|Default|GetDamagePercentageValue)))))
  (Variables|Gameplay|SetOverlapActions _structout))

(fn GetPendulumSpeed
  (return (.pitch (CallFunction|GetPendulumRotation))))