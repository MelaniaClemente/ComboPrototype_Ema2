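; BP_GlobalNotification is a ProHUD demo trigger actor that shows a global HUD notification when something overlaps its Box component.
; The overlap event calls DisplayGlobalNotification on the HUD manager, passing the display time, type and headline text, and background and particle colors from its variables.
; The construction script copies the Text variable onto a TextRender component as an in-world label.
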(event OnComponentBeginOverlap(Box)
  (params (OverlappedComponent :type Primitive%20Component%20Object%20Reference) (OtherActor :type Actor%20Object%20Reference) (OtherComp :type Primitive%20Component%20Object%20Reference) (OtherBodyIndex :type Integer) (bFromSweep :type Boolean) (SweepResult :type Hit%20Result%20Structure%20%28by%20ref%29))
  (Default|DisplayGlobalNotification (CallFunction|GetHUDManager) (Variables|Default|GetDISPLAYTIME) (Variables|Default|GetTYPETEXT) (Variables|Default|GetHEADLINETEXT) (Variables|Default|GetBGCOLOR) (Variables|Default|GetPARTICLESCOLOR)))

(fn ConstructionScript
  (Rendering|Components|TextRender|SetText (Variables|Default|GetTextRender) (Variables|Default|GetText)))